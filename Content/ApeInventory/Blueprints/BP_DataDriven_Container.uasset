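; Data-driven loot container actor that players interact with to view its inventory, with custom-depth highlighting.
; The construction script reads a data table row to set inventory size, mesh and material.
; On BeginPlay the server fills the inventory with designated items plus generated ones from the row's type table.
; Interaction passes a lazily created, cached container widget to player 0's HUD at the actor's screen position.
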(event `self.ReceiveBeginPlay`
  (if (`KismetSystemLibrary.IsServer`)
    (`self.GenerateContainer`)))

(event `/Game/ApeInventory/Blueprints/BPI_Interactable.INT_DoInteraction`
  (bind _returnvalue (`GameplayStatics.GetPlayerController` 0))
  ;[1 1 1] Player Open Container
  (bind _widget (`self.GetContrainerWidget`))
  (message `/Game/ApeInventory/Framework/BPI_ApeInventory_HUD.INT_AddContainerWidget` (`PlayerController.GetHUD` _returnvalue) _widget (`WidgetLayoutLibrary.ProjectWorldLocationToWidgetPosition` _returnvalue (`self.K2_GetActorLocation`))))

(event `/Game/ApeInventory/Blueprints/BPI_Interactable.INT_ToggleHightlight`
  (params (Toggle :type Boolean))
  ;[1 1 1] Interact hightlight
  (`PrimitiveComponent.SetRenderCustomDepth` (`self.StaticMesh`) Toggle))

(fn `GenerateContainer`
  (bind _inventory (`self.Inventory`))
  (bind (_datatable _rowname) (break `DataTableRowHandle` (`self.Container`)))
  (`|ExecutionSequence`
    (:`then_0`
      ;[1 1 1] Add designated item(s)
      (for _array_element (`self.DesignatedItems`)
        (bind _returnvalue (`|GetDataTableRow` "/Game/ApeInventory/Database/Item/DT_Item.DT_Item" _array_element)
          (:`then`
            (bind _returnvalue_2 (`|GenericCreateObject` "/Script/Ape_Inventory.Item"))
            (bind (_itemid _name _description _maxstack _itemtype) (break `/Game/ApeInventory/Database/Item/ST_Item` _returnvalue))
            (`Item.SetItemInfo` _returnvalue_2 (make `ItemInfo` _itemid _maxstack 1 _itemtype))
            (`InventoryComponent.AddItem` _inventory _returnvalue_2)))))
    (:`then_1`
      ;[1 1 1] Container generated item
      (bind _returnvalue_3 (`|GetDataTableRow` _datatable _rowname)
        (:`then`
          (bind _outitems (`/Game/ApeInventory/Framework/FL_ItemUtil.FL_GenerateContainer` (`.TypeDT_5_5D3E176D45A22819491D1893E6ACAC2F` (break `/Game/ApeInventory/Database/Container/ST_Container` _returnvalue_3)) (`self.Generate Amount`)))
          (for _array_element_2 _outitems
            (bind _returnvalue_4 (`|GenericCreateObject` "/Script/Ape_Inventory.Item"))
            (`Item.SetItemInfo` _returnvalue_4 _array_element_2)
            (`InventoryComponent.AddItem` _inventory _returnvalue_4)))))))

(fn `GetContrainerWidget`
  (returns (Widget :type "UserWidget Object Reference"))
  (`/Engine/EditorBlueprintResources/StandardMacros.IsValid` (`self.Container Widget`)
    (:`Is Valid`
      _)
    (:`Is Not Valid`
      (bind _returnvalue (`|CreateWidget` "/Game/ApeInventory/Widgets/WBP_Container.WBP_Container_C" (`GameplayStatics.GetPlayerController` 0)))
      (bind _output_get (set `self.Container Widget` _returnvalue))))
  (`/Game/ApeInventory/Widgets/WBP_Container.InitializeContainer` _output_get (`self.Inventory`) (`.DisplayName_18_744733B04F1C9687DC9B8DA41FB041D8` (break `/Game/ApeInventory/Database/Container/ST_Container` (`self.ST_Container`))))
  (return (`self.Container Widget`)))

(fn `UserConstructionScript`
  (bind _staticmesh (`self.StaticMesh`))
  (bind (_datatable _rowname) (break `DataTableRowHandle` (`self.Container`)))
  (bind _returnvalue (`|GetDataTableRow` _datatable _rowname)
    (:`then`
      (set `self.ST_Container` _returnvalue)
      (bind (_displayname _maxsize _typedt _icon _mesh _materialinstance) (break `/Game/ApeInventory/Database/Container/ST_Container` _returnvalue))
      (set `InventoryComponent.MaxSize` _maxsize (`self.Inventory`))
      (`|ExecutionSequence`
        (:`then_0`
          (bind _returnvalue_2 (`KismetSystemLibrary.LoadAsset_Blocking` _mesh))
          (bind _asstatic_mesh (cast `StaticMesh` _returnvalue_2))
          (`StaticMeshComponent.SetStaticMesh` _staticmesh _asstatic_mesh))
        (:`then_1`
          (if (`KismetSystemLibrary.IsValidSoftObjectReference` _materialinstance)
            (bind _returnvalue_3 (`KismetSystemLibrary.LoadAsset_Blocking` _materialinstance))
            (bind _asmaterial_instance (cast `MaterialInstance` _returnvalue_3))
            (`PrimitiveComponent.SetMaterial` _staticmesh 0 _asmaterial_instance)
            (else
              (bind _returnvalue_4 (`KismetSystemLibrary.LoadAsset_Blocking` _materialinstance))
              (bind _astexture_2d (cast `Texture2D` _returnvalue_4))
              (bind _returnvalue_5 (`KismetMaterialLibrary.CreateDynamicMaterialInstance` "/Game/ApeInventory/Materials/MAT_Container.MAT_Container"))
              (`MaterialInstanceDynamic.SetTextureParameterValue` _returnvalue_5 "TextureParam" _astexture_2d)
              (`PrimitiveComponent.SetMaterial` (`self.StaticMesh`) 0 _returnvalue_5))))))))