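; BP_CameraTracker is a steerable scene-capture camera that renders to a texture target and can lock onto actors.
; Locking uses tiered, FOV-scaled sphere traces, by object type then Visibility, storing the hit offset.
; Tick aims TrackRoot at that point, with CameraRoot adding pitch/yaw, and drops tracking when the actor leaves the view margin.
; Absolute-rotation toggles switch between tracking, world-stabilized and relative modes; helpers provide target distance and screen projection.
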(event `self.ReceiveTick`
  (params (DeltaSeconds :type "Float (single-precision)"))
  (bind _skipframe (`self.SkipFrame`))
  (`|ExecutionSequence`
    (:`then_0`
      (if (`self.IsTracking`)
        (`self.TrackRotateToTarget`)
        (`self.UpdateCamera`)
        (bind _withinscreen (`self.CheckTrackingTarget`))
        (if (not _withinscreen)
          (`self.ToggleTrackingMode` false)
          (`self.UpdateCamera`))
        (else
          (`self.UpdateCamera`))))
    (:`then_1`
      (if (> _skipframe 0)
        (`/Engine/EditorBlueprintResources/StandardMacros.DecrementInt` _skipframe)
        (else
          (`SceneCaptureComponent2D.CaptureScene` (`self.SceneCaptureCamera`)))))))

(fn `AddCameraOffset`
  (params (Pitch :type "Float (double-precision)") (Yaw :type "Float (double-precision)"))
  (bind _returnvalue (* Pitch -1.0))
  (bind _cameraroot (`self.CameraRoot`))
  (bind (_returnvalue_roll _returnvalue_pitch _returnvalue_yaw) (`KismetMathLibrary.BreakRotator` (`SceneComponent.K2_GetComponentRotation` _cameraroot)))
  (if (`self.WorldMode`)
    (`SceneComponent.K2_AddWorldRotation` _cameraroot (`KismetMathLibrary.MakeRotator` 0.0 (`KismetMathLibrary.SelectFloat` 0.0 _returnvalue (> (+ _returnvalue_pitch _returnvalue) 80.0)) Yaw) false false)
    (`SceneComponent.K2_SetWorldRotation` _cameraroot (`KismetMathLibrary.MakeRotator` 0.0 (`KismetMathLibrary.FClamp` _returnvalue_pitch (`self.Pitch_Min`) (`self.Pitch_Max`)) _returnvalue_yaw) false false)
    (else
      (set `self.CurrentPitch` (`KismetMathLibrary.FClamp` (+ (`self.CurrentPitch`) Pitch) (`self.Pitch_Min`) (`self.Pitch_Max`)))
      (set `self.CurrentYaw` (mod (+ Yaw (`self.CurrentYaw`)) 360.0)))))

(fn `CheckTrackingTarget`
  (returns (WithinScreen :type Boolean))
  (locals (bTrackingTarget :type Boolean :default false) (RenderTarget :type "TextureRenderTarget2D Object Reference") (TargetLocation :type "Vector Structure" :default (0.0 0.0 0.0)) (CameraSpaceLocation :type "Vector Structure" :default (0.0 0.0 0.0)) (AspectRatio :type "Float (double-precision)" :default 0.0) (HalfHorizontalFOV :type "Float (double-precision)" :default 0.0) (HalfVerticalFOV :type "Float (double-precision)" :default 0.0) (HorizontalAngle :type "Float (double-precision)" :default 0.0) (VerticalAngle :type "Float (double-precision)" :default 0.0) (AllowedHorizontalAngle :type "Float (double-precision)" :default 0.0) (AllowedVerticalAngle :type "Float (double-precision)" :default 0.0))
  (bind _scenecapturecamera (`self.SceneCaptureCamera`))
  (bind (_cameraspacelocation_x _cameraspacelocation_y _cameraspacelocation_z) (`KismetMathLibrary.BreakVector` (`local.CameraSpaceLocation`)))
  (bind _trackingmargin (`self.TrackingMargin`))
  (`|ExecutionSequence`
    (:`then_0`
      (if (`KismetSystemLibrary.IsValidSoftObjectReference` (`self.TargetActor`))
        (set `local.bTrackingTarget` true)
        (`|ExecutionSequence`
          (:`then_0`
            ;[1 1 1] Checking if target is within screen space margin
            (bind _output_get (set `local.RenderTarget` (`SceneCaptureComponent2D.TextureTarget` _scenecapturecamera)))
            (set `local.CameraSpaceLocation` (`KismetMathLibrary.InverseTransformLocation` (`SceneComponent.K2_GetComponentToWorld` _scenecapturecamera) (`self.K2_GetActorLocation` (`|ConvertAsset` (`self.TargetActor`)))))
            (set `local.AspectRatio` (/ (`KismetMathLibrary.Conv_IntToDouble` (`TextureRenderTarget2D.SizeX` _output_get)) (`KismetMathLibrary.Conv_IntToDouble` (`TextureRenderTarget2D.SizeY` _output_get))))
            (bind _output_get_2 (set `local.HalfHorizontalFOV` (`KismetMathLibrary.DegreesToRadians` (* (`SceneCaptureComponent2D.FOVAngle` (`self.SceneCaptureCamera`)) 0.5))))
            (set `local.AllowedHorizontalAngle` (* _output_get_2 _trackingmargin))
            (bind _output_get_3 (set `local.HalfVerticalFOV` (`KismetMathLibrary.Atan` (/ (`KismetMathLibrary.Tan` _output_get_2) (`local.AspectRatio`)))))
            (set `local.AllowedVerticalAngle` (* _output_get_3 _trackingmargin))
            (set `local.HorizontalAngle` (`KismetMathLibrary.Atan2` _cameraspacelocation_y _cameraspacelocation_x))
            (set `local.VerticalAngle` (`KismetMathLibrary.Atan2` _cameraspacelocation_z _cameraspacelocation_x)))
          (:`then_1`
            (if (not (and (<= (`KismetMathLibrary.Abs` (`local.HorizontalAngle`)) (`local.AllowedHorizontalAngle`)) (<= (`KismetMathLibrary.Abs` (`local.VerticalAngle`)) (`local.AllowedVerticalAngle`))))
              (set `local.bTrackingTarget` false))))
        (else
          (set `local.bTrackingTarget` false))))
    (:`then_1`
      (return (`local.bTrackingTarget`)))))

(fn `ConvertLocationToScreenPosition`
  (params (Location :type "Vector Structure"))
  (returns (RelativePosition :type "Vector2D Structure") (AbsolutePosition :type "Vector2D Structure"))
  (locals (CamreaSpace :type "Vector Structure") (AspectRatio :type "Float (double-precision)") (HalfHorizontalFOV :type "Float (double-precision)" :default 0.0) (HalfVerticalFOV :type "Float (double-precision)" :default 0.0) (HorizontalAngle :type "Float (double-precision)") (VerticalAngle :type "Float (double-precision)") (ScreenX :type "Float (double-precision)") (ScreenY :type "Float (double-precision)"))
  (bind (_camreaspace_x _camreaspace_y _camreaspace_z) (`KismetMathLibrary.BreakVector` (`local.CamreaSpace`)))
  (bind (_camreaspace_x_2 _camreaspace_y_2) (`KismetMathLibrary.BreakVector` (`local.CamreaSpace`)))
  (bind _screenx (`local.ScreenX`))
  (bind _texturetarget (`SceneCaptureComponent2D.TextureTarget` (`self.SceneCaptureCamera`)))
  (bind _texturetarget_2 (`SceneCaptureComponent2D.TextureTarget` (`self.SceneCaptureCamera`)))
  (bind _output_get (set `local.CamreaSpace` (`KismetMathLibrary.InverseTransformLocation` (`SceneComponent.K2_GetComponentToWorld` (`self.SceneCaptureCamera`)) Location)))
  (if (<= (`KismetMathLibrary.BreakVector3f` _output_get) 0.0)
    (return (0.0 0.0) (0.0 0.0))
    (else
      (`|ExecutionSequence`
        (:`then_0`
          (set `local.HalfHorizontalFOV` (`KismetMathLibrary.DegreesToRadians` (* (`SceneCaptureComponent2D.FOVAngle` (`self.SceneCaptureCamera`)) 0.5)))
          (`/Engine/EditorBlueprintResources/StandardMacros.IsValid` _texturetarget
            (:`Is Valid`
              (set `local.AspectRatio` (/ (`KismetMathLibrary.Conv_IntToDouble` (`TextureRenderTarget2D.SizeX` _texturetarget)) (`KismetMathLibrary.Conv_IntToDouble` (`TextureRenderTarget2D.SizeY` _texturetarget))))
              (set `local.HalfVerticalFOV` (`KismetMathLibrary.Atan` (/ (`KismetMathLibrary.Tan` (`local.HalfHorizontalFOV`)) (`local.AspectRatio`))))
              (set `local.HorizontalAngle` (`KismetMathLibrary.DegAtan2` _camreaspace_y_2 _camreaspace_x_2))
              (set `local.VerticalAngle` (`KismetMathLibrary.DegAtan2` _camreaspace_z _camreaspace_x))
              (set `local.ScreenX` (/ (`KismetMathLibrary.DegTan` (`local.HorizontalAngle`)) (`KismetMathLibrary.Tan` (`local.HalfHorizontalFOV`))))
              (set `local.ScreenY` (/ (`KismetMathLibrary.DegTan` (`local.VerticalAngle`)) (`KismetMathLibrary.Tan` (`local.HalfVerticalFOV`)))))))
        (:`then_1`
          (return (`KismetMathLibrary.MakeVector2D` _screenx (`local.ScreenY`)) (`KismetMathLibrary.MakeVector2D` (* _screenx (`KismetMathLibrary.Conv_IntToDouble` (`TextureRenderTarget2D.SizeX` _texturetarget_2))) (* (`local.ScreenY`) (`KismetMathLibrary.Conv_IntToDouble` (`TextureRenderTarget2D.SizeY` _texturetarget_2)) -1.0))))))))

(fn `FindCameraTarget`
  (returns (Found :type Boolean))
  (locals (Rotation :type "Rotator Structure" :default (struct)) (TempRotation :type "Rotator Structure" :default (struct)) (Transform :type "Transform Structure") (TraceHit :type Boolean :default false) (HitResult :type "HitResult Structure"))
  (bind (_returnvalue_roll _returnvalue_pitch) (`KismetMathLibrary.BreakRotator` (`SceneComponent.K2_GetComponentRotation` (`self.CameraRoot`))))
  (bind _hitresult (`self.GetCameraTrace`))
  (bind _output_get (set `local.HitResult` _hitresult))
  (bind (_bblockinghit _binitialoverlap _time _distance _location _impactpoint _normal _impactnormal _physmat _hitactor) (`GameplayStatics.BreakHitResult` _output_get))
  ;[1 1 1] Track
  (if _bblockinghit
    (set `self.TargetActor` (`|ConvertAsset` _hitactor))
    (set `self.TargetOffset` (- _impactpoint (`self.K2_GetActorLocation` _hitactor)))
    (set `self.TrackingLocation` _impactpoint)
    (set `self.CurrentPitch` _returnvalue_pitch)
    (set `self.CurrentYaw` 0.0)
    (`self.TrackRotateToTarget`)
    (`self.UpdateCamera`)
    (return true)
    (else
      (return false))))

(fn `GetCameraForwardLocation`
  (params (Distance :type "Float (double-precision)" :default 100.0))
  (returns (Location :type "Vector Structure"))
  (bind _cameraroot (`self.CameraRoot`))
  (return (+ (`SceneComponent.K2_GetComponentLocation` _cameraroot) (* (`SceneComponent.GetForwardVector` _cameraroot) Distance))))

(fn `GetCameraTrace`
  (returns (HitResult :type "HitResult Structure"))
  (bind (_start _end _radius) (`self.CameraTraceVectors` 400.0 8000.0 120.0))
  (bind (_start_2 _end_2 _radius_2) (`self.CameraTraceVectors` 8000.0 20000.0 300.0 0.8))
  (bind (_start_3 _end_3 _radius_3) (`self.CameraTraceVectors` 400.0 4000.0 200.0))
  (bind (_start_4 _end_4 _radius_4) (`self.CameraTraceVectors` 4000.0 8000.0 600.0 0.6))
  (bind (_start_5 _end_5 _radius_5) (`self.CameraTraceVectors` 8000.0 20000.0 1200.0 0.3))
  (bind _trackingtype (`self.TrackingType`))
  (bind _ignoredactors (`self.IgnoredActors`))
  (bind _ignoredactors_2 (`self.IgnoredActors`))
  ;[1 1 1] Trace by objects
  (bind (_outhit _returnvalue) (`KismetSystemLibrary.SphereTraceSingleForObjects` _start_3 _end_3 _radius_3 _trackingtype false _ignoredactors_2 "None" true (struct :`R` 1.0 :`A` 1.0) (struct :`G` 1.0 :`A` 1.0) 2.0))
  (if _returnvalue
    (return _outhit)
    (else
      (bind (_outhit_2 _returnvalue_2) (`KismetSystemLibrary.SphereTraceSingleForObjects` _start_4 _end_4 _radius_4 _trackingtype false _ignoredactors_2 "None" true (struct :`R` 1.0 :`A` 1.0) (struct :`G` 1.0 :`A` 1.0) 2.0))
      (if _returnvalue_2
        (return _outhit_2)
        (else
          (bind (_outhit_3 _returnvalue_3) (`KismetSystemLibrary.SphereTraceSingleForObjects` _start_5 _end_5 _radius_5 _trackingtype false _ignoredactors_2 "None" true (struct :`R` 1.0 :`A` 1.0) (struct :`G` 1.0 :`A` 1.0) 2.0))
          (if _returnvalue_3
            (return _outhit_3)
            (else
              ;[1 1 1] Trace by Visibility
              (bind (_outhit_4 _returnvalue_4) (`KismetSystemLibrary.SphereTraceSingle` _start _end _radius "TraceTypeQuery1" false _ignoredactors "None" true (struct :`R` 1.0 :`A` 1.0) (struct :`G` 1.0 :`A` 1.0) 2.0))
              (if _returnvalue_4
                (return _outhit_4)
                (else
                  (bind _outhit_5 (`KismetSystemLibrary.SphereTraceSingle` _start_2 _end_2 _radius_2 "TraceTypeQuery1" false _ignoredactors "None" true (struct :`R` 1.0 :`A` 1.0) (struct :`G` 1.0 :`A` 1.0) 2.0))
                  (return _outhit_5))))))))))

(fn `GetTargetDistance`
  (returns (Distance :type "Float (double-precision)") (IsTracking :type Boolean))
  (bind _istracking (`self.IsTracking`))
  (return (`KismetMathLibrary.SelectFloat` (`KismetMathLibrary.Vector_Distance` (`self.K2_GetActorLocation`) (`self.TrackingLocation`)) 0.0 _istracking) _istracking))

(fn `GetTextureTargetSize`
  (returns (SizeX :type "Float (double-precision)") (SizeY :type "Float (double-precision)"))
  (bind _texturetarget (`SceneCaptureComponent2D.TextureTarget` (`self.SceneCaptureCamera`)))
  (return (`KismetMathLibrary.Conv_IntToDouble` (`TextureRenderTarget2D.SizeX` _texturetarget)) (`KismetMathLibrary.Conv_IntToDouble` (`TextureRenderTarget2D.SizeY` _texturetarget))))

(fn `ToggleTrackingMode`
  (params (toggle :type Boolean))
  (returns (isTracking :type Boolean))
  (locals (NewRotation :type "Rotator Structure" :default (struct)) (AttachedActor :type "Actor Object Reference"))
  (bind _istracking (`self.IsTracking`))
  (bind _trackroot (`self.TrackRoot`))
  (bind (_returnvalue_location _returnvalue_rotation) (`KismetMathLibrary.BreakTransform` (`KismetMathLibrary.MakeRelativeTransform` (`SceneComponent.K2_GetComponentToWorld` _trackroot) (`SceneComponent.K2_GetComponentToWorld` (`self.Attached_Ref`)))))
  (`|ExecutionSequence`
    (:`then_0`
      (if toggle
        (bind _found (`self.FindCameraTarget`))
        (if _found
          (set `self.IsTracking` true)
          (set `self.SkipFrame` 1)
          (set `self.WorldMode` false))
        (else
          (set `self.IsTracking` false)
          (set `self.TargetActor` null)
          (`self.ED_OnTrackingStopped`)
          (`|ExecutionSequence`
            (:`then_0`
              (`/Engine/EditorBlueprintResources/StandardMacros.IsValid` (`self.Attached_Ref`)
                (:`Is Valid`
                  (set `local.NewRotation` (`KismetMathLibrary.MakeRotator` 0.0 (.pitch _returnvalue_rotation) (.yaw _returnvalue_rotation))) ; Relative Rotation
                )
                (:`Is Not Valid`
                  (set `local.NewRotation` (`SceneComponent.K2_GetComponentRotation` _trackroot)) ; World Rotation
                )))
            (:`then_1`
              (`SceneComponent.K2_SetRelativeRotation` _trackroot (`local.NewRotation`) false false))))))
    (:`then_1`
      (`SceneComponent.SetAbsolute` (`self.TrackRoot`) false (`self.IsTracking`) false)
      (`SceneComponent.SetAbsolute` (`self.CameraRoot`) false (not (`self.IsTracking`)) false)
      (if _istracking
        (return _istracking)
        (else
          (`self.ToggleWorldMode` true))))))

(fn `ToggleWorldMode`
  (params (toggle :type Boolean))
  (locals (TempRotation :type "Rotator Structure" :default (struct)))
  (bind _cameraroot (`self.CameraRoot`))
  (bind _temprotation (`local.TempRotation`))
  (bind (_returnvalue_location _returnvalue_rotation) (`KismetMathLibrary.BreakTransform` (`KismetMathLibrary.MakeRelativeTransform` (`SceneComponent.K2_GetComponentToWorld` (`self.CameraRoot`)) (`SceneComponent.K2_GetComponentToWorld` (`self.TrackRoot`)))))
  (if (!= (`self.WorldMode`) toggle)
    (bind _output_get (set `self.WorldMode` toggle))
    (`|ExecutionSequence`
      (:`then_0`
        (set `local.TempRotation` (`SceneComponent.K2_GetComponentRotation` (`self.CameraRoot`)))
        (if _output_get
          (if (`self.IsTracking`)
            (`self.ToggleTrackingMode` false))
          (`SceneComponent.SetAbsolute` _cameraroot false true false)
          (`SceneComponent.K2_SetWorldRotation` _cameraroot _temprotation false false)
          (else
            (`SceneComponent.SetAbsolute` (`self.CameraRoot`) false false false)
            (`SceneComponent.K2_SetWorldRotation` _cameraroot _temprotation false false)
            (set `self.CurrentPitch` (.pitch _returnvalue_rotation))
            (set `self.CurrentYaw` (.yaw _returnvalue_rotation))))))))

(fn `TrackRotateToTarget`
  (bind _output (`|ConvertAsset` (`self.TargetActor`)))
  (bind _returnvalue (+ (`self.TargetOffset`) (`self.K2_GetActorLocation` _output)))
  (bind (_returnvalue_roll _returnvalue_pitch _returnvalue_yaw) (`KismetMathLibrary.BreakRotator` (`KismetMathLibrary.FindLookAtRotation` (`SceneComponent.K2_GetComponentLocation` (`self.TrackRoot`)) _returnvalue)))
  (`/Engine/EditorBlueprintResources/StandardMacros.IsValid` _output
    (:`Is Valid`
      (`SceneComponent.K2_SetWorldRotation` (`self.TrackRoot`) (`KismetMathLibrary.MakeRotator` 0.0 _returnvalue_pitch _returnvalue_yaw) false false)
      (set `self.TrackingLocation` _returnvalue)
      (return))
    (:`Is Not Valid`
      (return))))

(fn `UpdateCamera`
  (bind (_returnvalue_roll _returnvalue_pitch _returnvalue_yaw) (`KismetMathLibrary.BreakRotator` (`SceneComponent.K2_GetComponentRotation` (`self.TrackRoot`))))
  (if (`self.IsTracking`)
    (`SceneComponent.K2_SetWorldRotation` (`self.CameraRoot`) (`KismetMathLibrary.MakeRotator` 0.0 (`self.CurrentPitch`) (+ _returnvalue_yaw (`self.CurrentYaw`))) false false :!label _label)
    (elif (not (`self.WorldMode`))
      (goto _label))))

(fn `UserConstructionScript`
  (set `SceneCaptureComponent2D.TextureTarget` (`self.TextureTarget_Ref`) (`self.SceneCaptureCamera`)))