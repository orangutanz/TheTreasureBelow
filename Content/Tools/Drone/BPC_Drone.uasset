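; Actor component that makes its owner a player-flyable drone with replicated movement, a control panel widget and a camera tracker.
; Server RPCs set control input; Tick interpolates pitch and roll, while the server applies yaw and drives a runtime-added, gravity-free ProjectileMovement.
; Velocity blends thrust and custom gravity in arcade or tilt-driven mode, with a downward trace halting descent.
; The camera tracker spawns only on the owning non-server client.
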(event `self.ReceiveEndPlay`
  (params (EndPlayReason :type "EEndPlayReason Enum" :default "Destroyed"))
  (bind _projectilemovement (`self.ProjectileMovement`))
  (bind _controlwbp (`self.ControlWBP`))
  (bind _cameratrackerref (`self.CameraTrackerRef`))
  (`|ExecutionSequence`
    (:`then_0`
      (`/Engine/EditorBlueprintResources/StandardMacros.IsValid` _projectilemovement
        (:`Is Valid`
          (`self.K2_DestroyComponent` _projectilemovement)
          (set `self.ProjectileMovement` null))))
    (:`then_1`
      (`/Engine/EditorBlueprintResources/StandardMacros.IsValid` _controlwbp
        (:`Is Valid`
          (`Widget.RemoveFromParent` _controlwbp)
          (set `self.ControlWBP` null))))
    (:`then_2`
      (`/Engine/EditorBlueprintResources/StandardMacros.IsValid` _cameratrackerref
        (:`Is Valid`
          (`Actor.K2_DestroyActor` _cameratrackerref)
          (set `self.CameraTrackerRef` null))))))

(event `self.ReceiveBeginPlay`
  (`self.Initialize`))

(event `self.ReceiveTick`
  (params (DeltaSeconds :type "Float (single-precision)"))
  (if (`self.ManualControl`)
    (`self.InterpControlMomvemnt`)))

(event `SERVER_ToggleControl`
  (params (Toggle :type Boolean))
  (set `self.ManualControl` Toggle))

(event `SERVER_InputControl`
  (params (ControlVector :type "Vector Structure") (Throttle :type "Float (double-precision)"))
  (set `self.ControlVector` ControlVector)
  (set `self.Throttle` Throttle))

(fn `Initialize`
  (bind _returnvalue (`self.GetOwner`))
  (bind _returnvalue_2 (`self.GetOwner`))
  (bind _returnvalue_3 (`Actor.GetOwner` _returnvalue_2))
  (bind _rootcomponent (`Actor.RootComponent` _returnvalue_3))
  (bind (_returnvalue_location _returnvalue_rotation _returnvalue_scale) (`KismetMathLibrary.BreakTransform` (`SceneComponent.K2_GetComponentToWorld` _rootcomponent)))
  (`Actor.SetReplicateMovement` _returnvalue_2 true)
  (if (`KismetSystemLibrary.IsServer`)
    (bind _returnvalue_4 (`|AddComponentByClass` _returnvalue "/Script/Engine.ProjectileMovementComponent"))
    (bind _output_get (set `self.ProjectileMovement` _returnvalue_4))
    (`MovementComponent.SetUpdatedComponent` _output_get (`Actor.RootComponent` _returnvalue))
    (set `ProjectileMovementComponent.ProjectileGravityScale` 0.0 _output_get)
    (set `ProjectileMovementComponent.bInterpRotation` true _returnvalue_4)
    (elif (== _returnvalue_3 (`GameplayStatics.GetPlayerPawn` 0))
      (bind _returnvalue_5 (`|SpawnActorFromClass` "/Game/Tools/Drone/BP_CameraTracker.BP_CameraTracker_C" (`KismetMathLibrary.MakeTransform` (+ _returnvalue_location (0.0 0.0 -50.0)) _returnvalue_rotation _returnvalue_scale) "Undefined" "MultiplyWithRoot" null null (`|MakeArray` _returnvalue_3) _rootcomponent (`|MakeArray` "ObjectTypeQuery3" :!type "EObjectTypeQuery Enum") -86.0 30.0 0.6 1.0 null))
      (set `self.CameraTrackerRef` _returnvalue_5))))

(fn `InterpControlMomvemnt`
  (locals (ThrustAcceleration :type "Float (double-precision)" :default 0.0))
  (bind _returnvalue (`GameplayStatics.GetWorldDeltaSeconds`))
  (bind _returnvalue_2 (`GameplayStatics.GetWorldDeltaSeconds`))
  (bind _returnvalue_3 (`self.GetOwner`))
  (bind _returnvalue_4 (`GameplayStatics.GetWorldDeltaSeconds`))
  (bind (_controlvector_x _controlvector_y) (`KismetMathLibrary.BreakVector` (`self.ControlVector`)))
  (bind _projectilemovement (`self.ProjectileMovement`))
  (bind _projectilemovement_2 (`self.ProjectileMovement`))
  (bind _projectilemovement_3 (`self.ProjectileMovement`))
  (bind _thrustacceleration (`local.ThrustAcceleration`))
  (bind (_x _y _z) (`KismetMathLibrary.BreakVector3f` (`self.ControlVector`)))
  (bind (_x_2 _y_2) (`KismetMathLibrary.BreakVector3f` (`self.ControlVector`)))
  (bind _rootcomponent (`Actor.RootComponent` (`self.GetOwner`)))
  (bind (_velocity_x _velocity_y) (`KismetMathLibrary.BreakVector` (`MovementComponent.Velocity` _projectilemovement)))
  (bind _velocity (`MovementComponent.Velocity` _projectilemovement_2))
  (bind _velocity_2 (`MovementComponent.Velocity` _projectilemovement_3))
  (bind _rootcomponent_2 (`Actor.RootComponent` (`self.GetOwner`)))
  (bind _returnvalue_5 (`SceneComponent.K2_GetComponentLocation` (`Actor.RootComponent` _returnvalue_3)))
  (bind (_relativerotation_roll _relativerotation_pitch) (`KismetMathLibrary.BreakRotator` (`SceneComponent.RelativeRotation` _rootcomponent_2)))
  (bind (_returnvalue_x _returnvalue_y _returnvalue_z) (`KismetMathLibrary.BreakVector` (+ (`KismetMathLibrary.MakeVector` 0.0 0.0 (`self.GravityAcceleration`)) (* (`SceneComponent.GetUpVector` (`Actor.RootComponent` (`self.GetOwner`))) (`local.ThrustAcceleration`)))))
  (bind (_returnvalue_x_2 _returnvalue_y_2) (`KismetMathLibrary.BreakVector` (`KismetMathLibrary.VInterpTo` _velocity (+ (* (`SceneComponent.GetForwardVector` _rootcomponent) _controlvector_x _thrustacceleration) (* (`SceneComponent.GetRightVector` _rootcomponent) _controlvector_y _thrustacceleration)) _returnvalue 4.0)))
  (bind _returnvalue_6 (`KismetMathLibrary.MakeVector` _returnvalue_x _returnvalue_y _returnvalue_z))
  (bind (_returnvalue_x_3 _returnvalue_y_3 _returnvalue_z_2) (`KismetMathLibrary.BreakVector` (`KismetMathLibrary.VInterpTo` _velocity (+ (`KismetMathLibrary.MakeVector` 0.0 0.0 (`self.GravityAcceleration`)) (* (`SceneComponent.GetUpVector` _rootcomponent) (`local.ThrustAcceleration`))) _returnvalue 2.0)))
  (bind (_returnvalue_x_4 _returnvalue_y_4 _returnvalue_z_3) (`KismetMathLibrary.BreakVector` (`KismetMathLibrary.VInterpTo` _velocity_2 _returnvalue_6 _returnvalue_4 2.0)))
  (bind (_returnvalue_x_5 _returnvalue_y_5) (`KismetMathLibrary.BreakVector` (`KismetMathLibrary.VInterpTo` _velocity_2 _returnvalue_6 _returnvalue_4 4.0)))
  ;[1 1 1] Rotate
  (`SceneComponent.K2_SetRelativeRotation` _rootcomponent_2 (`KismetMathLibrary.MakeRotator` (`KismetMathLibrary.FInterpTo` _relativerotation_roll (* _y_2 (`self.MaxRollAngle`)) _returnvalue_2 4.0) (`KismetMathLibrary.FInterpTo` _relativerotation_pitch (* (`self.MaxPitchAngle`) _x_2) _returnvalue_2 4.0)) false false)
  (if (`KismetSystemLibrary.IsServer`)
    (`|ExecutionSequence`
      (:`then_0`
        ;[1 1 1] Rotation
        (if (> (`KismetMathLibrary.Abs` _z) 0.08)
          (`Actor.K2_AddActorWorldRotation` (`self.GetOwner`) (`KismetMathLibrary.MakeRotator` 0.0 0.0 (* _z (`GameplayStatics.GetWorldDeltaSeconds`) 60.0)) false false)))
      (:`then_1`
        (set `local.ThrustAcceleration` (`KismetMathLibrary.Lerp` 0.0 (`self.MaxThrustAcceleration`) (`self.Throttle`))) ; Speed
        (if (`self.ArcadeMode`)
          ;[1 1 1] Arcade Velocity
          (set `MovementComponent.Velocity` (`KismetMathLibrary.MakeVector` _returnvalue_x_2 _returnvalue_y_2 _returnvalue_z_2) _projectilemovement_2)
          (else
            ;[1 1 1] Drone Velocity
            (set `MovementComponent.Velocity` (`KismetMathLibrary.MakeVector` _returnvalue_x_5 _returnvalue_y_5 _returnvalue_z_3) _projectilemovement_3))))
      (:`then_2`
        ;[1 1 1] Stop dropping if something below
        (if (< (`.Z` (`KismetMathLibrary.BreakVector3f` (`MovementComponent.Velocity` _projectilemovement))) 0.0)
          (bind (_outhit _returnvalue_7) (`KismetSystemLibrary.LineTraceSingle` _returnvalue_5 (+ _returnvalue_5 (0.0 0.0 -50.0)) "TraceTypeQuery1" false (`|MakeArray` _returnvalue_3)))
          (if _returnvalue_7
            (bind (_returnvalue_x_6 _returnvalue_y_6 _returnvalue_z_4) (`KismetMathLibrary.BreakVector` (- (`.Location` (`GameplayStatics.BreakHitResult` _outhit)) (+ _returnvalue_5 (`KismetMathLibrary.MakeVector` 0.0 0.0 (* (.z (`.BoxExtent` (`Actor.GetActorBounds` _returnvalue_3 false false))) 0.5))))))
            (set `MovementComponent.Velocity` (`KismetMathLibrary.MakeVector` _velocity_x _velocity_y (`KismetMathLibrary.FMax` _returnvalue_z_4)) _projectilemovement) ; Stop dropping
          ))))))

(fn `Toggle UI`
  (params (Toggle :type Boolean))
  (returns (WBP_Control :type "/Game/Tools/Drone/WBP_ControlPanel Object Reference") (BP_CameraTrackerRef :type "/Game/Tools/Drone/BP_CameraTracker Object Reference"))
  (bind _controlwbp (`self.ControlWBP`))
  (if (!= (`self.ToggleWidget`) Toggle)
    (bind _output_get (set `self.ToggleWidget` Toggle))
    (`|ExecutionSequence`
      (:`then_0`
        (if _output_get
          (`/Engine/EditorBlueprintResources/StandardMacros.IsValid` _controlwbp
            (:`Is Valid`
              _)
            (:`Is Not Valid`
              (bind _returnvalue (`|CreateWidget` "/Game/Tools/Drone/WBP_ControlPanel.WBP_ControlPanel_C"))
              (set `self.ControlWBP` _returnvalue)))
          (return (`self.ControlWBP`) (`self.CameraTrackerRef`))
          (else
            (`/Engine/EditorBlueprintResources/StandardMacros.IsValid` _controlwbp
              (:`Is Valid`
                (`Widget.RemoveFromParent` _controlwbp))
              (:`Is Not Valid`
                _))
            (return (`self.ControlWBP`) (`self.CameraTrackerRef`)))))
      (:`then_1`
        (return (`self.ControlWBP`) (`self.CameraTrackerRef`))))))