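; BP_Camera is a main menu camera actor that glides between two framings selected through MoveCamera.
; One framing matches the PlayerStart transform; the other sits in front of the player character, slightly below its location, looking back at it.
; Each Tick recomputes the target for the current CameraType, then eases location and rotation toward it with interpolation.
; BeginPlay caches both actors and a BP_Door, which is otherwise unused here.
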(event `self.ReceiveBeginPlay`
  (bind _returnvalue (`GameplayStatics.GetActorOfClass` "/Script/Engine.PlayerStart"))
  (set `self.PlayerStart` _returnvalue)
  (bind _returnvalue_2 (`GameplayStatics.GetActorOfClass` "/Game/Core/Blueprints/BP_PlayerCharacter.BP_PlayerCharacter_C"))
  (set `self.PlayerCharactor` _returnvalue_2)
  (bind _returnvalue_3 (`GameplayStatics.GetActorOfClass` "/Game/Core/Blueprints/LevelDesign/BP_Door.BP_Door_C"))
  (set `self.Door` _returnvalue_3))

(event `self.ReceiveTick`
  (params (DeltaSeconds :type "Float (single-precision)"))
  (bind (_returnvalue_location _returnvalue_rotation) (`KismetMathLibrary.BreakTransform` (`self.GetTransform`)))
  (bind _playercharactor (`self.PlayerCharactor`))
  (bind _returnvalue (`self.K2_GetActorLocation` _playercharactor))
  (bind _returnvalue_2 (+ _returnvalue (* (`self.GetActorForwardVector` _playercharactor) 250.0) (0.0 0.0 -15.0)))
  (`|ExecutionSequence`
    (:`then_0`
      (switch `int` (`self.CameraType`)
        (:`0`
          (set `self.Target` (`self.GetTransform` (`self.PlayerStart`))))
        (:`1`
          (set `self.Target` (`KismetMathLibrary.MakeTransform` _returnvalue_2 (`KismetMathLibrary.FindLookAtRotation` _returnvalue_2 _returnvalue))))))
    (:`then_1`
      (`self.K2_SetActorTransform` (`KismetMathLibrary.MakeTransform` (`KismetMathLibrary.VInterpTo` _returnvalue_location (.location (`self.Target`)) DeltaSeconds 4.0) (`KismetMathLibrary.RInterpTo` _returnvalue_rotation (.rotation (`self.Target`)) DeltaSeconds 4.0))))))

(fn `MoveCamera`
  (params (PositionType :type Integer))
  (set `self.CameraType` PositionType))

(fn `UserConstructionScript`
  (set `self.Target` (`self.GetTransform`)))