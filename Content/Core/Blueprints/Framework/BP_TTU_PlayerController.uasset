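; TTU player controller that handles cursor input mode and player interaction with actors.
; On BeginPlay it adds the default Enhanced Input mapping context for the local controller.
; A toggle event switches between Game and UI input with a visible cursor and game-only input.
; Selected interactable actors pass a squared-distance check from the pawn before a server event sends them the interface message, with no range recheck there.
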(event `/Game/Core/Blueprints/Interface/BPI_PlayerController.ToggleInputMode`
  (params (ToggleCursor :type Boolean))
  ;[1 1 1] Toggle Input
  (if ToggleCursor
    (`WidgetBlueprintLibrary.SetInputMode_GameAndUIEx` self null "DoNotLock" true true)
    (set `self.bShowMouseCursor` true)
    (else
      (`WidgetBlueprintLibrary.SetInputMode_GameOnly` self)
      (set `self.bShowMouseCursor` false))))

(event `/Game/Core/Blueprints/Interface/BPI_PlayerController.InteractActorOnServer`
  (params (SelectActor :type "Actor Object Reference"))
  ;[1 1 1] Interaction
  (cast `/Game/Core/Blueprints/Interface/BPI_Interactable` SelectActor)
  (if (< (`self.GetSquaredDistanceTo` SelectActor (`self.K2_GetPawn`)) 66000.0)
    (`self.SERVER_InteracteActor` SelectActor)))

(event `SERVER_InteracteActor`
  (params (Actor :type "Actor Object Reference"))
  ;[1 1 1] Interaction
  (message `/Game/Core/Blueprints/Interface/BPI_Interactable.Server_Interaction` Actor self))

(event `self.ReceiveBeginPlay`
  (if (`self.IsLocalPlayerController`)
    (`EnhancedInputSubsystemInterface.AddMappingContext` (subsystem `EnhancedInputLocalPlayerSubsystem`) "/Game/Core/Input/IMC_Default.IMC_Default" 0 (struct))))

(fn `UserConstructionScript`)