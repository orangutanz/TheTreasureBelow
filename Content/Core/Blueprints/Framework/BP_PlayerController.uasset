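; Core player controller that handles input mode, server-routed interaction and ambient audio.
; On BeginPlay, the local controller adds the default Enhanced Input mapping context, switches to game-only input and starts a 2D dungeon cave ambience.
; A toggle event switches between cursor-visible game-and-UI input and cursor-hidden game-only input.
; Interaction checks the selected actor for BPI_Interactable, then forwards it through a server event that messages the actor with this controller.
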(event `/Game/Core/Blueprints/Interface/BPI_PlayerController.ToggleInputMode`
  (params (ToggleCursor :type Boolean))
  ;[1 1 1] Toggle Input
  (if ToggleCursor
    (`WidgetBlueprintLibrary.SetInputMode_GameAndUIEx` self null "LockInFullscreen" true true)
    (set `self.bShowMouseCursor` true)
    (else
      (`WidgetBlueprintLibrary.SetInputMode_GameOnly` self)
      (set `self.bShowMouseCursor` false))))

(event `/Game/Core/Blueprints/Interface/BPI_PlayerController.InteractActorOnServer`
  (params (SelectActor :type "Actor Object Reference"))
  ;[1 1 1] Interaction
  (cast `/Game/Core/Blueprints/Interface/BPI_Interactable` SelectActor)
  (`self.SERVER_InteracteActor` SelectActor))

(event `SERVER_InteracteActor`
  (params (Actor :type "Actor Object Reference"))
  ;[1 1 1] Interaction
  (message `/Game/Core/Blueprints/Interface/BPI_Interactable.Server_Interaction` Actor self))

(event `self.ReceiveBeginPlay`
  (if (`self.IsLocalPlayerController`)
    (`EnhancedInputSubsystemInterface.AddMappingContext` (subsystem `EnhancedInputLocalPlayerSubsystem`) "/Game/Core/Input/IMC_Default.IMC_Default" 0 (struct))
    (`/Game/Core/Blueprints/Interface/BPI_PlayerController.ToggleInputMode` false)
    (bind _returnvalue (`GameplayStatics.CreateSound2D` "/Game/Audio/SmallSoundKit/SSKWav/AmbienceWav/Amb_DungeCave_Generic_01.Amb_DungeCave_Generic_01" 1.0 1.0 0.0 null false false))
    (bind _output_get (set `self.AmbientSound` _returnvalue))
    (`ActorComponent.SetActive` _output_get true false)))

(fn `UserConstructionScript`)