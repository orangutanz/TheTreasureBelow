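; Game mode that handles item drops, safe-point respawns, player death and winning the game.
; Dropped items spawn as BP_Item_Pickup, thrown along the control rotation when coming from a player.
; Respawn and death, which also fires OnPlayerDead, teleport the pawn near the latest safepoint, retrying navmesh picks, or to PlayerStart.
; Winning awards DefeatBoss and returns clients to menu, or destroys the session first when only one controller exists.
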(event `/Game/Core/Blueprints/Framework/BPI_GameMode.DropItem`
  (params (Actor :type "Actor Object Reference") (ItemInfo :type "ItemInfo Structure") (`FromPlayer?` :type Boolean))
  (bind (_origin _boxextent) (`self.GetActorBounds` Actor false false))
  ;[1 1 1] Drop Item
  (bind _returnvalue (`|SpawnActorFromClass` "/Game/Core/Blueprints/LevelBP/BP_Item_Pickup.BP_Item_Pickup_C" (`KismetMathLibrary.MakeTransform` (`KismetMathLibrary.SelectVector` (+ (`self.K2_GetActorLocation` Actor) (`KismetMathLibrary.MakeVector` 0.0 0.0 (`KismetMathLibrary.RandomFloatInRange` 50.0 70.0))) (+ _origin (`KismetMathLibrary.MakeVector` 0.0 0.0 (+ (* (.z _boxextent) 3.0) 20.0))) `FromPlayer?`) (`KismetMathLibrary.RandomRotator` false)) "AdjustIfPossibleButAlwaysSpawn" "OverrideRootScale" null true ItemInfo null))
  (if `FromPlayer?`
    (bind _ascharacter (cast `Character` Actor))
    (`PrimitiveComponent.AddImpulse` (`/Game/Core/Blueprints/LevelBP/BP_Item_Pickup.StaticMesh` _returnvalue) (`KismetMathLibrary.MakeVector` (.x (* (`KismetMathLibrary.GetForwardVector` (`Pawn.GetControlRotation` _ascharacter)) 500.0)) (.y (* (`KismetMathLibrary.GetForwardVector` (`Pawn.GetControlRotation` _ascharacter)) 500.0)) (`KismetMathLibrary.FMax` (.z (* (`KismetMathLibrary.GetForwardVector` (`Pawn.GetControlRotation` _ascharacter)) 500.0)) 50.0)) "None" true)))

(event `/Game/Core/Blueprints/Framework/BPI_GameMode.UpdateNewSafePoint`
  (params (NewSafepointRef :type "Actor Object Reference"))
  ;[1 1 1] Spawn Point
  (if (!= NewSafepointRef (`self.Safepoint`))
    (set `self.Safepoint` NewSafepointRef)))

(event `/Game/Core/Blueprints/Framework/BPI_GameMode.RespawnPlayerPawn`
  (params (PlayerPawn :type "Pawn Object Reference"))
  (bind _safepoint (`self.Safepoint`))
  ;[1 1 1] Spawn Point
  (`/Engine/EditorBlueprintResources/StandardMacros.IsValid` _safepoint
    (:`Is Valid`
      (bind (_randomlocation _returnvalue) (`NavigationSystemV1.K2_GetRandomLocationInNavigableRadius` (`self.K2_GetActorLocation` _safepoint) 200.0 null null :!label _label))
      (if _returnvalue
        (`self.K2_SetActorLocation` PlayerPawn (+ _randomlocation (0.0 0.0 120.0)) false true)
        (else
          (goto _label))))
    (:`Is Not Valid`
      (bind _returnvalue_2 (`GameplayStatics.GetActorOfClass` "/Script/Engine.PlayerStart"))
      (`self.K2_SetActorLocation` PlayerPawn (`self.K2_GetActorLocation` _returnvalue_2) false true)))
  (message `/Game/Core/Blueprints/Interface/BPI_Player.OnRespawn` PlayerPawn))

(event `/Game/Core/Blueprints/Framework/BPI_GameMode.WinGame`
  (bind _returnvalue (`GameplayStatics.GetNumPlayerControllers`))
  (bind _returnvalue_2 (`GameplayStatics.GetPlayerController` 0))
  ;[1 1 1] Win Game
  (if (> _returnvalue 1)
    ;;[1 1 1] Clients
    (for _index (range 1 _returnvalue)
      (bind _returnvalue_3 (`GameplayStatics.GetPlayerController` _index))
      (message `/Game/Core/Blueprints/Framework/BPI_PlayerController.UnlockAchievement` _returnvalue_3 "DefeatBoss")
      (message `/Game/Core/Blueprints/Framework/BPI_PlayerController.ReturnToMainMenu` _returnvalue_3))
    (else
      ;;[1 1 1] Server
      (`KismetSystemLibrary.Delay` 2.0)
      (`DestroySessionCallbackProxy.DestroySession` _returnvalue_2
        (:`OnSuccess`
          _)
        (:`OnFailure`
          _))
      (message `/Game/Core/Blueprints/Framework/BPI_PlayerController.UnlockAchievement` _returnvalue_2 "DefeatBoss")
      (message `/Game/Core/Blueprints/Framework/BPI_PlayerController.ReturnToMainMenu` _returnvalue_2))))

(event `/Game/Core/Blueprints/Framework/BPI_GameMode.HandleDeadPlayerPawn`
  (params (Ref :type "Pawn Object Reference"))
  (bind _safepoint (`self.Safepoint`))
  ;[1 1 1] On Player Death
  (`self.ED_OnPlayerDead` Ref)
  (`/Engine/EditorBlueprintResources/StandardMacros.IsValid` _safepoint
    (:`Is Valid`
      (bind (_randomlocation _returnvalue) (`NavigationSystemV1.K2_GetRandomLocationInNavigableRadius` (`self.K2_GetActorLocation` _safepoint) 200.0 null null :!label _label_2))
      (if _returnvalue
        (`self.K2_SetActorLocation` Ref (+ _randomlocation (0.0 0.0 120.0)) false true)
        (else
          (goto _label_2))))
    (:`Is Not Valid`
      (bind _returnvalue_2 (`GameplayStatics.GetActorOfClass` "/Script/Engine.PlayerStart"))
      (`self.K2_SetActorLocation` Ref (`self.K2_GetActorLocation` _returnvalue_2) false true)))
  (message `/Game/Core/Blueprints/Interface/BPI_Player.OnRespawn` Ref))

(fn `UserConstructionScript`)