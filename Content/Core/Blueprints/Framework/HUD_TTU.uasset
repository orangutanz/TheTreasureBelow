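; HUD that owns the player's UI and tracks the interactable actor the player looks at.
; Its construction script creates the main HUD and inventory widgets.
; Each tick, a camera sphere trace updates TargetActor, toggles its highlight message and prints its name.
; Helper functions manage open container widgets and the targeted one, show or toggle the inventory, and expose the current targets.
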(event `self.ReceiveTick`
  (params (DeltaSeconds :type "Float (single-precision)"))
  (bind _targetactor (`self.TargetActor`))
  (`self.UpdateLookatTarget`)
  (`/Engine/EditorBlueprintResources/StandardMacros.IsValid` _targetactor
    (:`Is Valid`
      (`KismetSystemLibrary.PrintText` (`KismetTextLibrary.Conv_StringToText` (`KismetSystemLibrary.GetObjectName` _targetactor)) true false (struct :`R` 0.09375 :`G` 1.0 :`B` 0.20407 :`A` 1.0) 0.0))
    (:`Is Not Valid`
      (set `self.TargetActor` null))))

(fn `AddContainerWidget`
  (params (Widget :type "UserWidget Object Reference") (Position :type "Vector2D Structure"))
  (bind _returnvalue (`KismetArrayLibrary.Array_AddUnique` (`self.ContainerWidgets`) Widget))
  (if (!= _returnvalue -1)
    (`Widget.SetRenderTranslation` Widget Position)
    (`UserWidget.AddToViewport` Widget 0)
    (set `self.TargetWidget` (`|ConvertAsset` Widget))
    (`self.ToggleInveotory` false)
    (return)))

(fn `GetInventoryWidget`
  (returns (InventoryWidget :type "UserWidget Object Reference"))
  (return (`self.InventoryWidget`)))

(fn `GetTargetActor`
  (returns (TargetActor :type "Actor Object Reference"))
  (return (`self.TargetActor`)))

(fn `GetTargetContainerWidget`
  (returns (Widget :type "UserWidget Object Reference"))
  (bind _targetwidget (`self.TargetWidget`))
  (if (`KismetSystemLibrary.IsValidSoftObjectReference` _targetwidget)
    (return (`|ConvertAsset` _targetwidget))
    (else
      (return null))))

(fn `InitializeHUD`
  (bind _returnvalue (`GameplayStatics.GetPlayerController` 0))
  (`|ExecutionSequence`
    (:`then_0`
      (bind _returnvalue_2 (`|CreateWidget` "/Game/Core/Widgets/HUD/WB_HUD.WB_HUD_C" _returnvalue))
      (bind _output_get (set `self.HUD` _returnvalue_2))
      (`UserWidget.AddToViewport` _output_get 0))
    (:`then_1`
      (bind _returnvalue_3 (`|CreateWidget` "/Game/Core/Widgets/Item/WBP_Inventory.WBP_Inventory_C" _returnvalue))
      (set `self.InventoryWidget` _returnvalue_3))))

(fn `RemoveContainerWidget`
  (params (Widget :type "UserWidget Object Reference"))
  (bind _containerwidgets (`self.ContainerWidgets`))
  (bind _returnvalue (`KismetArrayLibrary.Array_RemoveItem` _containerwidgets Widget))
  (`|ExecutionSequence`
    (:`then_0`
      (if _returnvalue
        (if (== (`self.TargetWidget`) Widget)
          (if (`KismetArrayLibrary.Array_IsEmpty` _containerwidgets)
            (`self.ToggleInveotory` false)
            (set `self.TargetWidget` null)
            (else
              (set `self.TargetWidget` (`|ConvertAsset` (`|GetArrayItem` _containerwidgets (- (`KismetArrayLibrary.Array_Length` _containerwidgets) 1)))))))))
    (:`then_1`
      (`Widget.RemoveFromParent` Widget)
      (return))))

(fn `SetTargetContainerWidget`
  (params (NewTarget :type "UserWidget Object Reference"))
  (if (>= (`KismetArrayLibrary.Array_Find` (`self.ContainerWidgets`) NewTarget) 0)
    (set `self.TargetWidget` (`|ConvertAsset` NewTarget))
    (return)))

(fn `ToggleInveotory`
  (params (DoToggle :type Boolean) (DoShow :type Boolean))
  (returns (IsShown :type Boolean))
  (bind _inventorywidget (`self.InventoryWidget`))
  (`/Engine/EditorBlueprintResources/StandardMacros.IsValid` _inventorywidget
    (:`Is Valid`
      (if DoToggle
        (if (`Widget.IsInViewport` _inventorywidget)
          _
          (else
            (`UserWidget.AddToViewport` _inventorywidget 0 :!label _label)
            (return true)))
        (elif DoShow
          (goto _label)
          (else
            _)))
      (`Widget.RemoveFromParent` _inventorywidget)
      (return false))))

(fn `UpdateLookatTarget`
  (bind _returnvalue (`GameplayStatics.GetPlayerCameraManager` 0))
  (bind _returnvalue_2 (`GameplayStatics.GetPlayerPawn` 0))
  (bind _targetactor (`self.TargetActor`))
  (bind _returnvalue_3 (`self.K2_GetActorLocation` _returnvalue))
  (bind _returnvalue_4 (`self.GetActorForwardVector` _returnvalue))
  ;[1 1 1] Highlight interactables
  (`/Engine/EditorBlueprintResources/StandardMacros.IsValid` _returnvalue_2
    (:`Is Valid`
      (bind _outhit (`KismetSystemLibrary.SphereTraceSingleForObjects` (+ _returnvalue_3 (* _returnvalue_4 50.0)) (+ _returnvalue_3 (* _returnvalue_4 600.0)) 3.0 (`|MakeArray` "ObjectTypeQuery2" "ObjectTypeQuery4" :!type "EObjectTypeQuery Enum") false (`|MakeArray` _returnvalue_2 :!type "Actor Object Reference") "None" true (struct :`R` 1.0 :`A` 1.0) (struct :`G` 1.0 :`A` 1.0) 0.1))
      (bind (_bblockinghit _binitialoverlap _time _distance _location _impactpoint _normal _impactnormal _physmat _hitactor) (`GameplayStatics.BreakHitResult` _outhit))
      (if _bblockinghit
        (`/Engine/EditorBlueprintResources/StandardMacros.IsValid` _targetactor
          (:`Is Valid`
            (if (!= _targetactor _hitactor)
              (message `/Game/Core/Blueprints/Interface/BPI_Interactable.Client_ToggleHightlight` _targetactor false)
              (bind _output_get (set `self.TargetActor` _hitactor :!label _label))
              (message `/Game/Core/Blueprints/Interface/BPI_Interactable.Client_ToggleHightlight` _output_get true)))
          (:`Is Not Valid`
            (goto _label)))
        (else
          (`/Engine/EditorBlueprintResources/StandardMacros.IsValid` _targetactor
            (:`Is Valid`
              (message `/Game/Core/Blueprints/Interface/BPI_Interactable.Client_ToggleHightlight` _targetactor false)
              (set `self.TargetActor` null))))))
    (:`Is Not Valid`
      (message `/Game/Core/Blueprints/Interface/BPI_Interactable.Client_ToggleHightlight` (`self.TargetActor`) false)
      (set `self.TargetActor` null))))

(fn `UserConstructionScript`
  (`self.InitializeHUD`))