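; Utility function library with helpers for time, random placement, direction and value mapping.
; Time difference sums DateTime components into seconds, using only the new day number when months differ.
; Location helpers pick random points ahead of an actor or around a center, the latter raised slightly in Z.
; Others convert directions to yaw or eight-way labels, and map values to a 0–1 alpha outside an excluded band.
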(fn `FL_GetDirectionName`
  (params (Direction :type "Vector Structure"))
  (returns (DirectionName :type Name))
  (bind (_returnvalue_x _returnvalue_y) (`KismetMathLibrary.BreakVector` (`KismetMathLibrary.Vector_Normal2D` Direction 0.01)))
  (bind _returnvalue (< _returnvalue_y -0.5))
  (bind _returnvalue_2 (< _returnvalue_y -0.5))
  (bind _returnvalue_3 (< _returnvalue_y -0.5))
  (if (> _returnvalue_x 0.5)
    (if (or _returnvalue_2 (> _returnvalue_y 0.5))
      (return (select `bool` _returnvalue_2 :`false` "FR" :`true` "FL" :!type "Name"))
      (else
        (return "F")))
    (elif (< _returnvalue_x -0.5)
      (if (or _returnvalue_3 (> _returnvalue_y 0.5))
        (return (select `bool` _returnvalue_3 :`false` "BR" :`true` "BL" :!type "Name"))
        (else
          (return "B")))
      (elif (or _returnvalue (> _returnvalue_y 0.5))
        (return (select `bool` _returnvalue :`false` "R" :`true` "L" :!type "Name"))
        (else
          (return "F"))))))

(fn `FL_GetRotationFromDirection`
  (params (Direction :type "Vector Structure"))
  (returns (Rotation :type "Float (double-precision)"))
  (bind (_x _y) (`KismetMathLibrary.BreakVector3f` Direction))
  (return (* (/ 180.0 (`KismetMathLibrary.GetPI`)) (`KismetMathLibrary.Atan2` _y _x))))

(fn `FL_MapToAlphaExcludeRange`
  (params (InputValue :type "Float (double-precision)") (MinExclude :type "Float (double-precision)") (MaxExclude :type "Float (double-precision)") (MinValue :type "Float (double-precision)") (MaxValue :type "Float (double-precision)"))
  (returns (Alpha :type "Float (double-precision)"))
  (locals (OffsetAmount :type "Float (double-precision)"))
  (bind _offsetamount (`local.OffsetAmount`))
  (bind _returnvalue (+ MinValue _offsetamount))
  (bind _returnvalue_2 (+ InputValue _offsetamount))
  (bind _returnvalue_3 (+ MinExclude _offsetamount))
  (bind _returnvalue_4 (+ MaxExclude _offsetamount))
  (if (< InputValue 0.0)
    (set `local.OffsetAmount` (* InputValue -1.0)))
  (if (< _returnvalue_2 _returnvalue_3)
    (return (`KismetMathLibrary.FClamp` (/ (- _returnvalue_2 _returnvalue) (- _returnvalue_3 _returnvalue)))) ; the value is less than the excluded range, map it from MinValue to MinExclude (0 to 1)
    (elif (> _returnvalue_2 _returnvalue_4)
      (return (`KismetMathLibrary.FClamp` (/ (- _returnvalue_2 _returnvalue_4) (- (+ _offsetamount MaxValue) _returnvalue_4)))) ; the value is greater than the excluded range, map it from MaxExclude to MaxValue (0 to 1)
      (else
        (return 0.0) ; the value is inside the excluded range, return 0
      ))))

(fn `FL_RandomForwardLocation`
  (params (Actor :type "Actor Object Reference") (MinDistance :type "Float (double-precision)" :default 80.0) (MaxDistance :type "Float (double-precision)" :default 200.0))
  (returns (Location :type "Vector Structure"))
  (return (+ (`Actor.K2_GetActorLocation` Actor) (* (`Actor.GetActorForwardVector` Actor) (`KismetMathLibrary.RandomFloatInRange` MinDistance MaxDistance)))))

(fn `FL_RandomLocationWithDistance`
  (params (CenterLocation :type "Vector Structure") (MinDistance :type "Float (double-precision)") (MaxDistance :type "Float (double-precision)" :default 100.0))
  (returns (NewLocation :type "Vector Structure"))
  (bind _returnvalue (`KismetMathLibrary.RandomFloatInRange` MinDistance MaxDistance))
  (bind (_x _y _z) (`KismetMathLibrary.BreakVector3f` CenterLocation))
  (bind _returnvalue_2 (* (`KismetMathLibrary.RandomFloatInRange` 0.0 360.0) (/ (`KismetMathLibrary.GetPI`) 180.0)))
  (return (`KismetMathLibrary.MakeVector` (+ (* (`KismetMathLibrary.Cos` _returnvalue_2) _returnvalue) _x) (+ _y (* (`KismetMathLibrary.Sin` _returnvalue_2) _returnvalue)) (+ _z 30.0))))

(fn `FL_TimeDifference`
  (params (OldTime :type "DateTime Structure") (NewTime :type "DateTime Structure"))
  (returns (Seconds :type Integer) (SecondsFloat :type "Float (double-precision)"))
  (locals (SecondsLeft :type Integer :default 0) (MinutesLeft :type Integer :default 0) (HoursLeft :type Integer :default 0) (DaysLeft :type Integer :default 0) (MillisecondsLeft :type Integer :default 0))
  (bind (_year _month _day _hour _minute _second _millisecond) (`KismetMathLibrary.BreakDateTime` OldTime))
  (bind (_year_2 _month_2 _day_2 _hour_2 _minute_2 _second_2 _millisecond_2) (`KismetMathLibrary.BreakDateTime` NewTime))
  (bind _returnvalue (+ (`local.SecondsLeft`) (* (`local.MinutesLeft`) 60) (* (`local.HoursLeft`) 3600) (* (`local.DaysLeft`) 86400)))
  (if (< OldTime NewTime)
    (`|ExecutionSequence`
      (:`then_0`
        (set `local.HoursLeft` (- _hour_2 _hour))
        (set `local.MinutesLeft` (- _minute_2 _minute))
        (set `local.SecondsLeft` (- _second_2 _second))
        (set `local.MillisecondsLeft` (- _millisecond_2 _millisecond))
        (if (== _month_2 _month)
          (set `local.DaysLeft` (- _day_2 _day))
          (else
            (set `local.DaysLeft` _day_2))))
      (:`then_1`
        (return _returnvalue (+ (`KismetMathLibrary.Conv_IntToDouble` _returnvalue) (* (`KismetMathLibrary.Conv_IntToDouble` (`local.MillisecondsLeft`)) 0.001)))))
    (else
      (return 0 0.0))))