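; Blueprint function library of item helpers for inventory, loot and equipment.
; Lookup functions read item, consumable and equipment rows from DataTables by ID, blocking-load icons, and map equipment types to slot indices.
; Loot generation makes a cumulative weighted pick of one table entry, rolls a quantity and splits it into max-size stacks.
; A UI helper shows the split-item widget, located by interface or created from a blocking-loaded class.
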(fn `FL_FindMatchingEquipmentIndex`
  (params (ItemInfo :type "ItemInfo Structure") (EquipmentDefinition :type "Array of Name"))
  (returns (EquipmentIndex :type "Array of Integer"))
  (bind (_st_equipment _equipmenttype _found) (`self.FL_GetEquipmentInfo` (`.ItemID` (break `ItemInfo` ItemInfo))))
  (if _found
    (switch `/Game/Core/Database/Item/Equipment/E_EquipmentType` _equipmenttype
      (:`NewEnumerator3`
        (return (`|MakeArray`)))
      (:`NewEnumerator0`
        (return (`|MakeArray` (`KismetArrayLibrary.Array_Find` EquipmentDefinition "Weapon_1") (`KismetArrayLibrary.Array_Find` EquipmentDefinition "Weapon_2"))))
      (:`NewEnumerator2`
        (return (`|MakeArray` (`KismetArrayLibrary.Array_Find` EquipmentDefinition "Backpack"))))
      (:`NewEnumerator1`
        (return (`|MakeArray` (`KismetArrayLibrary.Array_Find` EquipmentDefinition "Trinket")))))
    (else
      (return))))

(fn `FL_GenerateLootFromTable`
  (params (LootTableName :type Name))
  (returns (OutItems :type "Array of ItemInfo Structure"))
  (locals (TotalWeight :type Integer) (TargetWeight :type Integer) (LootTable_ItemArr :type "Array of Name") (LootTable_ItemWeights :type "Array of Integer") (GeneratedItems :type "Array of ItemInfo Structure") (GeneratedAmount :type Integer :default 0))
  (bind _generateditems (`local.GeneratedItems`))
  (bind _generatedamount (`local.GeneratedAmount`))
  (bind _targetweight (`local.TargetWeight`))
  (bind _returnvalue (`|GetDataTableRow` "/Game/Core/Database/Container/DT_LootTables.DT_LootTables" LootTableName)
    (:`then`
      (for _array_element (`.TableItems_3_91E1E5914842F518ED9D0F90B93BA467` (break `/Game/Core/Database/Container/ST_LootTable` _returnvalue))
        (bind (_itemname _spawnweight _minamount _maxamount) (break `/Game/Core/Database/Container/ST_RandomItem` _array_element))
        ;[1 1 1] Total Weight
        (`|GetDataTableRow` "/Game/Core/Database/Item/DT_Items.DT_Items" _itemname
          (:`then`
            (set `local.TotalWeight` (+ (`local.TotalWeight`) _spawnweight))
            (`KismetArrayLibrary.Array_Add` (`local.LootTable_ItemWeights`) _spawnweight)
            (`KismetArrayLibrary.Array_Add` (`local.LootTable_ItemArr`) _itemname))))
      ;[1 1 1] Higher spawn wieght = higer chance to spawn
      (set `local.TargetWeight` (`KismetMathLibrary.RandomIntegerInRange` 1 (`local.TotalWeight`)))
      (for (_array_element_2 _array_index) (`local.LootTable_ItemArr`)
        (bind _output (`|GetArrayItem` (`local.LootTable_ItemWeights`) _array_index))
        (if (<= _targetweight _output)
          (set `local.GeneratedAmount` (`KismetMathLibrary.RandomIntegerInRange` _minamount _maxamount))
          (bind _returnvalue_2 (`|GetDataTableRow` "/Game/Core/Database/Item/DT_Items.DT_Items" _array_element_2)
            (:`then`
              (bind (_itemid _name _description _maxstack _itemtype) (break `/Game/Core/Database/Item/ST_Item` _returnvalue_2))
              (while (> _generatedamount _maxstack)
                (`KismetArrayLibrary.Array_Add` _generateditems (make `ItemInfo` _itemid _maxstack _maxstack _itemtype))
                (set `local.GeneratedAmount` (- _generatedamount _maxstack)))
              (`KismetArrayLibrary.Array_Add` _generateditems (make `ItemInfo` _itemid _maxstack (`local.GeneratedAmount`) _itemtype))
              (break)))
          (else
            (set `local.TargetWeight` (- _targetweight _output)))))
      (return (`local.GeneratedItems`)))))

(fn `FL_GetConsumable`
  (params (ItemID :type Name))
  (returns (ST_Consumable :type "/Game/Core/Database/Item/Consumable/ST_Consumable Structure"))
  (bind _returnvalue (`|GetDataTableRow` "/Game/Core/Database/Item/Consumable/DT_Consumable.DT_Consumable" ItemID)
    (:`then`
      (return _returnvalue))))

(fn `FL_GetEquipmentInfo`
  (params (ItemID :type Name))
  (returns (ST_Equipment :type "/Game/Core/Database/Item/Equipment/ST_Equipment Structure") (EquipmentType :type "/Game/Core/Database/Item/Equipment/E_EquipmentType Enum") (Found :type Boolean))
  (bind _returnvalue (`|GetDataTableRow` "/Game/Core/Database/Item/Equipment/DT_Equipment.DT_Equipment" ItemID)
    (:`then`
      (return _returnvalue (`.EquipmentType_55_04F675A74A5811E17EDF698FE5C4BC80` (break `/Game/Core/Database/Item/Equipment/ST_Equipment` _returnvalue)) true))
    (:`RowNotFound`
      (return (struct) "NewEnumerator3" false))))

(fn `FL_GetItemIcon`
  (params (ItemID :type Name))
  (returns (Texture2D :type "Texture2D Object Reference"))
  (bind _st_item (`self.FL_GetItemInfo` ItemID))
  (bind _returnvalue (`KismetSystemLibrary.LoadAsset_Blocking` (`.Icon_34_9220D7004AEA0194023BA390FD2D3EFD` (break `/Game/Core/Database/Item/ST_Item` _st_item))))
  (bind _astexture_2d (cast `Texture2D` _returnvalue))
  (return _astexture_2d))

(fn `FL_GetItemInfo`
  (params (ItemID :type Name))
  (returns (ST_Item :type "/Game/Core/Database/Item/ST_Item Structure") (DT_Ref :type "DataTable Object Reference"))
  (bind _returnvalue (`|GetDataTableRow` "/Game/Core/Database/Item/DT_Items.DT_Items" ItemID)
    (:`then`
      (return _returnvalue "/Game/Core/Database/Item/DT_Items.DT_Items"))))

(fn `FL_SplitItemWidget`
  (params (Item :type "Object Object Reference") (FromInventory :type "InventoryComponent Object Reference") (ToInventory :type "InventoryComponent Object Reference") (ToWorld :type Boolean))
  (bind _foundwidgets (`WidgetBlueprintLibrary.GetAllWidgetsWithInterface` null "/Game/Core/Widgets/Item/BPI_Split_Item_Widget.BPI_Split_Item_Widget_C"))
  (if (`KismetArrayLibrary.Array_IsEmpty` _foundwidgets)
    (bind _output (`|GetArrayItem` _foundwidgets))
    (message `/Game/Core/Widgets/Item/BPI_Split_Item_Widget.SetSplitWidget` _output FromInventory ToInventory)
    (`UserWidget.AddToViewport` _output 0)
    (else
      (bind _returnvalue (`KismetSystemLibrary.LoadClassAsset_Blocking` "/Game/Core/Widgets/Item/WBP_Split_Item.WBP_Split_Item_C"))
      (bind _asuser_widget (castclass `UserWidget` _returnvalue))
      (bind _returnvalue_2 (`|CreateWidget` _asuser_widget))
      (message `/Game/Core/Widgets/Item/BPI_Split_Item_Widget.SetSplitWidget` _returnvalue_2 FromInventory ToInventory)
      (`UserWidget.AddToViewport` _returnvalue_2 0))))