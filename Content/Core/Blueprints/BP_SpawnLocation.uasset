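; BP_SpawnLocation is a spawn point actor that delays spawning a named entity by a countdown.
; Starting the countdown stores the entity name, sets a one-shot timer and flags the location as spawning.
; When the timer fires, it calls the OnSpawning event dispatcher with the name and itself, then clears the flag.
; The replicated spawning flag's RepNotify shows the actor only while a spawn is pending.
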(event `CE_StartSpawnCountDown`
  (params (Time :type "Float (single-precision)" :default 5.0) (SpawnEntityName :type Name))
  (set `self.Spawn Entity Name` SpawnEntityName)
  (`KismetSystemLibrary.K2_SetTimerDelegate` (delegate `CE_OnSpawnTime`) Time)
  (set `self.IsSpawning` true))

(event `CE_OnSpawnTime`
  (`self.ED_OnSpawning` (`self.Spawn Entity Name`) self)
  (set `self.IsSpawning` false))

(fn `OnRep_IsSpawning`
  (`self.SetActorHiddenInGame` (not (`self.IsSpawning`))))

(fn `UserConstructionScript`)