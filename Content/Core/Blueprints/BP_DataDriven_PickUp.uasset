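; Data-driven item pickup actor that highlights through custom depth and adds its item to the player's inventory on interaction.
; The construction script resolves item data from a placed table row or ItemID lookup, then sets mesh and material, falling back to an icon-textured dynamic material.
; A full add destroys the actor, while a partial add updates its item info.
; On BeginPlay, DetectButton traces downward to snap it onto the surface below.
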(event `/Game/Core/Blueprints/Interface/BPI_Interactable.INT_ToggleHightlight`
  (params (Toggle :type Boolean))
  ;[1 1 1] Interact hightlight
  (`PrimitiveComponent.SetRenderCustomDepth` (`self.StaticMesh`) Toggle))

(event `/Game/Core/Blueprints/Interface/BPI_Interactable.INT_DoInteraction`
  ;[1 1 1] Interaction - Pick Up
  (bind _inventorycomponent (message `/Game/Core/Blueprints/Interface/BPI_InventoryActor.INT_GetOwnInventory` (`GameplayStatics.GetPlayerPawn` 0)))
  (bind _returnvalue (`|GenericCreateObject` "/Script/Ape_Inventory.Item"))
  (`Item.SetItemInfo` _returnvalue (`self.ItemInfo`))
  (bind _returnvalue_2 (`InventoryComponent.AddItem` _inventorycomponent _returnvalue))
  (if _returnvalue_2
    ;;[1 1 1] Destroy this pickup
    (`self.K2_DestroyActor`)
    (else
      ;;[1 1 1] Partially added, update quantity
      (bind _returnvalue_3 (`Item.GetItemInfo` _returnvalue))
      (set `self.ItemInfo` _returnvalue_3))))

(event `self.ReceiveBeginPlay`
  (`self.DetectButton`))

(fn `DetectButton`
  (bind _returnvalue (`self.K2_GetActorLocation`))
  (bind _returnvalue_2 (* (`.Z` (`KismetMathLibrary.BreakVector3f` (`.BoxExtent` (`KismetSystemLibrary.GetComponentBounds` (`self.StaticMesh`))))) 0.5))
  (bind _outhit (`KismetSystemLibrary.LineTraceSingle` _returnvalue (+ _returnvalue (0.0 0.0 -1000.0)) "TraceTypeQuery1"))
  (bind (_bblockinghit _binitialoverlap _time _distance _location) (`GameplayStatics.BreakHitResult` _outhit))
  (if _bblockinghit
    (if (not (< (`KismetMathLibrary.Vector_DistanceSquared` (- _returnvalue (`KismetMathLibrary.MakeVector` 0.0 0.0 _returnvalue_2)) _location) 1000.0))
      (`self.K2_SetActorLocation` (+ _location (`KismetMathLibrary.MakeVector` 0.0 0.0 (+ (`KismetMathLibrary.RandomFloat`) _returnvalue_2)))))))

(fn `UserConstructionScript`
  (locals (ST_ItemInfo :type "/Game/Core/Database/Item/ST_Item Structure"))
  (bind _staticmesh (`self.StaticMesh`))
  (bind (_datatable _rowname) (break `DataTableRowHandle` (`self.PlacedItem`)))
  (bind (_itemid _name _description _maxstack _itemtype _icon _mesh _materialinstance) (break `/Game/Core/Database/Item/ST_Item` (`local.ST_ItemInfo`)))
  ;[1 1 1] Using reference
  (if (== _rowname "None")
    (bind _st_item (`/Game/Core/Blueprints/Library/FL_ItemUtil.FL_GetItemInfo` (`.ItemID` (break `ItemInfo` (`self.ItemInfo`)))))
    (set `local.ST_ItemInfo` _st_item)
    (else
      (bind _returnvalue (`|GetDataTableRow` _datatable _rowname)
        (:`then`
          (set `local.ST_ItemInfo` _returnvalue)
          (bind (_itemid_2 _name_2 _description_2 _maxstack_2 _itemtype_2) (break `/Game/Core/Database/Item/ST_Item` _returnvalue))
          (set `self.ItemInfo` (make `ItemInfo` _itemid_2 _maxstack_2 (`KismetMathLibrary.Clamp` (`self.Amount`) 1 _maxstack_2) _itemtype_2))))))
  (`|ExecutionSequence`
    (:`then_0`
      (bind _returnvalue_2 (`KismetSystemLibrary.LoadAsset_Blocking` _mesh))
      (bind _asstatic_mesh (cast `StaticMesh` _returnvalue_2))
      (`StaticMeshComponent.SetStaticMesh` _staticmesh _asstatic_mesh))
    (:`then_1`
      (if (`KismetSystemLibrary.IsValidSoftObjectReference` _materialinstance)
        (bind _returnvalue_3 (`KismetSystemLibrary.LoadAsset_Blocking` _materialinstance))
        (bind _asmaterial_instance (cast `MaterialInstance` _returnvalue_3))
        (`PrimitiveComponent.SetMaterial` _staticmesh 0 _asmaterial_instance)
        (else
          (bind _returnvalue_4 (`KismetSystemLibrary.LoadAsset_Blocking` _icon))
          (bind _astexture_2d (cast `Texture2D` _returnvalue_4))
          (bind _returnvalue_5 (`PrimitiveComponent.CreateDynamicMaterialInstance` _staticmesh 0 "/Game/Assets/Materials/MAT_PickUp.MAT_PickUp" "None"))
          (`MaterialInstanceDynamic.SetTextureParameterValue` _returnvalue_5 "Normal" _astexture_2d)
          (`PrimitiveComponent.SetMaterial` _staticmesh 0 _returnvalue_5))))))