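; BloodLust ability actor that heals its owning player character by a small fraction of max HP when triggered while active.
; ActivateAbility caches the owner, shows the actor, multicasts healing FX and sound, and starts a short timer.
; Each trigger stamps the owner's cooldown time and sets the timer again, while the finish event deactivates and hides the actor.
; A separate helper applies new movement speeds according to the owner's action state.
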(event `CE_OnFinished`
  (set `self.IsActive` false)
  (`KismetSystemLibrary.K2_InvalidateTimerHandle` (`self.TimeHandle`))
  (set `self.TimeHandle` (struct))
  (`self.SetActorHiddenInGame` true))

(event `MULTICAST_Effect`
  (`ActorComponent.Activate` (`self.HealthFX`) true)
  (`GameplayStatics.PlaySoundAtLocation` "/Game/Audio/WAV/Click_05.Click_05" (`self.K2_GetActorLocation`) (struct) 1.0 1.0 0.1 "/Game/Audio/SA_Basic.SA_Basic" null null null))

(event `/Game/Core/Blueprints/Pawn/Ability/BPI_CharacterAbility.TriggerAbility`
  (bind _as_bp_player_character (`self.As BP Player Character`))
  (bind _output (`|ConvertAsset` _as_bp_player_character))
  (bind _st_playerstat_maxhp (break `/Game/Core/Database/Character/ST_PlayerStat` (`/Game/Core/Blueprints/Pawn/BP_PlayerCharacter.ST_PlayerStat` _output)))
  (if (`self.IsActive`)
    (if (`KismetSystemLibrary.IsValidSoftObjectReference` _as_bp_player_character)
      (set `/Game/Core/Blueprints/Pawn/BP_PlayerCharacter.AbilityCooldown_TimeStamp` (`KismetMathLibrary.UtcNow`) _output)
      (`/Game/Core/Blueprints/Pawn/BP_PlayerCharacter.SetHealth` _output (+ (`KismetMathLibrary.FMax` (* _st_playerstat_maxhp 0.01) 1.0) (`/Game/Core/Blueprints/Pawn/BP_PlayerCharacter.CurrentHealth` _output)))
      (bind _returnvalue (`KismetSystemLibrary.K2_SetTimerDelegate` (`|CreateDelegate` :!event `CE_OnFinished`) 2.0))
      (set `self.TimeHandle` _returnvalue))))

(fn `ActivateAbility`
  (params (OwnerCharacter :type "Character Object Reference"))
  (bind _asbp_player_character (cast `/Game/Core/Blueprints/Pawn/BP_PlayerCharacter` OwnerCharacter))
  (set `self.As BP Player Character` (`|ConvertAsset` _asbp_player_character))
  (`self.SetActorHiddenInGame` false)
  (bind _returnvalue (`KismetSystemLibrary.K2_SetTimerDelegate` (`|CreateDelegate` :!event `CE_OnFinished`) 2.0))
  (set `self.TimeHandle` _returnvalue)
  (`self.MULTICAST_Effect`)
  (set `self.IsActive` true)
  (return))

(fn `UserConstructionScript`)