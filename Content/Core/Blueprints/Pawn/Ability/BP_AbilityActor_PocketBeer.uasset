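; Pocket Beer ability actor that heals its owning player character with an instant boost followed by regeneration over time.
; ActivateAbility restores a share of max HP, shows the actor, multicasts the heal effect, starts a looping one-second timer and returns a fixed float.
; Each tick adds smaller clamped healing until the tick limit or a particular ActionState is reached, then clears the timer and hides the actor.
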(event `CE_RegenTickEvent`
  (bind _as_bp_player_character (`self.As BP Player Character`))
  (bind _st_playerstat_maxhp (break `/Game/Core/Database/Character/ST_PlayerStat` (`/Game/Core/Blueprints/Pawn/BP_PlayerCharacter.ST_PlayerStat` _as_bp_player_character)))
  (if (`|EnumEquality` (`/Game/Core/Blueprints/Pawn/BP_PlayerCharacter.ActionState` _as_bp_player_character) "NewEnumerator4")
    (`KismetSystemLibrary.K2_InvalidateTimerHandle` (`self.TimeHandle`) :!label _label)
    (set `self.TimeHandle` (struct))
    (`self.SetActorHiddenInGame` true)
    (elif (>= (`self.Times`) 4)
      (goto _label)
      (else
        (set `/Game/Core/Blueprints/Pawn/BP_PlayerCharacter.CurrentHealth` (`KismetMathLibrary.FMin` (+ (`/Game/Core/Blueprints/Pawn/BP_PlayerCharacter.CurrentHealth` _as_bp_player_character) (* _st_playerstat_maxhp 0.08)) _st_playerstat_maxhp) _as_bp_player_character) ; tick hp
        (set `self.Times` (+ (`self.Times`) 1))))))

(event `MULTICAST_Effect`
  (`ActorComponent.Activate` (`self.HealFX`) true))

(fn `ActivateAbility`
  (params (OwnerCharacter :type "Character Object Reference"))
  (returns (CooldownTime :type "Float (double-precision)"))
  (bind _asbp_player_character (cast `/Game/Core/Blueprints/Pawn/BP_PlayerCharacter` OwnerCharacter))
  (bind _output_get (set `self.As BP Player Character` _asbp_player_character))
  (bind _st_playerstat_maxhp (break `/Game/Core/Database/Character/ST_PlayerStat` (`/Game/Core/Blueprints/Pawn/BP_PlayerCharacter.ST_PlayerStat` _output_get)))
  (set `/Game/Core/Blueprints/Pawn/BP_PlayerCharacter.CurrentHealth` (`KismetMathLibrary.FMin` (+ (`/Game/Core/Blueprints/Pawn/BP_PlayerCharacter.CurrentHealth` _output_get) (* _st_playerstat_maxhp 0.2)) _st_playerstat_maxhp) _output_get) ; tick hp
  (`self.SetActorHiddenInGame` false)
  (bind _returnvalue (`KismetSystemLibrary.K2_SetTimerDelegate` (`|CreateDelegate` :!event `CE_RegenTickEvent`) 1.0 true))
  (set `self.TimeHandle` _returnvalue)
  (set `self.Times` 0)
  (`self.MULTICAST_Effect`)
  (return 12.0))

(fn `UserConstructionScript`)