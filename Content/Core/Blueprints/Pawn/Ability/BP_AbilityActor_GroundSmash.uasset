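; Ground smash ability actor that deals an area hit around itself when the player character activates it.
; ActivateAbility enables query collision on its capsule and loops over overlapping actors, skipping the owner and other players.
; Each target takes damage scaled from the owner's Power stat, applied only on the server, and receives a damage reaction message with guaranteed interrupt.
; A locally controlled owner also triggers a world camera shake for each hit.
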(fn `ActivateAbility`
  (params (OwnerCharacter :type "Character Object Reference"))
  (bind _capsule (`self.Capsule`))
  (bind _asbp_player_character (cast `/Game/Core/Blueprints/Pawn/BP_PlayerCharacter` OwnerCharacter))
  (set `self.As BP Player Character` (`|ConvertAsset` _asbp_player_character))
  (`PrimitiveComponent.SetCollisionEnabled` _capsule "QueryOnly")
  (for _array_element (`PrimitiveComponent.GetOverlappingActors` _capsule null)
    (if (!= _array_element OwnerCharacter)
      (cast `/Game/Core/Blueprints/Interface/BPI_Player` _array_element
        (:`CastFailed`
          (if (`KismetSystemLibrary.IsServer`)
            (bind (_st_playerstat_maxhp _st_playerstat_speed _st_playerstat_power) (break `/Game/Core/Database/Character/ST_PlayerStat` (`/Game/Core/Blueprints/Pawn/BP_PlayerCharacter.ST_PlayerStat` _asbp_player_character)))
            (bind _returnvalue (* _st_playerstat_power 2.0))
            (`GameplayStatics.ApplyDamage` _array_element _returnvalue (`Pawn.GetController` OwnerCharacter) _asbp_player_character))
          (message `/Game/Core/Blueprints/Pawn/Enemy/BPI_Enemy.Enemy_DamageReaction` _array_element _returnvalue (`|ConvertAsset` (`self.As BP Player Character`)) 100.0 0.0)
          (if (`Pawn.IsLocallyControlled` (`|ConvertAsset` (`self.As BP Player Character`)))
            (`GameplayStatics.PlayWorldCameraShake` "/Game/Core/Blueprints/BP_CameraShake.BP_CameraShake_C" (`self.K2_GetActorLocation`) 0.0 500.0))))))
  (return))

(fn `UserConstructionScript`)