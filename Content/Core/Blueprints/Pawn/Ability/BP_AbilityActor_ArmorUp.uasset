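; BP_AbilityActor_ArmorUp is an ability actor that grants the player character armor equal to half its max HP.
; ActivateAbility binds to the character's health-update dispatcher, sets the armor, shows the actor and multicasts an activation FX and sound.
; OnArmorChange deactivates and hides the actor once armor is depleted, while OnRep_IsActive mirrors visibility from the active flag.
; TriggerAbility is empty.
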(event `MULTICAST_Effect`
  (`ActorComponent.Activate` (`self.SpeedFX`) true)
  (`GameplayStatics.PlaySoundAtLocation` "/Game/Audio/WAV/Click_05.Click_05" (`self.K2_GetActorLocation`) (struct) 1.0 1.0 0.1 "/Game/Audio/SA_Basic.SA_Basic" null null null))

(event `/Game/Core/Blueprints/Pawn/Ability/BPI_CharacterAbility.TriggerAbility`)

(fn `ActivateAbility`
  (params (OwnerCharacter :type "Character Object Reference"))
  (bind _asbp_player_character (cast `/Game/Core/Blueprints/Pawn/BP_PlayerCharacter` OwnerCharacter))
  (add `/Game/Core/Blueprints/Pawn/BP_PlayerCharacter.ED_OnHealthUpdate` _asbp_player_character (`|CreateDelegate` :!event `OnArmorChange`))
  (bind _st_playerstat_maxhp (break `/Game/Core/Database/Character/ST_PlayerStat` (`/Game/Core/Blueprints/Pawn/BP_PlayerCharacter.ST_PlayerStat` _asbp_player_character)))
  (set `/Game/Core/Blueprints/Pawn/BP_PlayerCharacter.Armor` (* _st_playerstat_maxhp 0.5) _asbp_player_character)
  (set `self.IsActive` true)
  (`self.SetActorHiddenInGame` false)
  (`self.MULTICAST_Effect`)
  (return))

(fn `OnArmorChange`
  (params (CurrentHealth :type "Float (double-precision)") (MaxHealth :type "Float (double-precision)") (Armor :type "Float (double-precision)"))
  (if (<= Armor 0.0)
    (set `self.IsActive` false)
    (`self.SetActorHiddenInGame` true)))

(fn `OnRep_IsActive`
  (if (`self.IsActive`)
    (`self.SetActorHiddenInGame` false)
    (else
      (`self.SetActorHiddenInGame` true))))

(fn `UserConstructionScript`)