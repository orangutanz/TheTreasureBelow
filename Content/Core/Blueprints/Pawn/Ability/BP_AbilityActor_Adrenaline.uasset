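; Adrenaline ability actor that gives a player character a temporary movement speed boost.
; ActivateAbility unhides the actor, multicasts speed FX and a sound, starts a five-second timer, sets IsActive and returns the character's cooldown time.
; The IsActive RepNotify applies boosted or normal run, walk and aim limits, updating CharacterMovement to match the current action state.
; When finished, it clears IsActive and the timer, then hides the actor.
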(event `CE_OnFinished`
  (set `self.IsActive` false)
  (`KismetSystemLibrary.K2_InvalidateTimerHandle` (`self.TimeHandle`))
  (set `self.TimeHandle` (struct))
  (`self.SetActorHiddenInGame` true))

(event `MULTICAST_Effect`
  (`ActorComponent.Activate` (`self.SpeedFX`) true)
  (`GameplayStatics.PlaySoundAtLocation` "/Game/Audio/WAV/Click_05.Click_05" (`self.K2_GetActorLocation`) (struct) 1.0 1.0 0.1 "/Game/Audio/SA_Basic.SA_Basic" null null null))

(fn `ActivateAbility`
  (params (OwnerCharacter :type "Character Object Reference"))
  (returns (CooldownTime :type "Float (double-precision)"))
  (bind _asbp_player_character (cast `/Game/Core/Blueprints/Pawn/BP_PlayerCharacter` OwnerCharacter))
  (set `self.As BP Player Character` (`|ConvertAsset` _asbp_player_character))
  (`self.SetActorHiddenInGame` false)
  (bind _returnvalue (`KismetSystemLibrary.K2_SetTimerDelegate` (`|CreateDelegate` :!event `CE_OnFinished`) 5.0))
  (set `self.TimeHandle` _returnvalue)
  (`self.MULTICAST_Effect`)
  (set `self.IsActive` true)
  (bind (_ability_info_name _ability_info_displayname _ability_info_description _ability_info_icon _ability_info_animmontage _ability_info_abilitybp _ability_info_bonesocket _ability_info_actiontimespend _ability_info_cooldowntime) (break `/Game/Core/Database/Character/ST_CharacterAbilityInfo` (`/Game/Core/Blueprints/Pawn/BP_PlayerCharacter.Ability_Info` _asbp_player_character)))
  (return _ability_info_cooldowntime))

(fn `OnRep_IsActive`
  (if (`self.IsActive`)
    (`self.UpdateMovementComponent` 800.0 500.0 310.0)
    (else
      (`self.UpdateMovementComponent` 500.0 310.0 150.0))))

(fn `UserConstructionScript`)