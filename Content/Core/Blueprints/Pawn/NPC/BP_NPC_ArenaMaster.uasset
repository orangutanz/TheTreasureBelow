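; Arena Master NPC Blueprint that gives the player access to the arena menu through interaction.
; On client interaction, it gets the arena manager message object from player controller 0 and, if valid, toggles the arena menu through it.
; When interaction ends, it closes the menu through the same object.
; The construction script only calls the parent version.
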(event `/Game/Core/Blueprints/Interface/BPI_Interactable.Client_Interaction`
  (bind _managerref (message `/Game/Core/Blueprints/Framework/BPI_PlayerController.GetArenaManager` (`GameplayStatics.GetPlayerController` 0)))
  (`/Engine/EditorBlueprintResources/StandardMacros.IsValid` _managerref
    (:`Is Valid`
      (message `/Game/Core/Blueprints/Arena/BPI_ArenaManager.ToggleArenaMenu` _managerref))))

(fn `OnInteractionOff`
  (bind _managerref (message `/Game/Core/Blueprints/Framework/BPI_PlayerController.GetArenaManager` (`GameplayStatics.GetPlayerController` 0)))
  (`/Engine/EditorBlueprintResources/StandardMacros.IsValid` _managerref
    (:`Is Valid`
      (message `/Game/Core/Blueprints/Arena/BPI_ArenaManager.CloseArenaMenu` _managerref))))

(fn `UserConstructionScript`
  (`parent.UserConstructionScript`))