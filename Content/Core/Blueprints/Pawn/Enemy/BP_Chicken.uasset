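; Chicken enemy pawn that pecks with a neck-attached weapon, clucks periodically and gets launched when hit.
; Attacks multicast one of two random montages; the server passes montage length plus random padding to the AI controller, and montage completion or interruption disables attack collision.
; A self-rescheduling timer plays clucks at random intervals until death.
; Damage reactions extend the parent's, launching the chicken up and away from the attacker, scaled by capped damage.
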(event `/Game/Core/Blueprints/Pawn/Enemy/BPI_Enemy.Enemy_Attack`
  (params (AttackName :type Name) (Target :type "Actor Soft Object Reference (by ref)"))
  ;[1 1 1] Attack
  (`self.MULTICAST_Attack` (`KismetMathLibrary.RandomInteger` 2)))

(event `MULTICAST_Attack`
  (params (Type :type Integer))
  (bind _returnvalue (select `int` Type :`0` "/Game/Characters/StylizedCreaturesBundle/Animations/Chicken/AM_Chicken_Attack1.AM_Chicken_Attack1" :`1` "/Game/Characters/StylizedCreaturesBundle/Animations/Chicken/AM_Chicken_Attack2.AM_Chicken_Attack2" :!type "AnimMontage Object Reference"))
  (bind _mesh (`self.Mesh`))
  ;[1 1 1] Attack
  (`/Engine/EditorBlueprintResources/StandardMacros.IsValid` _mesh
    (:`Is Valid`
      (`|PlayMontage` _mesh _returnvalue
        (:`then`
          (`/Engine/EditorBlueprintResources/ActorMacros.Switch Has Authority`
            (:`Authority`
              (message `/Ape_StateComponent/BPI_AI_Controller.SetActionTime` (`AIBlueprintHelperLibrary.GetAIController` self) (+ (`AnimationAsset.GetPlayLength` _returnvalue) (`KismetMathLibrary.RandomFloat`))))))
        (:`OnCompleted`
          (`self.ToggleAttackCollision` false :!label _label))
        (:`OnInterrupted`
          (goto _label))))))

(event `self.ReceiveBeginPlay`
  (`self.Initialize`)
  (bind _returnvalue (`KismetSystemLibrary.K2_SetTimerDelegate` (delegate `CE_ChickenBuck`) (+ (`KismetMathLibrary.RandomFloat`) 1.5)))
  (set `self.ChickenBuck` _returnvalue))

(event `CE_ChickenBuck`
  (if (`self.IsDead`)
    (`KismetSystemLibrary.K2_PauseTimerHandle` (`self.ChickenBuck`))
    (else
      (`GameplayStatics.PlaySoundAtLocation` "/Game/Audio/CUE/SC_Chicken_Buck.SC_Chicken_Buck" (`self.K2_GetActorLocation`) (struct) 1.0 1.0 0.0 "/Game/Audio/SA_Basic.SA_Basic" null self null)
      (`KismetSystemLibrary.K2_SetTimerDelegate` (delegate `CE_ChickenBuck`) (+ (`KismetMathLibrary.RandomFloat`) 1.5)))))

(fn `On Damage Reaction`
  (params (DamageAmount :type "Float (double-precision)") (ByActor :type "Actor Object Reference") (InterruptChance :type "Float (double-precision)") (KnockChance :type "Float (double-precision)"))
  (bind _returnvalue (`KismetMathLibrary.FMin` (/ DamageAmount 10.0) 3.0))
  (bind (_returnvalue_x _returnvalue_y) (`KismetMathLibrary.BreakVector` (`KismetMathLibrary.Vector_Normal2D` (- (`self.K2_GetActorLocation`) (`self.K2_GetActorLocation` ByActor)))))
  (bind _returnvalue_2 (* _returnvalue 300.0))
  (`parent.On Damage Reaction` DamageAmount ByActor InterruptChance KnockChance)
  (`MovementComponent.StopMovementImmediately` (`self.CharacterMovement`))
  (`self.LaunchCharacter` (`KismetMathLibrary.MakeVector` (* _returnvalue_x _returnvalue_2) (* _returnvalue_y _returnvalue_2) (+ (* _returnvalue 100.0) 300.0)) true))

(fn `UserConstructionScript`
  (`parent.UserConstructionScript`)
  (`SceneComponent.K2_AttachToComponent` (`self.Weapon`) (`self.Mesh`) "neck_01" "KeepRelative" "KeepRelative" "KeepRelative" true))