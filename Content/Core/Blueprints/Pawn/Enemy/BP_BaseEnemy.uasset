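; Base enemy pawn with data-table stats, a health bar and an AI controller driven by interface messages.
; Damage lowers health and alerts the AI, while a separate reaction event plays sounds, flashes an overlay material and can interrupt montages.
; Toggled attack collision damages each non-enemy actor once per activation.
; RepNotify handlers update the health bar and trigger death, where the server drops items and the body sinks before its lifespan ends.
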(event `self.ReceiveAnyDamage`
  (params (Damage :type "Float (single-precision)") (DamageType :type "DamageType Object Reference") (InstigatedBy :type "Controller Object Reference") (DamageCauser :type "Actor Object Reference"))
  ;[1 1 1] Shared
  (`self.MakeNoise` 1.0 null (`self.K2_GetActorLocation`) 1000.0)
  (`self.NotDead`
    (:`NotDead`
      (bind _output_get (set `self.CurrentHealth` (`KismetMathLibrary.FMax` (- (`self.CurrentHealth`) Damage))))
      (if (== _output_get 0.0)
        (set `self.ActionState` "NewEnumerator4")
        (else
          (message `/Ape_StateComponent/BPI_AI_Controller.OnDamaged` (`AIBlueprintHelperLibrary.GetAIController` self) (`Controller.K2_GetPawn` InstigatedBy)))))))

(event `/Game/Core/Blueprints/Interface/BPI_Pawn.ToggleAttack`
  (params (IsAttacking :type Boolean) (AttackName :type Name))
  ;[1 1 1] Pawn Interface
  (`self.ToggleAttackCollision` IsAttacking AttackName))

(event `/Game/Core/Blueprints/Interface/BPI_Pawn.BroadcastMontage`
  (params (Montage :type "AnimMontage Object Reference"))
  ;[1 1 1] Pawn Interface
  (`self.MULTICAST_PlayMontage` Montage))

(event `MULTICAST_PlayMontage`
  (params (AnimMontage :type "AnimMontage Object Reference"))
  (bind _mesh (`self.Mesh`))
  ;[1 1 1] Pawn Interface
  (`/Engine/EditorBlueprintResources/StandardMacros.IsValid` _mesh
    (:`Is Valid`
      (`/Engine/EditorBlueprintResources/StandardMacros.IsValid` AnimMontage
        (:`Is Valid`
          (`|PlayMontage` _mesh AnimMontage))))))

(event `self.AttackCollision.OnComponentBeginOverlap`
  (params (OverlappedComponent :type "PrimitiveComponent Object Reference") (OtherActor :type "Actor Object Reference") (OtherComp :type "PrimitiveComponent Object Reference") (OtherBodyIndex :type Integer) (bFromSweep :type Boolean) (SweepResult :type "HitResult Structure (by ref)"))
  ;[1 1 1] Shared
  (`self.HandleAttackCollision` OtherActor SweepResult))

(event `/Game/Core/Blueprints/Pawn/Enemy/BPI_Enemy.SetEnemyTypeName`
  (params (ST_Enemy :type "/Game/Core/Database/Enemy/ST_EnemyEntity Structure") (EnemyTypeName :type Name))
  (bind ((`PowerValues_39_CC2D38F64E403AC1E00318AC93541F2B` _powervalues) (`Health_28_441228CC4B713597ECFB098548B7002D` _health) (`MeleeReach_42_352DEF6A4650A5830B0F448E8759BEBD` _meleereach) (`RangeReach_43_D6B3F75249F9FFA10EF9F2A5923E0349` _rangereach)) (break `/Game/Core/Database/Enemy/ST_EnemyEntity` ST_Enemy))
  ;[1 1 1] Enemy Interface (Shared)
  (set `self.Name ID` EnemyTypeName)
  (set `self.MaxHealth` _health)
  (set `self.CurrentHealth` _health)
  (set `self.MeleeReach` _meleereach)
  (set `self.RangeReach` _rangereach)
  (set `self.AttackDamage` (`KismetMathLibrary.Conv_IntToDouble` _powervalues))
  (`self.Initialize`))

(event `self.ReceiveBeginPlay`
  ;[1 0 0.01749] BeginPlay
  (`self.Initialize`))

(event `/Game/Core/Blueprints/Pawn/Enemy/BPI_Enemy.RotateToFaceTarget`
  (bind _targetref (`self.TargetRef`))
  (bind (_returnvalue_roll _returnvalue_pitch _returnvalue_yaw) (`KismetMathLibrary.BreakRotator` (`KismetMathLibrary.FindLookAtRotation` (`self.K2_GetActorLocation`) (`self.K2_GetActorLocation` _targetref))))
  ;[1 1 1] Enemy Interface (Shared)
  (`self.NotDead`
    (:`NotDead`
      (if (`KismetSystemLibrary.IsValid` _targetref)
        (`self.K2_SetActorRotation` (`KismetMathLibrary.MakeRotator` 0.0 0.0 _returnvalue_yaw))))))

(event `CE_StartDeathDecay`
  (`KismetSystemLibrary.Delay` 2.0)
  (`KismetSystemLibrary.K2_SetTimerDelegate` (delegate `CE_DeathDecay`) 0.2 true))

(event `/Game/Core/Blueprints/Interface/BPI_Pawn.SetTarget`
  (params (NewTarget :type "Actor Object Reference"))
  ;[1 1 1] Enemy Interface (Shared)
  (set `self.TargetRef` NewTarget))

(event `CE_DeathDecay`
  (`SceneComponent.K2_AddLocalOffset` (`self.Mesh`) (0.0 0.0 -2.0) false false))

(event `/Game/Core/Blueprints/Pawn/Enemy/BPI_Enemy.Enemy_DamageReaction`
  (params (DamageAmount :type "Float (double-precision)") (ByActor :type "Actor Object Reference") (InterruptChance :type "Float (double-precision)") (KnockChance :type "Float (double-precision)"))
  (bind _damagereactionmaterial (`self.DamageReactionMaterial`))
  ;[1 1 1] Damage Reaction
  (if (not (`self.IsDead`))
    (`self.On Damage Reaction` DamageAmount ByActor InterruptChance KnockChance)
    (`/Engine/EditorBlueprintResources/StandardMacros.IsValid` _damagereactionmaterial
      (:`Is Valid`
        (`MeshComponent.SetOverlayMaterial` (`self.DamageReaction_Meshes`) _damagereactionmaterial)
        (`KismetSystemLibrary.K2_SetTimerDelegate` (delegate `CE_HandleDamageMaterial`) 0.05)))))

(event `CE_HandleDamageMaterial`
  ;[1 1 1] Damage Reaction
  (`MeshComponent.SetOverlayMaterial` (`self.DamageReaction_Meshes`) null))

(event `CE_PlayMontage`
  (params (MontageToPlay :type "AnimMontage Object Reference"))
  ;[1 1 1] Damage Reaction
  (`|PlayMontage` (`self.Mesh`) MontageToPlay))

(event `/Game/Core/Blueprints/Pawn/Enemy/BPI_Enemy.MulticastEnemy_HurtMontage`
  (`self.MULTICAST_HurtMontage`))

(event `MULTICAST_HurtMontage`
  (bind _hurtmontage (`self.HurtMontage`))
  (if (not (`self.IsDead`))
    (`/Engine/EditorBlueprintResources/StandardMacros.IsValid` _hurtmontage
      (:`Is Valid`
        (`|PlayMontage` (`self.Mesh`) _hurtmontage)))))

(fn `GetActionState`
  (returns (ActionState :type "/Game/Core/Blueprints/E_ActionState Enum"))
  (return (`self.ActionState`)))

(fn `GetAttackRange`
  (returns (MeleeDistance :type "Float (double-precision)") (RangeDistance :type "Float (double-precision)"))
  (return (`self.MeleeReach`) (`self.RangeReach`)))

(fn `GetDamage`
  (returns (Damage :type "Float (double-precision)"))
  (return (* (`self.AttackDamage`) (`KismetMathLibrary.RandomFloatInRange` 0.9 1.1))))

(fn `GetHealth`
  (returns (CurrentHealth :type "Float (double-precision)") (MaxHealth :type "Float (double-precision)"))
  (return (`self.CurrentHealth`) (`self.MaxHealth`)))

(fn `GetTarget`
  (returns (HasTarget :type Boolean) (TargetActor :type "Actor Object Reference") (Location :type "Vector Structure"))
  (bind _targetref (`self.TargetRef`))
  (`/Engine/EditorBlueprintResources/StandardMacros.IsValid` _targetref
    (:`Is Valid`
      (return true _targetref (+ (`self.K2_GetActorLocation` _targetref) (0.0 0.0 60.0))))
    (:`Is Not Valid`
      (return false null (+ (+ (`self.K2_GetActorLocation`) (* (`KismetMathLibrary.GetForwardVector` (`self.K2_GetActorRotation`)) 100.0)) (0.0 0.0 60.0))))))

(fn `HandleAttackCollision`
  (params (Actor :type "Actor Object Reference") (HitResult :type "HitResult Structure (by ref)"))
  (bind _attackedactors (`self.AttackedActors`))
  (`self.NotDead`
    (:`NotDead`
      (if (!= Actor self)
        (if (`Actor.bCanBeDamaged` Actor)
          (if (== (`KismetArrayLibrary.Array_Find` _attackedactors Actor) -1)
            (`KismetArrayLibrary.Array_Add` _attackedactors Actor)
            (cast `/Game/Core/Blueprints/Pawn/Enemy/BPI_Enemy` Actor
              (:`CastFailed`
                (bind _damage (`self.GetDamage`))
                (`GameplayStatics.ApplyPointDamage` Actor _damage (`KismetMathLibrary.GetDirectionUnitVector` (`self.K2_GetActorLocation` Actor) (`self.K2_GetActorLocation`)) HitResult (`self.GetController`) self)
                (`GameplayStatics.PlaySoundAtLocation` "/Game/Audio/CUE/SC_Click.SC_Click" (`.ImpactPoint` (`GameplayStatics.BreakHitResult` HitResult)) (struct) 1.0 1.0 0.0 "/Game/Audio/SA_Basic.SA_Basic" null self null)))))))))

(fn `Initialize`
  (bind _damagereaction_meshes (`self.DamageReaction_Meshes`))
  (bind _statswidget (`self.StatsWidget`))
  (bind _name_id (`self.Name ID`))
  (bind (_datatable _rowname) (break `DataTableRowHandle` (`self.EnemyType`)))
  (if (not (`self.bInitialized`))
    (set `self.bInitialized` true)
    (`self.ToggleAttackCollision` false)
    (`|ExecutionSequence`
      (:`then_0`
        (`/Engine/EditorBlueprintResources/ActorMacros.Switch Has Authority`
          (:`Authority`
            (bind _returnvalue (`|GetDataTableRow` _datatable (select `bool` (!= _name_id "0") :`false` _rowname :`true` _name_id))
              (:`then`
                (bind (_nameid _powervalues _health _meleereach _rangereach) (break `/Game/Core/Database/Enemy/ST_EnemyEntity` _returnvalue))
                (bind _output_get (set `self.CurrentHealth` _health))
                (set `self.MaxHealth` _output_get)
                (set `self.MeleeReach` _meleereach)
                (set `self.RangeReach` _rangereach)
                (set `self.AttackDamage` (`KismetMathLibrary.Conv_IntToDouble` _powervalues))
                (set `self.Name ID` _nameid)
                (message `/Ape_StateComponent/BPI_AI_Controller.InitializeController` (`AIBlueprintHelperLibrary.GetAIController` self) (`self.AIStates`)))))))
      (:`then_1`
        (bind _aswb_pawn_heath_bar (cast `/Game/Core/Widgets/HUD/WB_PawnHeathBar` (`WidgetComponent.GetWidget` _statswidget)))
        (`/Game/Core/Widgets/HUD/WB_PawnHeathBar.InitializeStats` _aswb_pawn_heath_bar (`self.CurrentHealth`) (`self.MaxHealth`) self 14.0 80.0)
        (`SceneComponent.K2_AttachToComponent` _statswidget (`self.Mesh`) "HealthBar" "SnapToTarget" "KeepRelative" "KeepRelative" false))
      (:`then_2`
        (bind _returnvalue_2 (`KismetMaterialLibrary.CreateDynamicMaterialInstance` "/Game/Assets/FX/Materials/MI_DamageReaction.MI_DamageReaction"))
        (set `self.DamageReactionMaterial` _returnvalue_2)
        (`KismetArrayLibrary.Array_Add` _damagereaction_meshes (`self.Weapon`))
        (`KismetArrayLibrary.Array_Add` _damagereaction_meshes (`self.Mesh`))))))

(fn `IsDead`
  (returns (IsDead :type Boolean))
  (return (`|EnumEquality` (`self.ActionState`) "NewEnumerator4")))

(fn `On Damage Reaction`
  (params (DamageAmount :type "Float (double-precision)") (ByActor :type "Actor Object Reference") (InterruptChance :type "Float (double-precision)") (KnockChance :type "Float (double-precision)"))
  (bind _returnvalue (`self.K2_GetActorLocation`))
  (bind _hurtsound (`self.HurtSound`))
  (bind _hurtmontage (`self.HurtMontage`))
  (bind _returnvalue_2 (`SkeletalMeshComponent.GetAnimInstance` (`self.Mesh`)))
  (bind _returnvalue_3 (`AIBlueprintHelperLibrary.GetAIController` self))
  (`|ExecutionSequence`
    (:`then_0`
      (`/Engine/EditorBlueprintResources/StandardMacros.IsValid` _hurtsound
        (:`Is Valid`
          (`GameplayStatics.PlaySoundAtLocation` _hurtsound _returnvalue (struct) 1.0 (`self.RandomSoundPitch`) 0.0 "/Game/Audio/SA_Basic.SA_Basic" null self null))
        (:`Is Not Valid`
          _))
      (`GameplayStatics.PlaySoundAtLocation` "/Game/Audio/CUE/SC_HitGore.SC_HitGore" _returnvalue (struct) 1.0 (`self.RandomSoundPitch`) 0.0 "/Game/Audio/SA_Basic.SA_Basic" null self null))
    (:`then_1`
      (if (> InterruptChance 0.0)
        (`AnimInstance.Montage_Stop` _returnvalue_2 0.1 null)
        (message `/Ape_StateComponent/BPI_AI_Controller.SetActionTime` _returnvalue_3 2.5)
        (`/Engine/EditorBlueprintResources/StandardMacros.IsValid` _hurtmontage :!label _label
          (:`Is Valid`
            (`self.PlayAnimMontage` _hurtmontage)
            (`KismetSystemLibrary.PrintString` "Hurt")))
        (elif (> DamageAmount (`KismetMathLibrary.RandomFloatInRange` 0.0 60.0))
          (`AnimInstance.Montage_Stop` _returnvalue_2 0.1 null)
          (message `/Ape_StateComponent/BPI_AI_Controller.SetActionTime` _returnvalue_3 1.5)
          (goto _label)
          (elif (not (`AnimInstance.Montage_IsPlaying` _returnvalue_2 null))
            (goto _label)))))))

(fn `OnDeath`
  (bind _deathsound (`self.DeathSound`))
  (bind _returnvalue (`AIBlueprintHelperLibrary.GetAIController` self))
  (`|ExecutionSequence`
    (:`then_0`
      (if (`KismetSystemLibrary.IsServer`)
        (set `self.bCanBeDamaged` false)
        (`Controller.StopMovement` _returnvalue)
        (message `/Ape_StateComponent/BPI_AI_Controller.OnDead` _returnvalue)
        (`Controller.UnPossess` _returnvalue)
        (for _array_element (`self.DropItemList`)
          (bind (_st_item _found) (`/Game/Core/Blueprints/Library/FL_ItemUtil.FL_GetItemInfo` _array_element))
          (if _found
            (bind (_itemid _name _description _maxstack _singleprice _itemtype) (break `/Game/Core/Database/Item/ST_Item` _st_item))
            (message `/Game/Core/Blueprints/Framework/BPI_GameMode.DropItem` (`GameplayStatics.GetGameMode`) self (make `ItemInfo` _itemid _maxstack 1 _itemtype) true)))
        (`self.SetLifeSpan` 10.0)))
    (:`then_1`
      (`SceneComponent.SetVisibility` (`self.StatsWidget`) false false)
      (`self.ED_OnDeath` self)
      (`PrimitiveComponent.SetCollisionProfileName` (`self.CapsuleComponent`) "CharacterMesh" false)
      (`PrimitiveComponent.SetCollisionProfileName` (`self.BlockingCapsule`) "CharacterMesh" false)
      (`self.CE_StartDeathDecay`)
      (`/Engine/EditorBlueprintResources/StandardMacros.IsValid` _deathsound
        (:`Is Valid`
          (`GameplayStatics.PlaySoundAtLocation` _deathsound (`self.K2_GetActorLocation`) (struct) 1.0 (+ 1.0 (`KismetMathLibrary.RandomFloatInRange` -0.1 0.1)) 0.0 "/Game/Audio/SA_Basic.SA_Basic" null self null))))))

(fn `OnNameID`)

(fn `OnRep_ActionState`
  (if (`|EnumEquality` (`self.ActionState`) "NewEnumerator4")
    (`self.OnDeath`)))

(fn `OnRep_CurrentHealth`
  (bind _statswidget (`self.StatsWidget`))
  (`/Engine/EditorBlueprintResources/StandardMacros.IsValid` _statswidget
    (:`Is Valid`
      (bind _aswb_pawn_heath_bar (cast `/Game/Core/Widgets/HUD/WB_PawnHeathBar` (`WidgetComponent.GetWidget` _statswidget)))
      (`/Game/Core/Widgets/HUD/WB_PawnHeathBar.OnHealthUpdate` _aswb_pawn_heath_bar (`self.CurrentHealth`) (`self.MaxHealth`)))))

(fn `OnRep_Name ID`
  (`self.OnNameID`))

(fn `ToggleAttackCollision`
  (params (Toggle :type Boolean) (AttackName :type Name))
  (`PrimitiveComponent.SetCollisionEnabled` (`self.AttackCollision`) (select `bool` Toggle :`false` "NoCollision" :`true` "QueryOnly" :!type "ECollisionEnabled Enum"))
  (`KismetArrayLibrary.Array_Clear` (`self.AttackedActors`)))

(fn `UserConstructionScript`)