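; Boar enemy pawn Blueprint with a randomized skin and two melee attack variants.
; The server picks a TypeIndex on BeginPlay, and its OnRep applies the matching body material.
; Server-chosen attacks multicast a montage and pitch-varied growl, set a random AI action delay on authority, and disable attack collision when the montage completes or is interrupted.
; The construction script attaches the Weapon component to the neck socket.
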(event `self.ReceiveBeginPlay`
  (`parent.ReceiveBeginPlay`)
  (if (`KismetSystemLibrary.IsServer`)
    (set `self.TypeIndex` (`KismetMathLibrary.RandomInteger` 4))))

(event `/Game/Core/Blueprints/Pawn/Enemy/BPI_Enemy.Enemy_Attack`
  (params (AttackName :type Name) (Target :type "Actor Soft Object Reference (by ref)"))
  ;[1 1 1] Attack
  (if (`KismetSystemLibrary.IsServer`)
    (`self.MULTICAST_Attack` (`KismetMathLibrary.RandomInteger` 2))))

(event `MULTICAST_Attack`
  (params (Type :type Integer))
  (bind _mesh (`self.Mesh`))
  ;[1 1 1] Attack
  (`/Engine/EditorBlueprintResources/StandardMacros.IsValid` _mesh
    (:`Is Valid`
      (`|PlayMontage` _mesh (select `int` Type :`0` "/Game/Characters/StylizedCreaturesBundle/Animations/Boar/AM_Boar_Attack1.AM_Boar_Attack1" :`1` "/Game/Characters/StylizedCreaturesBundle/Animations/Boar/AM_Boar_Attack2.AM_Boar_Attack2" :!type "AnimMontage Object Reference")
        (:`then`
          (`GameplayStatics.PlaySoundAtLocation` "/Game/Audio/CUE/SC_Boar_Growl.SC_Boar_Growl" (`self.K2_GetActorLocation`) (struct) 1.0 (+ 1.0 (`KismetMathLibrary.RandomFloatInRange` -0.1 0.1)) 0.0 "/Game/Audio/SA_Basic.SA_Basic" null self null)
          (`/Engine/EditorBlueprintResources/ActorMacros.Switch Has Authority`
            (:`Authority`
              (message `/Ape_StateComponent/BPI_AI_Controller.SetActionTime` (`AIBlueprintHelperLibrary.GetAIController` self) (`KismetMathLibrary.RandomFloatInRange` 3.0 5.0)))))
        (:`OnCompleted`
          (`self.ToggleAttackCollision` false :!label _label))
        (:`OnInterrupted`
          (goto _label))))))

(fn `OnRep_TypeIndex`
  (`PrimitiveComponent.SetMaterial` (`self.Mesh`) 0 (`|GetArrayItem` (`self.TypeMaterials`) (`self.TypeIndex`))))

(fn `UserConstructionScript`
  (`parent.UserConstructionScript`)
  (`SceneComponent.K2_AttachToComponent` (`self.Weapon`) (`self.Mesh`) "neck_01" "KeepRelative" "KeepRelative" "KeepRelative" true))