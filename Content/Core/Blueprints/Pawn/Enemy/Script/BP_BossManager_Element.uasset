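; Boss manager for an elemental boss fight that spawns Goblin_Ice adds as the boss enters new stages.
; On the server it binds to the boss's stage event, and stages one to three start timed countdowns on randomly picked non-busy spawners, one add per stage number.
; When a spawner fires, it looks up the enemy in DT_Enemy, blocking-loads its class, spawns it above the spawner and initializes its type data.
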(event `self.ReceiveBeginPlay`
  (if (`KismetSystemLibrary.IsServer`)
    (add `/Game/Core/Blueprints/Pawn/Enemy/BP_Elemental.ED_OnNewStage` (`self.BossRef`) (delegate `CE_HandleNewStage`))
    (for _array_element (`self.AddSpawners`)
      (add `/Game/Core/Blueprints/Arena/BP_SpawnLocation.ED_OnSpawning` _array_element (delegate `CE_OnSpawningEntity`)))))

(event `CE_OnSpawningEntity`
  (params (SpawnEntityName :type Name) (SpawnLocation :type "/Game/Core/Blueprints/Arena/BP_SpawnLocation Object Reference"))
  (bind _returnvalue (`|GetDataTableRow` "/Game/Core/Database/AI/DT_Enemy.DT_Enemy" SpawnEntityName)
    (:`then`
      (bind ((`NameID_15_850DA2BB440BE3CEFA7F87A224E39BC5` _nameid) (`PowerValues_39_CC2D38F64E403AC1E00318AC93541F2B` _powervalues) (`MeleeReach_42_352DEF6A4650A5830B0F448E8759BEBD` _meleereach) (`RangeReach_43_D6B3F75249F9FFA10EF9F2A5923E0349` _rangereach) (`PawnRef_31_887DF8C2413C039B55AC6F9E9964DB29` _pawnref)) (break `/Game/Core/Database/AI/ST_EnemyEntity` _returnvalue))
      (bind _returnvalue_2 (`KismetSystemLibrary.LoadClassAsset_Blocking` _pawnref))
      (bind _aspawn (castclass `Pawn` _returnvalue_2))
      (bind _returnvalue_3 (`|SpawnActorFromClass` _aspawn (`KismetMathLibrary.MakeTransform` (+ (`self.K2_GetActorLocation` SpawnLocation) (0.0 0.0 50.0)) (`self.K2_GetActorRotation` SpawnLocation)) "AdjustIfPossibleButAlwaysSpawn" "OverrideRootScale" null null))
      (bind _asbp_base_enemy (cast `/Game/Core/Blueprints/Pawn/Enemy/BP_BaseEnemy` _returnvalue_3))
      (message `/Game/Core/Blueprints/Pawn/Enemy/BPI_Enemy.SetEnemyTypeName` _asbp_base_enemy _returnvalue _nameid))))

(event `CE_HandleNewStage`
  (params (NewStage :type Integer))
  (switch `int` NewStage
    (:`1`
      (`self.SpawnAdds` 1))
    (:`2`
      (`self.SpawnAdds` 2))
    (:`3`
      (`self.SpawnAdds` 3))))

(fn `GetRndSpawnLocation`
  (returns (SpawnLocation :type "/Game/Core/Blueprints/Arena/BP_SpawnLocation Object Reference") (Success :type Boolean))
  (locals (FreeLocation :type "Array of /Game/Core/Blueprints/Arena/BP_SpawnLocation Object Reference"))
  (bind _freelocation (`local.FreeLocation`))
  (bind (_outitem _outindex) (`KismetArrayLibrary.Array_Random` _freelocation))
  (for _array_element (`self.AddSpawners`)
    (if (not (`/Game/Core/Blueprints/Arena/BP_SpawnLocation.IsSpawning` _array_element))
      (`KismetArrayLibrary.Array_Add` _freelocation _array_element)))
  (return _outitem (!= _outindex -1)))

(fn `SpawnAdds`
  (params (NumOfAdds :type Integer))
  (for _ (range 1 (+ NumOfAdds 1))
    (bind _spawnlocation (`self.GetRndSpawnLocation`))
    (`/Game/Core/Blueprints/Arena/BP_SpawnLocation.CE_StartSpawnCountDown` _spawnlocation 5.0 "Goblin_Ice")))

(fn `UserConstructionScript`)