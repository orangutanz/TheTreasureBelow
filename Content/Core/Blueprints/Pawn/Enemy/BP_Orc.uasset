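; BP_Orc is an orc enemy pawn with a replicated melee attack and a weapon attached to its right palm socket.
; EnemyAttack multicasts a random pick of three attack montages, halting movement while one plays.
; On authority, it also sends the AI controller a randomized action time.
; When the montage completes or is interrupted, attack collision is turned off and walk speed is restored.
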(event `MULTICAST_Attack`
  (params (Type :type Integer))
  (bind _mesh (`self.Mesh`))
  (bind _charactermovement (`self.CharacterMovement`))
  ;[1 1 1] Cleint
  (`/Engine/EditorBlueprintResources/StandardMacros.IsValid` _mesh
    (:`Is Valid`
      (`|PlayMontage` _mesh (select `int` Type :`0` "/Game/Characters/Orc_Hummer/Animations/AM_Orc_Attack_1.AM_Orc_Attack_1" :`1` "/Game/Characters/Orc_Hummer/Animations/AM_Orc_Attack_2.AM_Orc_Attack_2" :`2` "/Game/Characters/Orc_Hummer/Animations/AM_Orc_Attack_3.AM_Orc_Attack_3" :!type "AnimMontage Object Reference")
        (:`then`
          (set `CharacterMovementComponent.MaxWalkSpeed` 0.0 _charactermovement)
          (`/Engine/EditorBlueprintResources/ActorMacros.Switch Has Authority`
            (:`Authority`
              (message `/Ape_StateComponent/BPI_AI_Controller.SetActionTime` (`AIBlueprintHelperLibrary.GetAIController` self) (`KismetMathLibrary.RandomFloatInRange` 1.0 3.0)))))
        (:`OnCompleted`
          (`self.ToggleAttackCollision` false :!label _label)
          (set `CharacterMovementComponent.MaxWalkSpeed` 200.0 _charactermovement))
        (:`OnInterrupted`
          (goto _label))))))

(event `/Game/Core/Blueprints/Pawn/Enemy/BPI_Enemy.Enemy_Attack`
  (params (AttackName :type Name) (Target :type "Actor Soft Object Reference (by ref)"))
  ;[1 1 1] Cleint
  (`self.MULTICAST_Attack` (`KismetMathLibrary.RandomIntegerInRange` 0 2)))

(fn `UserConstructionScript`
  (`parent.UserConstructionScript`)
  (`SceneComponent.K2_AttachToComponent` (`self.Weapon`) (`self.Mesh`) "CATRigRArmPalm" "KeepRelative" "KeepRelative" "KeepRelative" true))