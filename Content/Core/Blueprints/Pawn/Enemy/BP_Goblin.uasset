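; Goblin enemy pawn with melee and ranged attacks, built on a parent enemy class.
; A DT_GoblinType row, chosen by NameID or EnemyType, sets meshes, leader-posed extra parts, held items, scale and offsets on construction and NameID change.
; EnemyAttack checks controller cooldown, then multicasts a montage; the authority sets the next action time and fires a pooled homing spell ball on montage notifies.
; Damage launches the goblin away from its attacker, scaled by damage.
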(event `MULTICAST_Attack`
  (params (AttackType :type Integer))
  (bind _targetref (`self.TargetRef`))
  (bind _mesh (`self.Mesh`))
  (bind _spellarrow (`self.SpellArrow`))
  (bind _returnvalue (`AIBlueprintHelperLibrary.GetAIController` self))
  (bind _returnvalue_2 (select `bool` (`KismetSystemLibrary.IsValid` _targetref) :`false` (`|ConvertAsset` (`self.LastTarget`)) :`true` _targetref))
  ;[1 1 1] Attack
  (`/Engine/EditorBlueprintResources/StandardMacros.IsValid` _mesh
    (:`Is Valid`
      (bind _notifyname (`|PlayMontage` _mesh (select `int` AttackType :`0` "/Game/Characters/Goblin/Animation/AM_AttackSwing.AM_AttackSwing" :`1` "/Game/Characters/Goblin/Animation/AM_Goblin_Wizard_attack_01.AM_Goblin_Wizard_attack_01" :`2` "/Game/Characters/Goblin/Animation/AM_Goblin_Wizard_attack_02.AM_Goblin_Wizard_attack_02" :!type "AnimMontage Object Reference"))
        (:`then`
          (`/Engine/EditorBlueprintResources/ActorMacros.Switch Has Authority`
            (:`Authority`
              (`|ExecutionSequence`
                (:`then_0`
                  (switch `int` AttackType
                    (:`Default`
                      (message `/Ape_StateComponent/BPI_AI_Controller.SetActionTime` _returnvalue (`KismetMathLibrary.RandomFloatInRange` 5.0 7.0)))
                    (:`0`
                      (message `/Ape_StateComponent/BPI_AI_Controller.SetActionTime` _returnvalue (`KismetMathLibrary.RandomFloatInRange` 2.0 3.0)))))))))
        (:`OnCompleted`
          (`self.ToggleAttackCollision` false :!label _label))
        (:`OnInterrupted`
          (goto _label))
        (:`OnNotifyBegin`
          (`/Engine/EditorBlueprintResources/ActorMacros.Switch Has Authority`
            (:`Authority`
              (bind _pooledactor (message `/Game/Core/Blueprints/Framework/BPI_GameMode.GetPoolActor` (`GameplayStatics.GetGameMode`) "/Game/Core/Blueprints/PoolObject/BP_SpellBall.BP_SpellBall_C"))
              (bind _asbp_spell_ball (cast `/Game/Core/Blueprints/PoolObject/BP_SpellBall` _pooledactor))
              (bind _output_get (set `self.As BP Spell Arrow` (`|ConvertAsset` _asbp_spell_ball)))
              (bind _output (`|ConvertAsset` _output_get))
              (`self.K2_SetActorLocationAndRotation` _output (`SceneComponent.K2_GetComponentLocation` _spellarrow) (`SceneComponent.K2_GetComponentRotation` _spellarrow) false false)
              (`/Engine/EditorBlueprintResources/StandardMacros.IsValid` _output
                (:`Is Valid`
                  (`/Game/Core/Blueprints/PoolObject/BP_SpellBall.MULTICAST_HomingTarget` _output _returnvalue_2)
                  (`PooledActor.SetActorActive` _output true 3.0))
                (:`Is Not Valid`
                  (`/Game/Core/Blueprints/PoolObject/BP_SpellBall.MULTICAST_HomingTarget` _output _returnvalue_2))))))))))

(event `/Game/Core/Blueprints/Pawn/Enemy/BPI_Enemy.Enemy_Attack`
  (params (AttackName :type Name) (Target :type "Actor Soft Object Reference (by ref)"))
  ;[1 1 1] Attack
  (bind _canact (message `/Ape_StateComponent/BPI_AI_Controller.GetNotOnActionCooldown` (`self.GetController`)))
  (if _canact
    (if (`KismetSystemLibrary.IsValidSoftObjectReference` Target)
      (set `self.LastTarget` Target))
    (switch `name` AttackName
      (:`Range`
        (`self.MULTICAST_Attack` (`KismetMathLibrary.RandomIntegerInRange` 1 2)))
      (:`Melee`
        (`self.MULTICAST_Attack` 0)))))

(fn `On Damage Reaction`
  (params (DamageAmount :type "Float (double-precision)") (ByActor :type "Actor Object Reference") (InterruptChance :type "Float (double-precision)") (KnockChance :type "Float (double-precision)"))
  (bind _returnvalue (`KismetMathLibrary.FMin` (/ DamageAmount 10.0) 3.0))
  (bind (_returnvalue_x _returnvalue_y) (`KismetMathLibrary.BreakVector` (`KismetMathLibrary.Vector_Normal2D` (- (`self.K2_GetActorLocation`) (`self.K2_GetActorLocation` ByActor)))))
  (bind _returnvalue_2 (* _returnvalue 250.0))
  (`parent.On Damage Reaction` DamageAmount ByActor InterruptChance KnockChance)
  (`MovementComponent.StopMovementImmediately` (`self.CharacterMovement`))
  (`self.LaunchCharacter` (`KismetMathLibrary.MakeVector` (* _returnvalue_x _returnvalue_2) (* _returnvalue_2 _returnvalue_y) (+ (* _returnvalue 100.0) 150.0)) true))

(fn `OnNameID`
  (`self.UpdateGoblinType`))

(fn `UpdateGoblinType`
  (bind _name_id (`self.Name ID`))
  (bind _mesh (`self.Mesh`))
  (bind _offhand_item (`self.OffHand_Item`))
  (bind _mesh_2 (`self.Mesh`))
  (bind _returnvalue (select `bool` (!= _name_id "0") :`false` (`.RowName` (break `DataTableRowHandle` (`self.EnemyType`))) :`true` _name_id))
  (`|ExecutionSequence`
    (:`then_0`
      (bind _returnvalue_2 (`|GetDataTableRow` "/Game/Core/Database/Enemy/DT_GoblinType.DT_GoblinType" _returnvalue)
        (:`then`
          (`|ExecutionSequence`
            (:`then_0`
              (bind (_sk_main _mat_main _sk_additional _sm_weapon_item _weaponoffset _sm_lefthand_item _scalemodifier) (break `/Game/Core/Database/Enemy/ST_ModularPawn` _returnvalue_2))
              (bind _returnvalue_3 (`KismetSystemLibrary.LoadAsset_Blocking` _sk_main))
              (bind _asskeletal_mesh (cast `SkeletalMesh` _returnvalue_3))
              (`SkeletalMeshComponent.SetSkeletalMeshAsset` _mesh _asskeletal_mesh)
              (bind _returnvalue_4 (`KismetSystemLibrary.LoadAsset_Blocking` _mat_main))
              (bind _asmaterial (cast `Material` _returnvalue_4))
              (`PrimitiveComponent.SetMaterial` (`self.Mesh`) 0 _asmaterial)
              (`SkeletalMeshComponent.SetAnimationMode` _mesh "AnimationBlueprint"))
            (:`then_1`
              (for _array_element _sk_additional
                (bind _returnvalue_5 (`KismetSystemLibrary.LoadAsset_Blocking` _array_element))
                (bind _asskeletal_mesh_2 (cast `SkeletalMesh` _returnvalue_5))
                (bind _returnvalue_6 (`AddComponent|NODE_AddSkeletalMeshComponent-0` :`bManualAttachment` true))
                (`SkeletalMeshComponent.SetSkeletalMeshAsset` _returnvalue_6 _asskeletal_mesh_2)
                (`SceneComponent.K2_AttachToComponent` _returnvalue_6 _mesh_2 "None" "KeepRelative" "KeepRelative" "SnapToTarget" true)
                (`SkinnedMeshComponent.SetLeaderPoseComponent` _returnvalue_6 _mesh_2 false false)
                (`KismetArrayLibrary.Array_Add` (`self.DamageReaction_Meshes`) _returnvalue_6)))
            (:`then_2`
              (bind _returnvalue_7 (`KismetSystemLibrary.LoadAsset_Blocking` _sm_weapon_item))
              (bind _asstatic_mesh (cast `StaticMesh` _returnvalue_7))
              (`StaticMeshComponent.SetStaticMesh` (`self.Weapon`) _asstatic_mesh))
            (:`then_3`
              (bind _returnvalue_8 (`KismetSystemLibrary.LoadAsset_Blocking` _sm_lefthand_item))
              (bind _asstatic_mesh_2 (cast `StaticMesh` _returnvalue_8)
                (:`then`
                  (`StaticMeshComponent.SetStaticMesh` _offhand_item _asstatic_mesh_2)
                  (`KismetArrayLibrary.Array_Add` (`self.DamageReaction_Meshes`) _offhand_item))
                (:`CastFailed`
                  (`StaticMeshComponent.SetStaticMesh` _offhand_item null))))
            (:`then_4`
              (`SceneComponent.SetRelativeScale3D` (`self.Mesh`) _scalemodifier)
              (`SceneComponent.K2_SetRelativeLocation` (`self.Weapon`) _weaponoffset false false)
              (`SceneComponent.K2_SetRelativeLocation` (`self.AttackCollision`) (+ _weaponoffset (0.0 0.0 40.0)) false false)
              (bind (_x _y) (`KismetMathLibrary.BreakVector3f` _weaponoffset))
              (set `CharacterMovementComponent.Mass` (* 100.0 (* _x _y)) (`self.CharacterMovement`)))))))
    (:`then_1`
      (set `self.IsCaster` (`KismetStringLibrary.Contains` (`KismetStringLibrary.Conv_NameToString` _returnvalue) "wizzard")))))

(fn `UserConstructionScript`
  (bind _mesh (`self.Mesh`))
  (`parent.UserConstructionScript`)
  (`self.UpdateGoblinType`)
  (`SceneComponent.K2_AttachToComponent` (`self.OffHand_Item`) _mesh "Base-HumanLPalm" "KeepRelative" "KeepRelative" "KeepRelative" true)
  (`SceneComponent.K2_AttachToComponent` (`self.Weapon`) _mesh "Base-HumanRPalm" "KeepRelative" "KeepRelative" "KeepRelative" true))