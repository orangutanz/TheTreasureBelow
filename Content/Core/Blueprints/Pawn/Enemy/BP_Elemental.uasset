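; Elemental enemy pawn with melee attacks and health-based stages, signalling each new stage through a dispatcher.
; EnemyAttack multicasts a random montage when off cooldown, and the server randomizes the AI controller's action timer.
; Toggleable left and right hit colliders feed shared attack handling.
; Server damage checks advance stages at health quarters, triggering a delayed multicast roar that blocks attacks until it ends.
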(event `MULTICAST_Attack`
  (params (AttackType :type Integer))
  (bind _returnvalue (`KismetMathLibrary.RandomFloatInRange` 3.0 5.0))
  (bind _mesh (`self.Mesh`))
  (bind _returnvalue_2 (`AIBlueprintHelperLibrary.GetAIController` self))
  ;[1 1 1] Attack
  (`/Engine/EditorBlueprintResources/StandardMacros.IsValid` _mesh
    (:`Is Valid`
      (`|PlayMontage` _mesh (select `int` AttackType :`0` "/Game/Characters/Rampage/Animations/AM_Attack1.AM_Attack1" :`1` "/Game/Characters/Rampage/Animations/AM_Attack2.AM_Attack2" :`2` "/Game/Characters/Rampage/Animations/AM_Attack3.AM_Attack3" :!type "AnimMontage Object Reference")
        (:`then`
          (`/Engine/EditorBlueprintResources/ActorMacros.Switch Has Authority`
            (:`Authority`
              ;;[1 1 1] Combo Attack?
              (if (!= (`self.AttackSpeedCache`) 0.0)
                (message `/Ape_StateComponent/BPI_AI_Controller.SetActionTime` _returnvalue_2 (`KismetMathLibrary.RandomFloatInRange` 3.5 6.0))
                (set `self.AttackSpeedCache` 0.0)
                (else
                  (bind _output_get (set `self.AttackSpeedCache` _returnvalue))
                  (message `/Ape_StateComponent/BPI_AI_Controller.SetActionTime` _returnvalue_2 _output_get)
                  (if (not (< _returnvalue 4.0))
                    (set `self.AttackSpeedCache` 0.0)))))))
        (:`OnCompleted`
          (`self.ToggleAttackCollision` false :!label _label))
        (:`OnInterrupted`
          (goto _label))))))

(event `/Game/Core/Blueprints/Pawn/Enemy/BPI_Enemy.Enemy_Attack`
  (params (AttackName :type Name))
  ;[1 1 1] Attack
  (bind _canact (message `/Ape_StateComponent/BPI_AI_Controller.GetNotOnActionCooldown` (`AIBlueprintHelperLibrary.GetAIController` self)))
  (if _canact
    (if (not (`self.IsChangingStage`))
      (switch `name` AttackName
        (:`Default`
          (`self.MULTICAST_Attack` (`KismetMathLibrary.RandomInteger` 2)))))))

(event `self.Right.OnComponentBeginOverlap`
  (params (OverlappedComponent :type "PrimitiveComponent Object Reference") (OtherActor :type "Actor Object Reference") (OtherComp :type "PrimitiveComponent Object Reference") (OtherBodyIndex :type Integer) (bFromSweep :type Boolean) (SweepResult :type "HitResult Structure (by ref)"))
  (`self.HandleAttackCollision` OtherActor SweepResult))

(event `self.Left.OnComponentBeginOverlap`
  (params (OverlappedComponent :type "PrimitiveComponent Object Reference") (OtherActor :type "Actor Object Reference") (OtherComp :type "PrimitiveComponent Object Reference") (OtherBodyIndex :type Integer) (bFromSweep :type Boolean) (SweepResult :type "HitResult Structure (by ref)"))
  (`self.HandleAttackCollision` OtherActor SweepResult))

(event `CE_OnStageChange`
  (params (NextStage :type Integer))
  (if (!= (`self.CurrentStage`) NextStage)
    (if (not (`self.IsChangingStage`))
      (set `self.IsChangingStage` true)
      (set `self.CurrentStage` NextStage)
      (`KismetSystemLibrary.Delay` 1.0)
      (`self.MULTICAST_Roar`))))

(event `MULTICAST_Roar`
  (bind _mesh (`self.Mesh`))
  (`/Engine/EditorBlueprintResources/StandardMacros.IsValid` _mesh
    (:`Is Valid`
      (`|PlayMontage` _mesh "/Game/Characters/Rampage/Animations/AM_Call_Emote.AM_Call_Emote"
        (:`then`
          (if (`KismetSystemLibrary.IsServer`)
            (`self.ED_OnNewStage` (`self.CurrentStage`))))
        (:`OnCompleted`
          (set `self.IsChangingStage` false :!label _label_2))
        (:`OnInterrupted`
          (goto _label_2))))))

(fn `CheckHPStage`
  (bind _maxhealth (`self.MaxHealth`))
  (bind _currenthealth (`self.CurrentHealth`))
  (switch `int` (`self.CurrentStage`)
    (:`0`
      (if (< _currenthealth (* _maxhealth 0.75))
        (`self.CE_OnStageChange` 1)))
    (:`1`
      (if (< _currenthealth (* _maxhealth 0.5))
        (`self.CE_OnStageChange` 2)))
    (:`2`
      (if (< _currenthealth (* _maxhealth 0.25))
        (`self.CE_OnStageChange` 3)))))

(fn `OnDamageReaction`
  (params (DamageAmount :type "Float (double-precision)") (ByActor :type "Actor Object Reference"))
  (bind _returnvalue (`self.K2_GetActorLocation`))
  (bind _hurtsound (`self.HurtSound`))
  (`/Engine/EditorBlueprintResources/StandardMacros.IsValid` _hurtsound
    (:`Is Valid`
      (`GameplayStatics.PlaySoundAtLocation` _hurtsound _returnvalue (struct) 1.0 1.0 0.0 "/Game/Audio/SA_Basic.SA_Basic" null null null))
    (:`Is Not Valid`
      _))
  (`GameplayStatics.PlaySoundAtLocation` "/Game/Audio/CUE/SC_HitGore.SC_HitGore" _returnvalue (struct) 1.0 1.0 0.0 "/Game/Audio/SA_Basic.SA_Basic" null self null)
  (if (`KismetSystemLibrary.IsServer`)
    (`self.CheckHPStage`)))

(fn `ToggleAttackCollision`
  (params (Toggle :type Boolean) (AttackName :type Name))
  (bind _left (`self.Left`))
  (if Toggle
    (`PrimitiveComponent.SetCollisionEnabled` (`self.AttackCollision`) "QueryOnly")
    (switch `name` AttackName
      (:`Left`
        (`PrimitiveComponent.SetCollisionEnabled` _left "QueryOnly"))
      (:`Right`
        (`PrimitiveComponent.SetCollisionEnabled` (`self.Right`) "QueryOnly")))
    (else
      (`PrimitiveComponent.SetCollisionEnabled` _left "NoCollision")
      (`PrimitiveComponent.SetCollisionEnabled` (`self.Right`) "NoCollision")
      (`PrimitiveComponent.SetCollisionEnabled` (`self.AttackCollision`) "NoCollision")))
  (`KismetArrayLibrary.Array_Clear` (`self.AttackedActors`)))

(fn `UserConstructionScript`
  (`parent.UserConstructionScript`))