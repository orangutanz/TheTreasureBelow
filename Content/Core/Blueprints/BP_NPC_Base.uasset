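; Base NPC that highlights on toggle and turns a look-at point toward the local player.
; The construction script reads a data table row to set the skeletal mesh, capsule scale and height of the look-at and throw points.
; Highlighting toggles custom depth; Tick smoothly moves the look-at point to the first player's pawn, or back to the throw point.
; GetTarget exposes that point without a target, and item info stays hidden.
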(event `self.ReceiveTick`
  (params (DeltaSeconds :type "Float (single-precision)"))
  (bind _lookatlocation (`self.LookAtLocation`))
  (bind _returnvalue (`SceneComponent.K2_GetComponentLocation` (`self.LookAtLocation`)))
  (if (`self.IsLooking`)
    (`SceneComponent.K2_SetWorldLocation` _lookatlocation (`KismetMathLibrary.VInterpTo` _returnvalue (+ (`self.K2_GetActorLocation` (`GameplayStatics.GetPlayerPawn` 0)) (0.0 0.0 92.0)) DeltaSeconds 10.0) false false)
    (else
      (`SceneComponent.K2_SetWorldLocation` _lookatlocation (`KismetMathLibrary.VInterpTo` _returnvalue (`SceneComponent.K2_GetComponentLocation` (`self.ThrowLocation`)) DeltaSeconds 10.0) false false))))

(event `/Game/Core/Blueprints/Interface/BPI_Interactable.Client_ToggleHightlight`
  (params (Toggle :type Boolean))
  (`PrimitiveComponent.SetRenderCustomDepth` (`self.Mesh`) Toggle)
  (set `self.IsLooking` Toggle)
  (if Toggle
    (`self.SetActorTickEnabled` true)))

(fn `Client_GetItemInfo`
  (returns (Show :type Boolean) (ItemInfo :type "ItemInfo Structure"))
  (return false))

(fn `GetTarget`
  (returns (HasTarget :type Boolean) (TargetActor :type "Actor Object Reference") (Location :type "Vector Structure"))
  (return false null (`SceneComponent.K2_GetComponentLocation` (`self.LookAtLocation`))))

(fn `UserConstructionScript`
  (bind (_datatable _rowname) (break `DataTableRowHandle` (`self.TypeDT`)))
  (bind _returnvalue (`|GetDataTableRow` _datatable _rowname)
    (:`then`
      (bind (_name _displayname _description _basestat _icon _skeletalmesh _sizescale) (break `/Game/Core/Database/Character/ST_CharacterInfo` _returnvalue))
      (bind _returnvalue_2 (`KismetSystemLibrary.LoadAsset_Blocking` _skeletalmesh))
      (bind _asskeletal_mesh (cast `SkeletalMesh` _returnvalue_2))
      (`SkeletalMeshComponent.SetSkeletalMeshAsset` (`self.Mesh`) _asskeletal_mesh)
      (`SceneComponent.SetRelativeScale3D` (`self.CapsuleComponent`) _sizescale)
      (`SceneComponent.K2_SetRelativeLocation` (`self.LookAtLocation`) (+ (400.0 0.0 0.0) (`KismetMathLibrary.MakeVector` 0.0 0.0 (* (`.Z` (`KismetMathLibrary.BreakVector3f` _sizescale)) 60.0))) false false)
      (`SceneComponent.K2_SetRelativeLocation` (`self.ThrowLocation`) (+ (400.0 0.0 0.0) (`KismetMathLibrary.MakeVector` 0.0 0.0 (* (`.Z` (`KismetMathLibrary.BreakVector3f` _sizescale)) 60.0))) false false))))