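; BP_SavePoint is an interactable brazier that acts as a save point, lit or unlit.
; Interacting while unlit sends a server message, and the server asks the GameMode to update the new safe point; when lit, it only prints a placeholder client menu string.
; ToggleLight, run at construction and on server toggle, swaps the brazier material and shows or hides the light and embers.
; Client highlighting uses custom depth.
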(event `/Game/Core/Blueprints/Interface/BPI_Interactable.Server_Interaction`
  (params (Player :type "PlayerController Object Reference"))
  ;[1 1 1] Server
  (message `/Game/Core/Blueprints/Interface/BPI_GameMode.UpdateNewSafePoint` (`GameplayStatics.GetGameMode`) self))

(event `/Game/Core/Blueprints/Interface/BPI_Interactable.Server_ToggleInteraction`
  (params (Toggle :type Boolean))
  ;[1 1 1] Server
  (`self.ToggleLight` Toggle))

(event `/Game/Core/Blueprints/Interface/BPI_Interactable.Client_ToggleHightlight`
  (params (Toggle :type Boolean))
  ;[1 1 1] Client
  (`PrimitiveComponent.SetRenderCustomDepth` (`self.SM-Brazier-01-01`) Toggle)
  (`PrimitiveComponent.SetRenderCustomDepth` (`self.SM-Brazier-01-02`) Toggle))

(event `/Game/Core/Blueprints/Interface/BPI_Interactable.Client_Interaction`
  ;[1 1 1] Client
  (if (`self.IsLit`)
    (`KismetSystemLibrary.PrintString` "Client Menu" true true (struct :`G` 0.66 :`B` 1.0 :`A` 1.0) 1.0)
    (else
      (message `/Game/Core/Blueprints/Interface/BPI_PlayerController.InteractActorOnServer` (`GameplayStatics.GetPlayerController` 0) self))))

(fn `Client_GetItemInfo`
  (returns (Show :type Boolean) (ItemInfo :type "ItemInfo Structure"))
  (return false))

(fn `ToggleLight`
  (params (Toggle :type Boolean))
  (bind _output_get (set `self.IsLit` Toggle))
  (bind _returnvalue (`KismetMaterialLibrary.CreateDynamicMaterialInstance` (select `bool` _output_get :`false` "/Game/Kobo_Dungeon/Materials/M-Instance/MI-Brazier-01-03.MI-Brazier-01-03" :`true` "/Game/Kobo_Dungeon/Materials/M-Instance/MI-Brazier-01-02.MI-Brazier-01-02" :!type "MaterialInterface Object Reference")))
  (`PrimitiveComponent.SetMaterial` (`self.SM-Brazier-01-02`) 0 _returnvalue)
  (`SceneComponent.SetVisibility` (`self.PointLight`) _output_get false)
  (`SceneComponent.SetVisibility` (`self.FX-BrazierEmbers-01`) _output_get false))

(fn `UserConstructionScript`
  (`self.ToggleLight` (`self.IsLit`)))