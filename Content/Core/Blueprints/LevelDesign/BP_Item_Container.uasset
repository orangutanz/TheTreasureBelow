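; Breakable, lootable world container that players highlight and open through a HUD widget showing its inventory.
; A data table row sets mesh, break sound and, on authority, inventory size.
; On BeginPlay the server fills the inventory once with designated items plus random loot from the container type's table.
; Point damage depletes HP until it drops all items and is destroyed with a sound; drops route through the GameMode.
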(event `self.ReceiveBeginPlay`
  (if (`KismetSystemLibrary.IsServer`)
    (`InventoryComponent.Initialize` (`self.Inventory`))
    (`self.GenerateContainer`)))

(event `self.ReceiveEndPlay`
  (params (EndPlayReason :type "EEndPlayReason Enum" :default "Destroyed"))
  (if (`KismetSystemLibrary.IsServer`) :!label _label
    (`InventoryComponent.ClearInventory` (`self.Inventory`))))

(event `self.ReceiveDestroyed`
  (`GameplayStatics.PlaySoundAtLocation` (`self.Break Sound`) (`self.K2_GetActorLocation`) (struct) 1.0 1.0 0.0 null null null null)
  (goto _label))

(event `self.ReceivePointDamage`
  (params (Damage :type "Float (single-precision)") (DamageType :type "DamageType Object Reference") (HitLocation :type "Vector Structure") (HitNormal :type "Vector Structure") (HitComponent :type "PrimitiveComponent Object Reference") (BoneName :type Name) (ShotFromDirection :type "Vector Structure") (InstigatedBy :type "Controller Object Reference") (DamageCauser :type "Actor Object Reference") (HitInfo :type "HitResult Structure (by ref)"))
  (bind _output_get (set `self.HP` (- (`self.HP`) Damage)))
  (if (<= _output_get 0.0)
    (`InventoryComponent.DropAllItems` (`self.Inventory`))
    (`self.K2_DestroyActor`)))

(event `/Game/Core/Blueprints/Interface/BPI_Interactable.Client_Interaction`
  (bind _returnvalue (`GameplayStatics.GetPlayerController` 0))
  ;[1 1 1] Player Open Container
  (bind _widget (`self.GetContrainerWidget`))
  (message `/Game/Core/Blueprints/Interface/BPI_HUD.AddContainerWidget` (`PlayerController.GetHUD` _returnvalue) _widget (`WidgetLayoutLibrary.ProjectWorldLocationToWidgetPosition` _returnvalue (`self.K2_GetActorLocation`))))

(event `/Game/Core/Blueprints/Interface/BPI_Interactable.Client_ToggleHightlight`
  (params (Toggle :type Boolean))
  ;[1 1 1] Interact hightlight
  (`PrimitiveComponent.SetRenderCustomDepth` (`self.StaticMesh`) Toggle)
  (if (not Toggle)
    (message `/Game/Core/Blueprints/Interface/BPI_HUD.RemoveContainerWidget` (`PlayerController.GetHUD` (`GameplayStatics.GetPlayerController` 0)) (`self.Container Widget`))))

(fn `Client_GetItemInfo`
  (returns (Show :type Boolean) (ItemInfo :type "ItemInfo Structure"))
  (return false))

(fn `DropItem`
  (params (itemInfo :type "ItemInfo Structure"))
  (message `/Game/Core/Blueprints/Interface/BPI_GameMode.DropItem` (`GameplayStatics.GetGameMode`) self itemInfo false))

(fn `GenerateContainer`
  (bind _inventory (`self.Inventory`))
  (bind (_datatable _rowname) (break `DataTableRowHandle` (`self.Container`)))
  (if (not (`self.bInitialized`))
    (set `self.bInitialized` true)
    (`|ExecutionSequence`
      (:`then_0`
        ;[1 1 1] Add designated item(s)
        (for _array_element (`self.DesignatedItems`)
          (bind _returnvalue (`|GetDataTableRow` "/Game/Core/Database/Item/DT_Items.DT_Items" _array_element)
            (:`then`
              (bind _returnvalue_2 (`|GenericCreateObject` "/Script/Ape_Inventory.ItemSlot"))
              (bind (_itemid _name _description _maxstack _itemtype) (break `/Game/Core/Database/Item/ST_Item` _returnvalue))
              (`ItemSlot.SetItemInfo` _returnvalue_2 (make `ItemInfo` _itemid _maxstack 1 _itemtype))
              (`InventoryComponent.AddItem` _inventory _returnvalue_2)))))
      (:`then_1`
        ;[1 1 1] Container generated item
        (bind _returnvalue_3 (`|GetDataTableRow` _datatable _rowname)
          (:`then`
            (bind _outitems (`/Game/Core/Blueprints/Library/FL_ItemUtil.FL_GenerateLootTable` (`.TypeDT_5_5D3E176D45A22819491D1893E6ACAC2F` (break `/Game/Core/Database/Container/ST_Container` _returnvalue_3)) (`self.Generate Amount`)))
            (for _array_element_2 _outitems
              (bind _returnvalue_4 (`|GenericCreateObject` "/Script/Ape_Inventory.ItemSlot"))
              (`ItemSlot.SetItemInfo` _returnvalue_4 _array_element_2)
              (`InventoryComponent.AddItem` _inventory _returnvalue_4))))))))

(fn `GetContrainerWidget`
  (returns (Widget :type "UserWidget Object Reference"))
  (`/Engine/EditorBlueprintResources/StandardMacros.IsValid` (`self.Container Widget`)
    (:`Is Valid`
      _)
    (:`Is Not Valid`
      (bind _returnvalue (`|CreateWidget` "/Game/Core/Widgets/Item/WBP_Container.WBP_Container_C" (`GameplayStatics.GetPlayerController` 0) (`self.Inventory`)))
      (bind _output_get (set `self.Container Widget` _returnvalue))))
  (`/Game/Core/Widgets/Item/WBP_Container.InitializeContainer` _output_get (`self.Inventory`) (`.DisplayName_18_744733B04F1C9687DC9B8DA41FB041D8` (break `/Game/Core/Database/Container/ST_Container` (`self.ST_Container`))))
  (return (`self.Container Widget`)))

(fn `UserConstructionScript`
  (bind _inventory (`self.Inventory`))
  (bind (_datatable _rowname) (break `DataTableRowHandle` (`self.Container`)))
  (bind _returnvalue (`|GetDataTableRow` _datatable _rowname)
    (:`then`
      (`/Engine/EditorBlueprintResources/ActorMacros.Switch Has Authority`
        (:`Authority`
          (bind (_displayname _maxsize _typedt _icon _mesh _materialinstance _breaksound) (break `/Game/Core/Database/Container/ST_Container` _returnvalue))
          (set `InventoryComponent.InventorySize` _maxsize _inventory)
          (add `InventoryComponent.OnDropInventoryItem` _inventory (`|CreateDelegate` :!event `DropItem`)))
        (:`Remote`
          _))
      (bind _returnvalue_2 (`KismetSystemLibrary.LoadAsset_Blocking` _breaksound))
      (bind _assound_base (cast `SoundBase` _returnvalue_2))
      (set `self.Break Sound` _assound_base)
      (bind _returnvalue_3 (`KismetSystemLibrary.LoadAsset_Blocking` _mesh))
      (bind _asstatic_mesh (cast `StaticMesh` _returnvalue_3))
      (`StaticMeshComponent.SetStaticMesh` (`self.StaticMesh`) _asstatic_mesh))))