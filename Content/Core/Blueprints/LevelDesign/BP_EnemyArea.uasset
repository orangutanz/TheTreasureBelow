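; BP_EnemyArea is a level-design spawn area that populates its sphere radius with enemy pawns on the server at BeginPlay.
; Name IDs into DT_EnemyList and per-entry row references each resolve to a blocking-loaded pawn class.
; Pawns spawn above random navigable points, with DoN-limited retries, then receive their row as stats.
; EndPlay destroys pawns in PawnRefs, though this graph never adds spawned pawns to it.
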(event `self.ReceiveEndPlay`
  (params (EndPlayReason :type "EEndPlayReason Enum" :default "Destroyed"))
  (for _array_element (`self.PawnRefs`)
    (`self.K2_DestroyActor` _array_element))
  (`KismetArrayLibrary.Array_Clear` (`self.PawnRefs`)))

(event `self.ReceiveBeginPlay`
  (if (`KismetSystemLibrary.IsServer`)
    (`|ExecutionSequence`
      (:`then_0`
        (for _array_element (`self.Spawn_NameIDs`)
          (bind _returnvalue (`|GetDataTableRow` "/Game/Core/Blueprints/AI/Data/DT_EnemyList.DT_EnemyList" _array_element)
            (:`then`
              (bind _returnvalue_2 (`KismetSystemLibrary.LoadClassAsset_Blocking` (`.PawnRef_18_887DF8C2413C039B55AC6F9E9964DB29` (break `/Game/Core/Blueprints/AI/Data/ST_EnemyEntity` _returnvalue))))
              (bind _aspawn (castclass `Pawn` _returnvalue_2))
              (`|ExecutionSequence`
                (:`then_0`
                  (goto _label_2 :!via `Reset`))
                (:`then_1`
                  (bind (_randomlocation _returnvalue_3) (`NavigationSystemV1.K2_GetRandomLocationInNavigableRadius` (`self.K2_GetActorLocation`) (`SphereComponent.SphereRadius` (`self.Sphere`)) null null :!label _label))
                  (if _returnvalue_3
                    (bind _returnvalue_4 (`|SpawnActorFromClass` _aspawn (`KismetMathLibrary.MakeTransform` (+ _randomlocation (0.0 0.0 120.0))) "AdjustIfPossibleButAlwaysSpawn" "OverrideRootScale" null null))
                    (message `/Game/Core/Blueprints/AI/BPI_Enemy.SetPawnStats` _returnvalue_4 _returnvalue)
                    (else
                      (`/Engine/EditorBlueprintResources/StandardMacros.Do N` 3 :!label _label_2
                        (:`Exit`
                          (goto _label)))))))))))
      (:`then_1`
        (for _array_element_2 (`self.Spawn_Row_Refs`)
          (bind (_datatable _rowname) (break `DataTableRowHandle` (`.DT_EnemyRow_4_396CD6AD4146718E84BB13B3E651900F` (break `/Game/Core/Blueprints/LevelDesign/ST_EnemyInfoRow` _array_element_2))))
          (bind _returnvalue_5 (`|GetDataTableRow` _datatable _rowname)
            (:`then`
              (bind _returnvalue_6 (`KismetSystemLibrary.LoadClassAsset_Blocking` (`.PawnRef_18_887DF8C2413C039B55AC6F9E9964DB29` (break `/Game/Core/Blueprints/AI/Data/ST_EnemyEntity` _returnvalue_5))))
              (bind _aspawn_2 (castclass `Pawn` _returnvalue_6))
              (`|ExecutionSequence`
                (:`then_0`
                  (goto _label_4 :!via `Reset`))
                (:`then_1`
                  (bind (_randomlocation_2 _returnvalue_7) (`NavigationSystemV1.K2_GetRandomLocationInNavigableRadius` (`self.K2_GetActorLocation`) (`SphereComponent.SphereRadius` (`self.Sphere`)) null null :!label _label_3))
                  (if _returnvalue_7
                    (bind _returnvalue_8 (`|SpawnActorFromClass` _aspawn_2 (`KismetMathLibrary.MakeTransform` (+ _randomlocation_2 (0.0 0.0 120.0))) "AdjustIfPossibleButAlwaysSpawn" "OverrideRootScale" null null))
                    (message `/Game/Core/Blueprints/AI/BPI_Enemy.SetPawnStats` _returnvalue_8 _returnvalue_5)
                    (else
                      (`/Engine/EditorBlueprintResources/StandardMacros.Do N` 3 :!label _label_4
                        (:`Exit`
                          (goto _label_3))))))))))))))

(fn `UserConstructionScript`)