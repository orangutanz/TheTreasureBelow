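; Breakable loot container that loses HP from point damage, then drops loot and destroys itself when HP runs out.
; Its construction script sets the static mesh from the container's data table row.
; Loot generation runs once, dropping designated items from DT_Item plus a random roll from the container's loot table, each rolled item kept on a coin flip.
; Drops are spawned through GameMode's DropItemMessage; the container widget getter is empty.
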(event `self.ReceivePointDamage`
  (params (Damage :type "Float (single-precision)") (DamageType :type "DamageType Object Reference") (HitLocation :type "Vector Structure") (HitNormal :type "Vector Structure") (HitComponent :type "PrimitiveComponent Object Reference") (BoneName :type Name) (ShotFromDirection :type "Vector Structure") (InstigatedBy :type "Controller Object Reference") (DamageCauser :type "Actor Object Reference") (HitInfo :type "HitResult Structure (by ref)"))
  (bind _output_get (set `self.HP` (- (`self.HP`) Damage)))
  (if (<= _output_get 0.0)
    (`self.GenerateLoot`)
    (`self.K2_DestroyActor`)))

(fn `GenerateLoot`
  (bind _returnvalue (`GameplayStatics.GetGameMode`))
  (bind (_datatable _rowname) (break `DataTableRowHandle` (`self.Container`)))
  (if (not (`self.bInitialized`))
    (set `self.bInitialized` true)
    (`|ExecutionSequence`
      (:`then_0`
        ;[1 1 1] Add designated item(s)
        (for _array_element (`self.DesignatedItems`)
          (bind _returnvalue_2 (`|GetDataTableRow` "/Game/Core/Database/Item/DT_Item.DT_Item" _array_element)
            (:`then`
              (bind (_itemid _name _description _maxstack _itemtype) (break `/Game/Core/Database/Item/ST_Item` _returnvalue_2))
              (message `/Game/Core/Blueprints/Interface/BPI_GameMode.DropItem` _returnvalue self (make `ItemInfo` _itemid _maxstack 1 _itemtype) false)))))
      (:`then_1`
        ;[1 1 1] Container generated item
        (bind _returnvalue_3 (`|GetDataTableRow` _datatable _rowname)
          (:`then`
            (bind (_displayname _maxsize _typedt) (break `/Game/Core/Database/Container/ST_Container` _returnvalue_3))
            (bind _outitems (`/Game/Core/Blueprints/Library/FL_ItemUtil.FL_GenerateLootTable` _typedt _maxsize))
            (for _array_element_2 _outitems
              (if (`KismetMathLibrary.RandomBool`)
                (message `/Game/Core/Blueprints/Interface/BPI_GameMode.DropItem` _returnvalue self _array_element_2 false)))))))))

(fn `GetContrainerWidget`
  (returns (Widget :type "UserWidget Object Reference")))

(fn `UserConstructionScript`
  (bind (_datatable _rowname) (break `DataTableRowHandle` (`self.Container`)))
  (bind _returnvalue (`|GetDataTableRow` _datatable _rowname)
    (:`then`
      (bind _returnvalue_2 (`KismetSystemLibrary.LoadAsset_Blocking` (`.Mesh_11_45394B734F3621FC849D28A62D0C555B` (break `/Game/Core/Database/Container/ST_Container` _returnvalue))))
      (bind _asstatic_mesh (cast `StaticMesh` _returnvalue_2))
      (`StaticMeshComponent.SetStaticMesh` (`self.StaticMesh`) _asstatic_mesh))))