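; Modular goblin enemy character whose body, material and held items come from a data table row chosen by NameID or a default row.
; Construction and NameID changes load assets synchronously, attaching extra meshes that follow the main mesh's pose.
; Non-caster attacks multicast a swing montage, with authority setting a random AI action delay and montage end disabling attack collision.
; Damage launches it up and away from the attacker, scaled by capped damage.
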(event `MULTICAST_Attack`
  (params (AttackName :type Name))
  ;[1 1 1] Attack
  (if (not (`self.IsCaster`))
    (`|PlayMontage` (`self.Mesh`) "/Game/Characters/Goblin/Animation/AM_AttackSwing.AM_AttackSwing"
      (:`then`
        (`/Engine/EditorBlueprintResources/ActorMacros.Switch Has Authority`
          (:`Authority`
            (message `/Ape_StateComponent/BPI_AI_Controller.SetActionTime` (`AIBlueprintHelperLibrary.GetAIController` self) (`KismetMathLibrary.RandomFloatInRange` 2.0 3.0)))))
      (:`OnCompleted`
        (`self.ToggleAttackCollision` false :!label _label))
      (:`OnInterrupted`
        (goto _label)))))

(event `/Game/Core/Blueprints/AI/BPI_Enemy.Enemy_Attack`
  (params (AttackName :type Name))
  ;[1 1 1] Attack
  (`self.MULTICAST_Attack` AttackName))

(fn `OnDamageReaction`
  (params (DamageAmount :type "Float (double-precision)") (ByActor :type "Actor Object Reference"))
  (bind _returnvalue (`KismetMathLibrary.FMin` (/ DamageAmount 10.0) 3.0))
  (bind (_returnvalue_x _returnvalue_y) (`KismetMathLibrary.BreakVector` (`KismetMathLibrary.Vector_Normal2D` (- (`self.K2_GetActorLocation`) (`self.K2_GetActorLocation` ByActor)))))
  (bind _returnvalue_2 (* _returnvalue 250.0))
  (`parent.OnDamageReaction` DamageAmount ByActor)
  (`MovementComponent.StopMovementImmediately` (`self.CharacterMovement`))
  (`self.LaunchCharacter` (`KismetMathLibrary.MakeVector` (* _returnvalue_x _returnvalue_2) (* _returnvalue_2 _returnvalue_y) (+ (* _returnvalue 100.0) 150.0)) true))

(fn `OnNameID`
  (`self.UpdateGoblinType`))

(fn `UpdateGoblinType`
  (bind _offhand_item (`self.OffHand_Item`))
  (bind _mesh (`self.Mesh`))
  (bind _name_id (`self.Name ID`))
  (bind (_datatable _rowname) (break `DataTableRowHandle` (`self.ModularType`)))
  (bind _returnvalue (`|GetDataTableRow` _datatable (select `bool` (!= _name_id "0") :`false` _rowname :`true` _name_id))
    (:`then`
      (`|ExecutionSequence`
        (:`then_0`
          (bind (_sk_main _mat_main _sk_additional _sm_weapon_item _sm_lefthand_item) (break `/Game/Core/Database/AI/ST_ModularPawn` _returnvalue))
          (bind _returnvalue_2 (`KismetSystemLibrary.LoadAsset_Blocking` _sk_main))
          (bind _asskeletal_mesh (cast `SkeletalMesh` _returnvalue_2))
          (`SkeletalMeshComponent.SetSkeletalMeshAsset` (`self.Mesh`) _asskeletal_mesh)
          (bind _returnvalue_3 (`KismetSystemLibrary.LoadAsset_Blocking` _mat_main))
          (bind _asmaterial (cast `Material` _returnvalue_3))
          (`PrimitiveComponent.SetMaterial` (`self.Mesh`) 0 _asmaterial))
        (:`then_1`
          (for _array_element _sk_additional
            (bind _returnvalue_4 (`KismetSystemLibrary.LoadAsset_Blocking` _array_element))
            (bind _asskeletal_mesh_2 (cast `SkeletalMesh` _returnvalue_4))
            (bind _returnvalue_5 (`AddComponent|NODE_AddSkeletalMeshComponent-0` :`bManualAttachment` true))
            (`SkeletalMeshComponent.SetSkeletalMeshAsset` _returnvalue_5 _asskeletal_mesh_2)
            (`SceneComponent.K2_AttachToComponent` _returnvalue_5 _mesh "None" "KeepRelative" "KeepRelative" "SnapToTarget" true)
            (`SkinnedMeshComponent.SetLeaderPoseComponent` _returnvalue_5 _mesh false false)
            (`KismetArrayLibrary.Array_Add` (`self.DamageReaction_Meshes`) _returnvalue_5)))
        (:`then_2`
          (bind _returnvalue_6 (`KismetSystemLibrary.LoadAsset_Blocking` _sm_weapon_item))
          (bind _asstatic_mesh (cast `StaticMesh` _returnvalue_6))
          (`StaticMeshComponent.SetStaticMesh` (`self.Weapon`) _asstatic_mesh))
        (:`then_3`
          (bind _returnvalue_7 (`KismetSystemLibrary.LoadAsset_Blocking` _sm_lefthand_item))
          (bind _asstatic_mesh_2 (cast `StaticMesh` _returnvalue_7))
          (`StaticMeshComponent.SetStaticMesh` _offhand_item _asstatic_mesh_2)
          (`KismetArrayLibrary.Array_Add` (`self.DamageReaction_Meshes`) _offhand_item))))))

(fn `UserConstructionScript`
  (bind _mesh (`self.Mesh`))
  (`parent.UserConstructionScript`)
  (`self.UpdateGoblinType`)
  (`SceneComponent.K2_AttachToComponent` (`self.OffHand_Item`) _mesh "Base-HumanLPalm" "KeepRelative" "KeepRelative" "KeepRelative" true)
  (`SceneComponent.K2_AttachToComponent` (`self.Weapon`) _mesh "Base-HumanRPalm" "KeepRelative" "KeepRelative" "KeepRelative" true))