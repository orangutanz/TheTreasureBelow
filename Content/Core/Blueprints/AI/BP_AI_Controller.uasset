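; AI controller that feeds perceived players to its pawn as targets and tracks a timed action window.
; Perception updates fill an empty target, while each successful sighting of a player replaces it through pawn interface messages; closest-actor selection exists but is unused.
; SetActionTime timestamps an action in UTC for elapsed and remaining-time queries, and CanMove checks the pawn's action state.
; OnDead disables AI sensing.
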(event `self.AIPerception.OnPerceptionUpdated`
  (params (UpdatedActors :type "Array of Actor Object Reference (by ref)"))
  (bind _returnvalue (`self.K2_GetPawn`))
  (bind (_hastarget _targetactor) (message `/Game/Core/Blueprints/Interface/BPI_Pawn.GetTarget` _returnvalue))
  (if (not _hastarget)
    (for _array_element UpdatedActors
      (cast `/Game/Core/Blueprints/Interface/BPI_Player` _array_element)
      (message `/Game/Core/Blueprints/Interface/BPI_Pawn.SetTarget` _returnvalue _array_element))))

(event `self.AIPerception.OnTargetPerceptionUpdated`
  (params (Actor :type "Actor Object Reference") (Stimulus :type "AIStimulus Structure"))
  (if (`.bSuccessfullySensed` (break `AIStimulus` Stimulus))
    (cast `/Game/Core/Blueprints/Interface/BPI_Player` Actor)
    (message `/Game/Core/Blueprints/Interface/BPI_Pawn.SetTarget` (`self.K2_GetPawn`) Actor)))

(event `/Game/Core/Blueprints/AI/BPI_AI_Controller.SetActionTime`
  (params (ActionTimeLength :type "Float (double-precision)"))
  (set `self.ActionTimeLength` ActionTimeLength)
  (set `self.ActionTimeStamp` (`KismetMathLibrary.UtcNow`)))

(event `/Game/Core/Blueprints/AI/BPI_AI_Controller.OnDead`
  (`AIPerceptionComponent.SetSenseEnabled` (`self.AIPerception`) "/Script/AIModule.AISense" false))

(fn `CanMove`
  (returns (CanMove :type Boolean))
  (bind _actionstate (message `/Game/Core/Blueprints/Interface/BPI_Pawn.GetActionState` (`self.K2_GetPawn`)))
  (if (`|EnumInequality` _actionstate "NewEnumerator4")
    (return true)
    (else
      (return false))))

(fn `CheckActionTimeLength`
  (returns (CanDoAction :type Boolean))
  (return (>= (`.SecondsFloat` (`/Game/Core/Blueprints/Library/FL_Utils.FL_TimeDifference` (`self.ActionTimeStamp`) (`KismetMathLibrary.UtcNow`))) (`self.ActionTimeLength`))))

(fn `GetActionTime`
  (returns (TimeLength :type "Float (double-precision)"))
  (return (`KismetMathLibrary.FMax` (- (`self.ActionTimeLength`) (`.SecondsFloat` (`/Game/Core/Blueprints/Library/FL_Utils.FL_TimeDifference` (`self.ActionTimeStamp`) (`KismetMathLibrary.UtcNow`)))))))

(fn `HandleTarget`)

(fn `UserConstructionScript`
  (set `self.ActionTimeStamp` (`KismetMathLibrary.UtcNow`)))