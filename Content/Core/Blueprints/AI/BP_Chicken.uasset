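; BP_Chicken is a chicken enemy character with melee attacks, hurt reactions and periodic clucking.
; Melee swings multicast one of two random attack montages, turning attack collision off when they end.
; Damage plays a hurt montage, and the authority applies damage-scaled, capped knockback.
; Authority also sends action times to the AI controller after hits and attacks.
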(event `/Game/Core/Blueprints/AI/BPI_Enemy.Enemy_DamageReaction`
  (params (DamageAmount :type "Float (double-precision)") (FromDirectionX :type "Float (double-precision)") (FromDirectionY :type "Float (double-precision)") (ByActor :type "Actor Object Reference"))
  (bind _returnvalue (`KismetMathLibrary.FMin` (/ DamageAmount 10.0) 3.0))
  (bind _returnvalue_2 (* _returnvalue 500.0))
  (if (not (`self.IsDead`))
    (`|PlayMontage` (`self.Mesh`) "/Game/Characters/StylizedCreaturesBundle/Animations/Chicken/AM_Chicken_Hurt.AM_Chicken_Hurt"
      (:`then`
        (`/Engine/EditorBlueprintResources/ActorMacros.Switch Has Authority`
          (:`Authority`
            (`MovementComponent.StopMovementImmediately` (`self.CharacterMovement`))
            (`self.LaunchCharacter` (`KismetMathLibrary.MakeVector` (* FromDirectionX _returnvalue_2) (* FromDirectionY _returnvalue_2) (+ (* _returnvalue 100.0) 300.0)) true)
            (message `/Game/Core/Blueprints/AI/BPI_AI_Controller.SetActionTime` (`AIBlueprintHelperLibrary.GetAIController` self) (`KismetMathLibrary.SelectFloat` 0.0 0.3 (> DamageAmount 10.0)))))))))

(event `/UtilityCombatPlugin/Interface/UtilityControlledPawnCommands_BP.SwingMelee_CPC`
  ;[1 1 1] Attack
  (`self.MULTICAST_Attack` (`KismetMathLibrary.RandomInteger` 2)))

(event `MULTICAST_Attack`
  (params (Type :type Integer))
  ;[1 1 1] Attack
  (`|PlayMontage` (`self.Mesh`) (select `int` Type :`0` "/Game/Characters/StylizedCreaturesBundle/Animations/Chicken/AM_Chicken_Attack1.AM_Chicken_Attack1" :`1` "/Game/Characters/StylizedCreaturesBundle/Animations/Chicken/AM_Chicken_Attack2.AM_Chicken_Attack2" :!type "AnimMontage Object Reference")
    (:`then`
      (`/Engine/EditorBlueprintResources/ActorMacros.Switch Has Authority`
        (:`Authority`
          (message `/Game/Core/Blueprints/AI/BPI_AI_Controller.SetActionTime` (`AIBlueprintHelperLibrary.GetAIController` self) (`KismetMathLibrary.RandomFloatInRange` 3.0 5.0)))))
    (:`OnCompleted`
      (`self.ToggleAttackCollision` false :!label _label))
    (:`OnInterrupted`
      (goto _label))))

(event `self.ReceiveBeginPlay`
  (`parent.ReceiveBeginPlay`)
  (bind _returnvalue (`KismetSystemLibrary.K2_SetTimerDelegate` (delegate `CE_ChickenBuck`) (+ (`KismetMathLibrary.RandomFloat`) 1.0) true))
  (set `self.ChickenBuck` _returnvalue))

(event `CE_ChickenBuck`
  (if (`self.IsDead`)
    (`KismetSystemLibrary.K2_PauseTimerHandle` (`self.ChickenBuck`))
    (else
      (`GameplayStatics.PlaySoundAtLocation` "/Game/Audio/CUE/SC_Chicken_Buck.SC_Chicken_Buck" (`self.K2_GetActorLocation`) (struct) 1.0 1.0 0.0 null null null null))))

(fn `UserConstructionScript`
  (`parent.UserConstructionScript`)
  (`SceneComponent.K2_AttachToComponent` (`self.Weapon`) (`self.Mesh`) "neck_01" "KeepRelative" "KeepRelative" "KeepRelative" true))