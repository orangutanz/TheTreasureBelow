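; Merchant NPC Blueprint that opens a shop window when the player interacts with it.
; Its construction script rebuilds the merchandise list from configured item rows looked up in DT_Items.
; Client interaction toggles the shop: it closes an open merchant widget, or shows the inventory and adds a WBP_Merchant widget fed with that list through the HUD.
; Ending interaction closes all widgets if the merchant one is active.
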(event `/Game/Core/Blueprints/Interface/BPI_Interactable.Client_Interaction`
  (bind _returnvalue (`PlayerController.GetHUD` (`GameplayStatics.GetPlayerController` 0)))
  (bind _widgettype (message `/Game/Core/Blueprints/Framework/BPI_HUD.GetActiveWIdgetType` _returnvalue))
  (if (`|EnumEquality` _widgettype "NewEnumerator4")
    (message `/Game/Core/Blueprints/Framework/BPI_HUD.CloseAllWidgets` _returnvalue)
    (else
      (message `/Game/Core/Blueprints/Framework/BPI_HUD.CloseAllWidgets` _returnvalue)
      (message `/Game/Core/Blueprints/Framework/BPI_HUD.ShowInventroy` _returnvalue)
      (bind _returnvalue_2 (`|CreateWidget` "/Game/Core/Widgets/Item/WBP_Merchant.WBP_Merchant_C" null (`self.MerchantInfo`)))
      (message `/Game/Core/Blueprints/Framework/BPI_HUD.AddWidgetRef` _returnvalue _returnvalue_2 "NewEnumerator4"))))

(fn `OnInteractionOff`
  (bind _returnvalue (`PlayerController.GetHUD` (`GameplayStatics.GetPlayerController` 0)))
  (bind _widgettype (message `/Game/Core/Blueprints/Framework/BPI_HUD.GetActiveWIdgetType` _returnvalue))
  (if (`|EnumEquality` _widgettype "NewEnumerator4")
    (message `/Game/Core/Blueprints/Framework/BPI_HUD.CloseAllWidgets` _returnvalue)))

(fn `UserConstructionScript`
  (`parent.UserConstructionScript`)
  (`KismetArrayLibrary.Array_Clear` (`self.MerchantInfo`))
  (for _array_element (`self.ItemDataRow`)
    (bind _returnvalue (`|GetDataTableRow` "/Game/Core/Database/Item/DT_Items.DT_Items" (`.RowName` (break `DataTableRowHandle` _array_element)))
      (:`then`
        (bind (_itemid _name _description _maxstack _singleprice _itemtype) (break `/Game/Core/Database/Item/ST_Item` _returnvalue))
        (`KismetArrayLibrary.Array_Add` (`self.MerchantInfo`) (make `ItemInfo` _itemid _maxstack 1 _itemtype))))))