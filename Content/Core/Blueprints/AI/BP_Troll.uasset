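; BP_Troll is an AI troll character that visibly reacts to being hit by flashing its point light.
; Point damage calls a multicast event that turns the light red, then a retriggerable delay restores pale green, so rapid hits extend the flash.
; GetActionState exposes its action state.
; Authority-side random wandering and knockback launch logic exist but are disconnected, and BeginPlay is empty.
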(event `MULTICAST_Trigger`
  (bind _pointlight (`self.PointLight`))
  (`LightComponent.SetLightColor` _pointlight (struct :`R` 1.0 :`G` 0.011765 :`A` 1.0) true)
  (`KismetSystemLibrary.RetriggerableDelay` 0.2)
  (`LightComponent.SetLightColor` _pointlight (struct :`R` 0.592157 :`G` 1.0 :`B` 0.482353 :`A` 1.0) true))

(event `self.ReceivePointDamage`
  (params (Damage :type "Float (single-precision)") (DamageType :type "DamageType Object Reference") (HitLocation :type "Vector Structure") (HitNormal :type "Vector Structure") (HitComponent :type "PrimitiveComponent Object Reference") (BoneName :type Name) (ShotFromDirection :type "Vector Structure") (InstigatedBy :type "Controller Object Reference") (DamageCauser :type "Actor Object Reference") (HitInfo :type "HitResult Structure (by ref)"))
  (`self.MULTICAST_Trigger`)
  (cast `Character` DamageCauser))

(event `self.ReceiveBeginPlay`)

(fn `GetActionState`
  (returns (ActionState :type "/Game/Core/Blueprints/E_ActionState Enum"))
  (return (`self.ActionState_0`)))

(fn `UserConstructionScript`)