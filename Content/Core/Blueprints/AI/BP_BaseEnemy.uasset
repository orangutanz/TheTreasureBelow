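; Base enemy pawn with replicated health, action state and name ID, implementing pawn and enemy interfaces for AI targeting and attack queries.
; On authority, a DataTable row supplies health and attack reach.
; Damage emits noise, may retarget to the attacking player and, at zero health, triggers death, which unpossesses the AI and expires the actor.
; Toggled attack collision damages each non-enemy actor once per swing; a widget shows health.
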(event `self.ReceiveAnyDamage`
  (params (Damage :type "Float (single-precision)") (DamageType :type "DamageType Object Reference") (InstigatedBy :type "Controller Object Reference") (DamageCauser :type "Actor Object Reference"))
  ;[1 1 1] Shared
  (`self.MakeNoise` 1.0 (`Controller.K2_GetPawn` InstigatedBy) (`self.K2_GetActorLocation`) 1000.0)
  (`self.NotDead`
    (:`NotDead`
      (`|ExecutionSequence`
        (:`then_0`
          (bind _output_get (set `self.CurrentHealth` (`KismetMathLibrary.FMax` (- (`self.CurrentHealth`) Damage))))
          (if (== _output_get 0.0)
            (`self.OnDeath`)))
        (:`then_1`
          (`/Engine/EditorBlueprintResources/StandardMacros.IsValid` (`self.TargetActor`)
            (:`Is Valid`
              (cast `/Game/Core/Blueprints/Interface/BPI_Player` DamageCauser)
              (if (not (`KismetMathLibrary.RandomBool`))
                (set `self.TargetActor` DamageCauser :!label _label)))
            (:`Is Not Valid`
              (cast `/Game/Core/Blueprints/Interface/BPI_Player` DamageCauser)
              (goto _label))))))))

(event `/Game/Core/Blueprints/Interface/BPI_Pawn.SetTarget`
  (params (NewTarget :type "Actor Object Reference"))
  ;[1 1 1] Pawn Interface
  (set `self.TargetActor` NewTarget))

(event `/Game/Core/Blueprints/Interface/BPI_Pawn.BroadcastMontage`
  (params (Montage :type "AnimMontage Object Reference"))
  ;[1 1 1] Pawn Interface
  (`self.MULTICAST_PlayMontage` Montage))

(event `/Game/Core/Blueprints/Interface/BPI_Pawn.ToggleAttack`
  (params (IsAttacking :type Boolean) (AttackName :type Name))
  ;[1 1 1] Pawn Interface
  (`self.ToggleAttackCollision` IsAttacking AttackName))

(event `MULTICAST_PlayMontage`
  (params (AnimMontage :type "AnimMontage Object Reference"))
  ;[1 1 1] Pawn Interface
  (`|PlayMontage` (`self.Mesh`) AnimMontage))

(event `self.AttackCollision.OnComponentBeginOverlap`
  (params (OverlappedComponent :type "PrimitiveComponent Object Reference") (OtherActor :type "Actor Object Reference") (OtherComp :type "PrimitiveComponent Object Reference") (OtherBodyIndex :type Integer) (bFromSweep :type Boolean) (SweepResult :type "HitResult Structure (by ref)"))
  ;[1 1 1] Shared
  (`self.HandleAttackCollision` OtherActor SweepResult))

(event `/Game/Core/Blueprints/AI/BPI_Enemy.SetEnemyTypeName`
  (params (ST_Enemy :type "/Game/Core/Database/AI/ST_EnemyEntity Structure") (EnemyTypeName :type Name))
  (bind (_nameid _scale _health _attackreach) (break `/Game/Core/Database/AI/ST_EnemyEntity` ST_Enemy))
  ;[1 1 1] Enemy Interface (Shared)
  (set `self.Name ID` EnemyTypeName)
  (set `self.MaxHealth` _health)
  (set `self.CurrentHealth` _health)
  (set `self.AttackReach` _attackreach))

(event `self.ReceiveBeginPlay`
  ;[1 0 0.01749] BeginPlay
  (`self.Initialize`))

(event `/Game/Core/Blueprints/AI/BPI_Enemy.RotateToFaceTarget`
  (bind _targetactor (`self.TargetActor`))
  (bind (_returnvalue_roll _returnvalue_pitch _returnvalue_yaw) (`KismetMathLibrary.BreakRotator` (`KismetMathLibrary.FindLookAtRotation` (`self.K2_GetActorLocation`) (`self.K2_GetActorLocation` _targetactor))))
  ;[1 1 1] Enemy Interface (Shared)
  (`self.NotDead`
    (:`NotDead`
      (if (`KismetSystemLibrary.IsValid` _targetactor)
        (`self.K2_SetActorRotation` (`KismetMathLibrary.MakeRotator` 0.0 0.0 _returnvalue_yaw))))))

(event `DeathEvent`
  (`KismetSystemLibrary.Delay` 0.5)
  (`SceneComponent.SetVisibility` (`self.StatsWidget`) false false)
  (`self.SetLifeSpan` 10.0))

(fn `Enemy_IsReadyToAttack`
  (returns (IsReadyToAttack :type Boolean) (AttackName :type Name))
  (bind _targetactor (`self.TargetActor`))
  (bind _returnvalue (+ (`CapsuleComponent.CapsuleRadius` (`self.CapsuleComponent`)) (`self.AttackReach`)))
  (`/Engine/EditorBlueprintResources/StandardMacros.IsValid` _targetactor
    (:`Is Valid`
      (bind _timelength (message `/Game/Core/Blueprints/AI/BPI_AI_Controller.GetActionTime` (`AIBlueprintHelperLibrary.GetAIController` self)))
      (return (and (== _timelength 0.0) (<= (`self.GetSquaredDistanceTo` _targetactor self) (* _returnvalue _returnvalue))) "Weapon"))
    (:`Is Not Valid`
      (return false "Weapon"))))

(fn `GetActionState`
  (returns (ActionState :type "/Game/Core/Blueprints/E_ActionState Enum"))
  (return (`self.ActionState`)))

(fn `GetAttackRange`
  (returns (AttackRange :type "Float (double-precision)"))
  (return (`self.AttackReach`)))

(fn `GetDamage`
  (returns (Damage :type "Float (double-precision)"))
  (return 10.0))

(fn `GetHealth`
  (returns (CurrentHealth :type "Float (double-precision)") (MaxHealth :type "Float (double-precision)"))
  (return (`self.CurrentHealth`) (`self.MaxHealth`)))

(fn `GetNormalizedStat`
  (params (InputStatName :type Name))
  (returns (ReturnValue :type "Float (single-precision)"))
  (return 0.0))

(fn `GetTarget`
  (returns (HasTarget :type Boolean) (TargetActor :type "Actor Object Reference") (Location :type "Vector Structure"))
  (bind _targetactor (`self.TargetActor`))
  (`/Engine/EditorBlueprintResources/StandardMacros.IsValid` _targetactor
    (:`Is Valid`
      (bind _actionstate (message `/Game/Core/Blueprints/Interface/BPI_Pawn.GetActionState` _targetactor))
      (if (`|EnumInequality` _actionstate "NewEnumerator4")
        (return true _targetactor (`self.K2_GetActorLocation` _targetactor))
        (else
          (set `self.TargetActor` null))))
    (:`Is Not Valid`
      _))
  (return false null (`self.K2_GetActorLocation`)))

(fn `HandleAttackCollision`
  (params (Actor :type "Actor Object Reference") (HitResult :type "HitResult Structure (by ref)"))
  (bind _attackedactors (`self.AttackedActors`))
  (`self.NotDead`
    (:`NotDead`
      (if (!= Actor self)
        (if (`Actor.bCanBeDamaged` Actor)
          (if (== (`KismetArrayLibrary.Array_Find` _attackedactors Actor) -1)
            (`KismetArrayLibrary.Array_Add` _attackedactors Actor)
            (cast `/Game/Core/Blueprints/AI/BPI_Enemy` Actor
              (:`CastFailed`
                (bind _damage (`self.GetDamage`))
                (`GameplayStatics.ApplyPointDamage` Actor _damage (`KismetMathLibrary.GetDirectionUnitVector` (`self.K2_GetActorLocation` Actor) (`self.K2_GetActorLocation`)) HitResult (`self.GetController`) self)
                (`GameplayStatics.PlaySoundAtLocation` "/Game/Audio/CUE/SC_Click.SC_Click" (`.ImpactPoint` (`GameplayStatics.BreakHitResult` HitResult)) (struct) 1.0 1.0 0.0 null null null null)))))))))

(fn `Initialize`
  (bind _name_id (`self.Name ID`))
  (bind (_datatable _rowname) (break `DataTableRowHandle` (`self.EnemyType`)))
  (if (not (`self.bInitialized`))
    (set `self.bInitialized` true)
    (`self.ToggleAttackCollision` false)
    (`|ExecutionSequence`
      (:`then_0`
        (`/Engine/EditorBlueprintResources/ActorMacros.Switch Has Authority`
          (:`Authority`
            (bind _returnvalue (`|GetDataTableRow` _datatable (select `bool` (!= _name_id "0") :`false` _rowname :`true` _name_id))
              (:`then`
                (bind (_nameid _scale _health _attackreach) (break `/Game/Core/Database/AI/ST_EnemyEntity` _returnvalue))
                (bind _output_get (set `self.CurrentHealth` _health))
                (set `self.MaxHealth` _output_get)
                (set `self.AttackReach` _attackreach)
                (set `self.Name ID` _nameid))))))
      (:`then_1`
        (bind _aswb_pawn_heath_bar (cast `/Game/Core/Widgets/HUD/WB_PawnHeathBar` (`WidgetComponent.GetWidget` (`self.StatsWidget`))))
        (`/Game/Core/Widgets/HUD/WB_PawnHeathBar.InitializeStats` _aswb_pawn_heath_bar (`self.CurrentHealth`) (`self.MaxHealth`) self)))))

(fn `IsDead`
  (returns (IsDead :type Boolean))
  (return (`|EnumEquality` (`self.ActionState`) "NewEnumerator4")))

(fn `IsFocusMeleeAttack`
  (returns (ReturnValue :type Boolean))
  (return false))

(fn `IsFocusRangeAttack`
  (returns (ReturnValue :type Boolean))
  (return false))

(fn `IsInMelee`
  (returns (ReturnValue :type Boolean))
  (return false))

(fn `OnDeath`
  (bind _returnvalue (`AIBlueprintHelperLibrary.GetAIController` self))
  (`|ExecutionSequence`
    (:`then_0`
      (set `self.ActionState` "NewEnumerator4")
      (set `self.TargetActor` null)
      (set `self.bCanBeDamaged` false))
    (:`then_1`
      (`Controller.StopMovement` _returnvalue)
      (message `/Game/Core/Blueprints/AI/BPI_AI_Controller.OnDead` _returnvalue)
      (`Controller.UnPossess` _returnvalue)
      (`self.ED_OnDeath`)
      (`self.DeathEvent`))))

(fn `OnNameID`)

(fn `OnRep_ActionState`
  (bind _deathsound (`self.DeathSound`))
  (if (`|EnumEquality` (`self.ActionState`) "NewEnumerator4")
    (`PrimitiveComponent.SetCollisionProfileName` (`self.CapsuleComponent`) "CharacterMesh" false)
    (`PrimitiveComponent.SetCollisionProfileName` (`self.InnerCapsule`) "CharacterMesh" false)
    (`/Engine/EditorBlueprintResources/StandardMacros.IsValid` _deathsound
      (:`Is Valid`
        (`GameplayStatics.PlaySoundAtLocation` _deathsound (`self.K2_GetActorLocation`) (struct) 1.0 1.0 0.0 null null null null)))))

(fn `OnRep_CurrentHealth`
  (bind _aswb_pawn_heath_bar (cast `/Game/Core/Widgets/HUD/WB_PawnHeathBar` (`WidgetComponent.GetWidget` (`self.StatsWidget`))))
  (`/Game/Core/Widgets/HUD/WB_PawnHeathBar.OnHealthUpdate` _aswb_pawn_heath_bar (`self.CurrentHealth`) (`self.MaxHealth`)))

(fn `OnRep_Name ID`
  (`self.OnNameID`))

(fn `ToggleAttackCollision`
  (params (Toggle :type Boolean) (AttackName :type Name))
  (`PrimitiveComponent.SetCollisionEnabled` (`self.AttackCollision`) (select `bool` Toggle :`false` "NoCollision" :`true` "QueryOnly" :!type "ECollisionEnabled Enum"))
  (`KismetArrayLibrary.Array_Clear` (`self.AttackedActors`)))

(fn `UserConstructionScript`
  (bind _capsulecomponent (`self.CapsuleComponent`))
  (bind _innercapsule (`self.InnerCapsule`))
  (`CapsuleComponent.SetCapsuleHalfHeight` _innercapsule (* (`CapsuleComponent.CapsuleHalfHeight` _capsulecomponent) 0.8) true)
  (`CapsuleComponent.SetCapsuleRadius` _innercapsule (* (`CapsuleComponent.CapsuleRadius` _capsulecomponent) 0.5) true)
  (`PrimitiveComponent.SetCollisionEnabled` (`self.AttackCollision`) "NoCollision")
  (`PrimitiveComponent.SetCollisionEnabled` (`self.Weapon`) "NoCollision")
  (`PrimitiveComponent.SetCollisionEnabled` (`self.OffHand_Item`) "NoCollision")
  (`PrimitiveComponent.SetCollisionEnabled` (`self.Mesh`) "NoCollision")
  (`SceneComponent.K2_AttachToComponent` (`self.StatsWidget`) (`self.Mesh`) "HealthBar" "SnapToTarget" "KeepRelative" "KeepRelative" false))