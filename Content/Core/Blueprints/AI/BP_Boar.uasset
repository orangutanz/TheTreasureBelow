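; Boar AI character that varies its look and performs melee attacks in multiplayer.
; The server picks a random type on BeginPlay, and the TypeIndex RepNotify applies the matching mesh material.
; Melee swings multicast one of two random attack montages; authority sends the AI controller a randomized action time, and montage end or interruption disables attack collision.
; The construction script attaches the Weapon component to the neck socket.
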(event `self.ReceiveBeginPlay`
  (`parent.ReceiveBeginPlay`)
  (if (`KismetSystemLibrary.IsServer`)
    (set `self.TypeIndex` (`KismetMathLibrary.RandomInteger` 4))))

(event `/UtilityCombatPlugin/Interface/UtilityControlledPawnCommands_BP.SwingMelee_CPC`
  ;[1 1 1] Attack
  (`self.MULTICAST_Attack` (`KismetMathLibrary.RandomInteger` 2)))

(event `MULTICAST_Attack`
  (params (Type :type Integer))
  ;[1 1 1] Attack
  (`|PlayMontage` (`self.Mesh`) (select `int` Type :`0` "/Game/Characters/StylizedCreaturesBundle/Animations/Boar/AM_Boar_Attack1.AM_Boar_Attack1" :`1` "/Game/Characters/StylizedCreaturesBundle/Animations/Boar/AM_Boar_Attack2.AM_Boar_Attack2" :!type "AnimMontage Object Reference")
    (:`then`
      (`/Engine/EditorBlueprintResources/ActorMacros.Switch Has Authority`
        (:`Authority`
          (message `/Game/Core/Blueprints/AI/BPI_AI_Controller.SetActionTime` (`AIBlueprintHelperLibrary.GetAIController` self) (`KismetMathLibrary.RandomFloatInRange` 3.0 5.0)))))
    (:`OnCompleted`
      (`self.ToggleAttackCollision` false :!label _label))
    (:`OnInterrupted`
      (goto _label))))

(fn `OnRep_TypeIndex`
  (`PrimitiveComponent.SetMaterial` (`self.Mesh`) 0 (`|GetArrayItem` (`self.TypeMaterials`) (`self.TypeIndex`))))

(fn `UserConstructionScript`
  (`parent.UserConstructionScript`)
  (`SceneComponent.K2_AttachToComponent` (`self.Weapon`) (`self.Mesh`) "neck_01" "KeepRelative" "KeepRelative" "KeepRelative" true))