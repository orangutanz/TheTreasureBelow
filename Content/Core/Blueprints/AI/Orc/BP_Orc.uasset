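; BP_Orc is an orc enemy Blueprint handling melee attacks and damage reactions, with its weapon attached to a hand socket.
; EnemyAttack multicasts a random montage behind a timestamp cooldown, halting movement until it ends, then disabling attack collision.
; Damage launches the living orc with damage-scaled knockback, interrupts movement and flashes its point light red alongside a hit montage.
; On authority, both paths send action times to the AI controller.
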(event `/Game/Core/Blueprints/AI/BPI_Enemy.Enemy_DamageReaction`
  (params (DamageAmount :type "Float (double-precision)") (FromDirectionX :type "Float (double-precision)") (FromDirectionY :type "Float (double-precision)") (ByActor :type "Actor Object Reference"))
  (bind _returnvalue (/ DamageAmount 10.0))
  (bind _pointlight (`self.PointLight`))
  (bind _returnvalue_2 (* _returnvalue 75.0))
  (if (not (`self.IsDead`))
    (`/Engine/EditorBlueprintResources/ActorMacros.Switch Has Authority`
      (:`Authority`
        (`|ExecutionSequence`
          (:`then_0`
            (`self.LaunchCharacter` (`KismetMathLibrary.MakeVector` (* FromDirectionX _returnvalue_2) (* FromDirectionY _returnvalue_2) (+ (* _returnvalue 75.0) 100.0)))
            (`NavMovementComponent.StopMovementKeepPathing` (`self.CharacterMovement`))
            (message `/Ape_StateComponent/BPI_AI_Controller.SetActionTime` (`AIBlueprintHelperLibrary.GetAIController` self) (`KismetMathLibrary.SelectFloat` (* _returnvalue 0.3) 0.3 (> DamageAmount 10.0))))
          (:`then_1`
            (`self.StopAnimMontage` "/Game/Characters/Orc_Hummer/Animations/AM_Orc_Attack_2.AM_Orc_Attack_2" :!label _label)
            (`|PlayMontage` (`self.Mesh`) "/Game/Characters/Orc_Hummer/Animations/AM_Orc_Hit_React.AM_Orc_Hit_React"
              (:`then`
                (`LightComponent.SetLightColor` _pointlight (struct :`R` 1.0 :`G` 0.011765 :`A` 1.0) true)
                (`KismetSystemLibrary.RetriggerableDelay` 0.2)
                (`LightComponent.SetLightColor` _pointlight (struct :`R` 0.592157 :`G` 1.0 :`B` 0.482353 :`A` 1.0) true))))))
      (:`Remote`
        (goto _label)))))

(event `MULTICAST_Attack`
  (params (Type :type Integer))
  (bind _returnvalue (`KismetMathLibrary.UtcNow`))
  (bind _charactermovement (`self.CharacterMovement`))
  ;[1 1 1] Cleint
  (if (> (`/Game/Core/Blueprints/Library/FL_Utils.FL_TimeDifference` (`self.CD`) _returnvalue) 2)
    (set `self.CD` _returnvalue)
    (`|PlayMontage` (`self.Mesh`) (select `int` Type :`0` "/Game/Characters/Orc_Hummer/Animations/AM_Orc_Attack_1.AM_Orc_Attack_1" :`1` "/Game/Characters/Orc_Hummer/Animations/AM_Orc_Attack_2.AM_Orc_Attack_2" :`2` "/Game/Characters/Orc_Hummer/Animations/AM_Orc_Attack_3.AM_Orc_Attack_3" :!type "AnimMontage Object Reference")
      (:`then`
        (set `CharacterMovementComponent.MaxWalkSpeed` 0.0 _charactermovement)
        (`/Engine/EditorBlueprintResources/ActorMacros.Switch Has Authority`
          (:`Authority`
            (message `/Ape_StateComponent/BPI_AI_Controller.SetActionTime` (`AIBlueprintHelperLibrary.GetAIController` self) (`KismetMathLibrary.RandomFloatInRange` 3.0 5.0)))))
      (:`OnCompleted`
        (`self.ToggleAttackCollision` false :!label _label_2)
        (set `CharacterMovementComponent.MaxWalkSpeed` 200.0 _charactermovement))
      (:`OnInterrupted`
        (goto _label_2)))))

(event `/Game/Core/Blueprints/AI/BPI_Enemy.Enemy_Attack`
  (params (AttackName :type Name))
  ;[1 1 1] Cleint
  (`self.MULTICAST_Attack` (`KismetMathLibrary.RandomIntegerInRange` 0 2)))

(fn `UserConstructionScript`
  (`parent.UserConstructionScript`)
  (`SceneComponent.K2_AttachToComponent` (`self.Weapon`) (`self.Mesh`) "CATRigRArmPalm" "KeepRelative" "KeepRelative" "KeepRelative" true))