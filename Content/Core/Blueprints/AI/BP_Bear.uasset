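; BP_Bear is a bear enemy AI character built on a parent class, with randomized appearance and melee attacks.
; On BeginPlay the server picks one of four type indices, and its OnRep swaps the mesh material to match.
; Attacks are server-chosen and multicast, playing a pitch-varied sound and one of three montages, then clearing attack collision when the montage ends.
; The authority also sends the AI controller a randomized action delay.
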(event `self.ReceiveBeginPlay`
  (`parent.ReceiveBeginPlay`)
  (if (`KismetSystemLibrary.IsServer`)
    (set `self.TypeIndex` (`KismetMathLibrary.RandomInteger` 4))))

(event `/Game/Core/Blueprints/AI/BPI_Enemy.Enemy_Attack`
  (params (AttackName :type Name))
  ;[1 1 1] Attack
  (if (`KismetSystemLibrary.IsServer`)
    (`self.MULTICAST_Attack` (`KismetMathLibrary.RandomInteger` 3))))

(event `MULTICAST_Attack`
  (params (Type :type Integer))
  ;[1 1 1] Attack
  (`GameplayStatics.PlaySoundAtLocation` "/Game/Audio/Sounds/Enemy/Bear_Attack.Bear_Attack" (`self.K2_GetActorLocation`) (struct) 1.0 (+ 1.0 (`KismetMathLibrary.RandomFloatInRange` -0.1 0.1)) 0.0 null null null null)
  (`|PlayMontage` (`self.Mesh`) (select `int` Type :`0` "/Game/Characters/StylizedCreaturesBundle/Animations/Bear/AM_Bear_Attack1.AM_Bear_Attack1" :`1` "/Game/Characters/StylizedCreaturesBundle/Animations/Bear/AM_Bear_Attack2.AM_Bear_Attack2" :`2` "/Game/Characters/StylizedCreaturesBundle/Animations/Bear/AM_Bear_Attack3.AM_Bear_Attack3" :!type "AnimMontage Object Reference")
    (:`then`
      (`/Engine/EditorBlueprintResources/ActorMacros.Switch Has Authority`
        (:`Authority`
          (message `/Ape_StateComponent/BPI_AI_Controller.SetActionTime` (`AIBlueprintHelperLibrary.GetAIController` self) (`KismetMathLibrary.RandomFloatInRange` 3.0 5.0)))))
    (:`OnCompleted`
      (`self.ToggleAttackCollision` false :!label _label))
    (:`OnInterrupted`
      (goto _label))))

(fn `OnRep_TypeIndex`
  (`PrimitiveComponent.SetMaterial` (`self.Mesh`) 0 (`|GetArrayItem` (`self.TypeMaterials`) (`self.TypeIndex`))))

(fn `UserConstructionScript`
  (`parent.UserConstructionScript`)
  (`SceneComponent.K2_AttachToComponent` (`self.Weapon`) (`self.Mesh`) "spine_03" "KeepRelative" "KeepRelative" "KeepRelative" true))