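; Orc AI character that reacts to being shot and exposes target, patrol point and action state through getter functions.
; Point damage knocks it back, stops movement while keeping its path, and multicasts a brief red light flash.
; A Character damage causer becomes its target, cleared by a retriggerable delay after ten seconds without further hits.
; A server-side random-wander loop remains in the graph but is never run.
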(event `MULTICAST_Trigger`
  (bind _pointlight (`self.PointLight`))
  (`LightComponent.SetLightColor` _pointlight (struct :`R` 1.0 :`G` 0.011765 :`A` 1.0) true)
  (`KismetSystemLibrary.RetriggerableDelay` 0.2)
  (`LightComponent.SetLightColor` _pointlight (struct :`R` 0.592157 :`G` 1.0 :`B` 0.482353 :`A` 1.0) true))

(event `self.ReceivePointDamage`
  (params (Damage :type "Float (single-precision)") (DamageType :type "DamageType Object Reference") (HitLocation :type "Vector Structure") (HitNormal :type "Vector Structure") (HitComponent :type "PrimitiveComponent Object Reference") (BoneName :type Name) (ShotFromDirection :type "Vector Structure") (InstigatedBy :type "Controller Object Reference") (DamageCauser :type "Actor Object Reference") (HitInfo :type "HitResult Structure (by ref)"))
  (`self.LaunchCharacter` (`KismetMathLibrary.MakeVector` (* ShotFromDirection_X 150.0) (* ShotFromDirection_Y 150.0) 100.0))
  (`NavMovementComponent.StopMovementKeepPathing` (`self.CharacterMovement`))
  (`self.MULTICAST_Trigger`)
  (bind _ascharacter (cast `Character` DamageCauser))
  (set `self.Target` _ascharacter)
  (`KismetSystemLibrary.RetriggerableDelay` 10.0)
  (set `self.Target` null))

(event `self.ReceiveBeginPlay`)

(fn `GetActionState`
  (returns (ActionState :type "/Game/Core/Blueprints/E_ActionState Enum"))
  (return (`self.ActionState`)))

(fn `GetPatrolDestination`
  (returns (Destination :type "Vector Structure"))
  (return (`NavigationSystemV1.K2_GetRandomReachablePointInRadius` (`self.K2_GetActorLocation`) 300.0 null null)))

(fn `GetTarget`
  (returns (HasTarget :type Boolean) (Actor :type "Actor Object Reference") (Location :type "Vector Structure"))
  (bind _target (`self.Target`))
  (`/Engine/EditorBlueprintResources/StandardMacros.IsValid` _target
    (:`Is Valid`
      (return true _target (+ (`self.K2_GetActorLocation` _target) (0.0 0.0 -200.0))))
    (:`Is Not Valid`
      (return false null (0.0 0.0 0.0)))))

(fn `UserConstructionScript`)