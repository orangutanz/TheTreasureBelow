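; BP_Elemental is an AI-controlled elemental character that roams the world.
; On BeginPlay, only the authority starts the BT_Roam behavior tree through the AI controller, then Initialize runs on both server and clients.
; The construction script attaches the OffHandItem and Weapon components to the left and right hand sockets of the mesh, keeping their relative transforms.
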(event `self.ReceiveBeginPlay`
  ;[1 0 0.01749] BeginPlay
  (`/Engine/EditorBlueprintResources/ActorMacros.Switch Has Authority`
    (:`Authority`
      (`AIController.RunBehaviorTree` (`AIBlueprintHelperLibrary.GetAIController` self) "/Game/Core/Blueprints/AI/Behavior/BT_Roam.BT_Roam"))
    (:`Remote`
      _))
  (`self.Initialize`))

(fn `UserConstructionScript`
  (bind _mesh (`self.Mesh`))
  (`SceneComponent.K2_AttachToComponent` (`self.OffHand_Item`) _mesh "hand_l" "KeepRelative" "KeepRelative" "KeepRelative" true)
  (`SceneComponent.K2_AttachToComponent` (`self.Weapon`) _mesh "hand_r" "KeepRelative" "KeepRelative" "KeepRelative" true))