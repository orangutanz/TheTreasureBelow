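; BP_Projectile is a thrown-item projectile that damages what its box overlaps and can drop back into the world as a pickup.
; Construction applies its velocity, flags player-instigated shots and reads damage from DT_Thorwable by item ID.
; Player shots trigger reactions on enemies and enemy shots target players; both hit interactables, with damage applied server-side.
; It is destroyed on hit or stop, and the server then spawns BP_Item_Pickup for valid item IDs.
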(event `self.Box.OnComponentBeginOverlap`
  (params (OverlappedComponent :type "PrimitiveComponent Object Reference") (OtherActor :type "Actor Object Reference") (OtherComp :type "PrimitiveComponent Object Reference") (OtherBodyIndex :type Integer) (bFromSweep :type Boolean) (SweepResult :type "HitResult Structure (by ref)"))
  (bind _returnvalue (`self.GetInstigator`))
  (bind _damageamount (`self.DamageAmount`))
  (bind (_x _y) (`KismetMathLibrary.BreakVector3f` (`KismetMathLibrary.GetDirectionUnitVector` (`self.K2_GetActorLocation`) (`self.K2_GetActorLocation` OtherActor))))
  (if (`self.FromPlayer`)
    (bind _asbpi_enemy (cast `/Game/Core/Blueprints/AI/BPI_Enemy` OtherActor)
      (:`then`
        (`/Game/Core/Blueprints/AI/BPI_Enemy.Enemy_DamageReaction` _asbpi_enemy _damageamount _x _y _returnvalue))
      (:`CastFailed`
        (cast `/Game/Core/Blueprints/Interface/BPI_Interactable` OtherActor :!label _label)))
    (else
      (cast `/Game/Core/Blueprints/Interface/BPI_Player` OtherActor
        (:`then`
          _)
        (:`CastFailed`
          (goto _label)))))
  (if (`KismetSystemLibrary.IsServer`)
    (`GameplayStatics.ApplyDamage` OtherActor _damageamount (`Pawn.GetController` _returnvalue) self))
  (`self.K2_DestroyActor`))

(event `self.ProjectileMovement.OnProjectileStop`
  (params (ImpactResult :type "HitResult Structure (by ref)"))
  (`self.K2_DestroyActor`))

(event `self.ReceiveDestroyed`
  (bind _fromitem (`self.FromItem`))
  (if (`KismetSystemLibrary.IsServer`)
    (if (!= (`.ItemID` (break `ItemInfo` _fromitem)) "0")
      (`|SpawnActorFromClass` "/Game/Core/Blueprints/LevelBP/BP_Item_Pickup.BP_Item_Pickup_C" (`KismetMathLibrary.MakeTransform` (.location (`self.GetTransform`)) (`KismetMathLibrary.RandomRotator` false)) "Undefined" "OverrideRootScale" null true _fromitem null))))

(fn `UserConstructionScript`
  (set `MovementComponent.Velocity` (`self.Velocity`) (`self.ProjectileMovement`))
  (cast `/Game/Core/Blueprints/Interface/BPI_Player` (`self.GetInstigator`)
    (:`then`
      (set `self.FromPlayer` true))
    (:`CastFailed`
      _))
  (bind _returnvalue (`|GetDataTableRow` "/Game/Core/Database/Item/Thrown/DT_Thorwable.DT_Thorwable" (`.ItemID` (break `ItemInfo` (`self.FromItem`))))
    (:`then`
      (set `self.DamageAmount` (`KismetMathLibrary.Conv_IntToDouble` (`.Damage_11_062802D24BE3AAEE3529E1911294B20D` (break `/Game/Core/Database/Item/Thrown/ST_Thrown` _returnvalue)))))))