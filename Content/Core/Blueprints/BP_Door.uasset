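; BP_Door is an interactable, networked door that swings open once, with its mesh chosen by DoorType in the construction script.
; While closed, it can highlight its frame and leaf through custom depth and forwards interaction through the player controller to the server, which sets IsOpened.
; The IsOpened RepNotify enables Tick, which rotates the hinge until it passes a quarter turn, then disables itself.
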(event `self.ReceiveTick`
  (params (DeltaSeconds :type "Float (single-precision)"))
  (bind _hinge (`self.Hinge`))
  (if (< (.yaw (`SceneComponent.RelativeRotation` _hinge)) -90.0)
    (`self.SetActorTickEnabled` false)
    (else
      (`SceneComponent.K2_AddRelativeRotation` _hinge (`KismetMathLibrary.MakeRotator` 0.0 0.0 (* DeltaSeconds -150.0)) false false))))

(event `/Game/Core/Blueprints/Interface/BPI_Interactable.Client_ToggleHightlight`
  (params (Toggle :type Boolean))
  (if Toggle
    (if (not (`self.IsOpened`))
      (`PrimitiveComponent.SetRenderCustomDepth` (`self.DoorFrame`) Toggle :!label _label)
      (`PrimitiveComponent.SetRenderCustomDepth` (`self.Door`) Toggle))
    (else
      (goto _label))))

(event `/Game/Core/Blueprints/Interface/BPI_Interactable.Client_Interaction`
  (if (not (`self.IsOpened`))
    (message `/Game/Core/Blueprints/Interface/BPI_PlayerController.InteractActorOnServer` (`GameplayStatics.GetPlayerController` 0) self)))

(event `/Game/Core/Blueprints/Interface/BPI_Interactable.Server_Interaction`
  (params (Player :type "PlayerController Object Reference"))
  (set `self.IsOpened` true))

(fn `Client_GetItemInfo`
  (returns (Show :type Boolean) (ItemInfo :type "ItemInfo Structure"))
  (return false))

(fn `OnRep_IsOpened`
  (`self.SetActorTickEnabled` true))

(fn `UserConstructionScript`
  (`StaticMeshComponent.SetStaticMesh` (`self.Door`) (select `int` (`self.DoorType`) :`0` "/Game/Kobo_Dungeon/Meshes/SM-Gate-01-02.SM-Gate-01-02" :`1` "/Game/Kobo_Dungeon/Meshes/SM-Gate-01-03.SM-Gate-01-03" :!type "StaticMesh Object Reference")))