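; Arena spawn point that runs a countdown for a named enemy and is visible only while that countdown is active.
; A one-shot timer started with the given delay broadcasts the spawning dispatcher with the enemy name and itself, leaving the actual spawn to listeners.
; RepNotify variables toggle visibility and, on a name change, async-load the pawn class from DT_Enemy during the countdown.
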(event `CE_StartSpawnCountDown`
  (params (Time :type "Float (single-precision)" :default 5.0) (SpawnEntityName :type Name))
  (set `self.SpawnEnemyName` SpawnEntityName)
  (`KismetSystemLibrary.K2_SetTimerDelegate` (delegate `CE_OnSpawnTime`) Time)
  (set `self.IsSpawning` true))

(event `CE_OnSpawnTime`
  (`self.ED_OnSpawning` (`self.SpawnEnemyName`) self)
  (set `self.IsSpawning` false))

(event `CE_AsyncLoadEnemy`
  (bind _returnvalue (`|GetDataTableRow` "/Game/Core/Database/AI/DT_Enemy.DT_Enemy" (`self.SpawnEnemyName`))
    (:`then`
      (`|LoadAssetClass` (`.PawnRef_31_887DF8C2413C039B55AC6F9E9964DB29` (break `/Game/Core/Database/AI/ST_EnemyEntity` _returnvalue))))))

(fn `OnRep_IsSpawning`
  (`self.SetActorHiddenInGame` (not (`self.IsSpawning`))))

(fn `OnRep_SpawnEnemyName`
  (`self.CE_AsyncLoadEnemy`))

(fn `UserConstructionScript`)