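; Arena manager that runs wave-based enemy fights and toggles the arena menu.
; ArenaState's OnRep drives the server through Entering and Fighting, starting waves, and announces state changes.
; Waves start countdowns on random free spawn points, whose callbacks spawn DT_EnemyList pawns and track deaths.
; Only Instant waves advance when cleared; the last wave sets Exiting, and SERVER_SetupNewWave either starts a hardcoded goblin/orc fight or resets from Exiting.
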(event `CE_ServerSetup`
  ;[1 1 1] Spawn entity flow
  (for _array_element (`self.SpawnLocations`)
    (add `/Game/Core/Blueprints/Arena/BP_SpawnLocation.ED_OnSpawning` _array_element (delegate `CE_OnSpawningEntity`))))

(event `CE_OnSpawningEntity`
  (params (SpawnEntityName :type Name) (SpawnLocation :type "/Game/Core/Blueprints/Arena/BP_SpawnLocation Object Reference"))
  ;[1 1 1] Spawn entity flow
  (bind _returnvalue (`|GetDataTableRow` "/Game/Core/Database/AI/DT_EnemyList.DT_EnemyList" SpawnEntityName)
    (:`then`
      (bind ((`NameID_15_850DA2BB440BE3CEFA7F87A224E39BC5` _nameid) (`PawnRef_31_887DF8C2413C039B55AC6F9E9964DB29` _pawnref)) (break `/Game/Core/Database/AI/ST_EnemyEntity` _returnvalue))
      (bind _returnvalue_2 (`KismetSystemLibrary.LoadClassAsset_Blocking` _pawnref))
      (bind _aspawn (castclass `Pawn` _returnvalue_2))
      (bind _returnvalue_3 (`|SpawnActorFromClass` _aspawn (`KismetMathLibrary.MakeTransform` (+ (`self.K2_GetActorLocation` SpawnLocation) (0.0 0.0 50.0)) (`self.K2_GetActorRotation` SpawnLocation)) "AdjustIfPossibleButAlwaysSpawn" "OverrideRootScale" null null))
      (bind _asbp_base_enemy (cast `/Game/Core/Blueprints/AI/BP_BaseEnemy` _returnvalue_3))
      (message `/Game/Core/Blueprints/AI/BPI_Enemy.SetEnemyTypeName` _asbp_base_enemy _returnvalue _nameid)
      (`KismetArrayLibrary.Array_Add` (`self.LiveEnemies`) _asbp_base_enemy)
      (add `/Game/Core/Blueprints/AI/BP_BaseEnemy.ED_OnDeath` _asbp_base_enemy (delegate `CE_OnEnemyDeath`)))))

(event `CE_SpawnEnemy`
  (params (Time :type "Float (single-precision)") (EnemyName :type Name :default "GoblinMelee"))
  ;[1 1 1] TO DO: Wave based enemies
  (bind (_spawnlocation _success) (`self.GetFreeSpawnLocation`))
  (if _success
    (`/Game/Core/Blueprints/Arena/BP_SpawnLocation.CE_StartSpawnCountDown` _spawnlocation Time EnemyName)
    (else
      (`KismetSystemLibrary.PrintString` "Failed to spawn enemy"))))

(event `CE_OnEnemyDeath`
  (params (DeadUnit :type "/Game/Core/Blueprints/AI/BP_BaseEnemy Object Reference"))
  ;[1 1 1] Spawn entity flow
  (`self.HandleDeadEnemy` DeadUnit))

(event `self.ReceiveBeginPlay`
  ;[1 0 0] Begin
  (if (`KismetSystemLibrary.IsServer`)
    (`self.CE_ServerSetup`))
  (message `/Game/Core/Blueprints/Interface/BPI_PlayerController.SetArenaManager` (`GameplayStatics.GetPlayerController` 0) self))

(event `self.SetupNewFight`
  (params (NewWaves :type "Array of /Game/Core/Blueprints/Arena/ST_ArenaWave Structure (by ref)"))
  ;[1 1 1] New Arena Fight
  (`self.IsArenaState` "NewEnumerator0"
    (:`true`
      (if (`KismetArrayLibrary.Array_IsNotEmpty` NewWaves)
        (set `self.ArenaWaves` NewWaves)
        (set `self.CurrentWave` 0)
        (set `self.ArenaState` "NewEnumerator1")))))

(event `SERVER_SetupNewWave`
  (switch `/Game/Core/Blueprints/Arena/Enum_ArenaState` (`self.ArenaState`)
    (:`NewEnumerator0`
      (`self.SetupNewFight` (`|MakeArray` (make `/Game/Core/Blueprints/Arena/ST_ArenaWave` "NewEnumerator0" 0.0 (`|MakeArray` "GoblinMelee" "GoblinMelee" :!type "Name")) (make `/Game/Core/Blueprints/Arena/ST_ArenaWave` "NewEnumerator0" 0.0 (`|MakeArray` "GoblinMelee" "Goblin_Ice" "GoblinMelee" :!type "Name")) (make `/Game/Core/Blueprints/Arena/ST_ArenaWave` "NewEnumerator0" 0.0 (`|MakeArray` "Orc" "Goblin_Ice" "GoblinMelee" :!type "Name")))))
    (:`NewEnumerator3`
      (set `self.ArenaState` "NewEnumerator0"))))

(event `self.ToggleArenaMenu`
  (`/Engine/EditorBlueprintResources/StandardMacros.IsValid` (`self.ArenaMenuRef`)
    (:`Is Valid`
      _)
    (:`Is Not Valid`
      (bind _returnvalue (`|CreateWidget` "/Game/Core/Widgets/Arena/WB_ArenaMenu.WB_ArenaMenu_C"))))
  (bind _output_get (set `self.ArenaMenuRef` _returnvalue))
  (message `/Game/Core/Blueprints/Interface/BPI_HUD.ToggleActiveWidget` (`PlayerController.GetHUD` (`GameplayStatics.GetPlayerController` 0)) _output_get))

(fn `GenerateArenaEntries`
  (params (Amount :type Integer :default 1))
  (locals (NewEntry :type "/Game/Core/Blueprints/Arena/ST_ArenaEntry Structure"))
  (bind _arenaentries (`self.ArenaEntries`))
  (`KismetArrayLibrary.Array_Clear` _arenaentries)
  (for _ (range 1 (+ Amount 1))
    (set `local.NewEntry` (struct))
    (for _ (range (+ (`KismetMathLibrary.RandomIntegerInRange` 0 4) 1))
      (`KismetArrayLibrary.Array_Add` (`.ArenaWaves_3_0B5DB7C643728670F14B0EBD12A1B2EB` (break `/Game/Core/Blueprints/Arena/ST_ArenaEntry` (`local.NewEntry`))) (make `/Game/Core/Blueprints/Arena/ST_ArenaWave` "NewEnumerator0" 0.0 (`|MakeArray` "None" "None" "None" :!type "Name"))))
    (`KismetArrayLibrary.Array_Add` _arenaentries (make `/Game/Core/Blueprints/Arena/ST_ArenaEntry` :`ArenaWaves` (`|MakeArray` (make `/Game/Core/Blueprints/Arena/ST_ArenaWave` "NewEnumerator0") (struct) (struct) (struct) (struct))))))

(fn `GetArenaState`
  (returns (State :type "/Game/Core/Blueprints/Arena/Enum_ArenaState Enum"))
  (return "NewEnumerator0"))

(fn `GetFreeSpawnLocation`
  (returns (SpawnLocation :type "/Game/Core/Blueprints/Arena/BP_SpawnLocation Object Reference") (Success :type Boolean))
  (locals (FreeLocations :type "Array of /Game/Core/Blueprints/Arena/BP_SpawnLocation Object Reference"))
  (bind _freelocations (`local.FreeLocations`))
  (bind (_outitem _outindex) (`KismetArrayLibrary.Array_Random` _freelocations))
  (for _array_element (`self.SpawnLocations`)
    (if (not (`/Game/Core/Blueprints/Arena/BP_SpawnLocation.IsSpawning` _array_element))
      (`KismetArrayLibrary.Array_Add` _freelocations _array_element)))
  (return _outitem (!= _outindex -1)))

(fn `HandleArenaWave`
  (locals (TimeValues :type "Float (double-precision)"))
  (bind _currentwave (`self.CurrentWave`))
  (bind (_wavetype _typevalue _waveenemies) (break `/Game/Core/Blueprints/Arena/ST_ArenaWave` (`|GetArrayItem` (`self.ArenaWaves`) _currentwave)))
  (switch `/Game/Core/Blueprints/Arena/Enum_WaveType` _wavetype
    (:`NewEnumerator0`
      (for _array_element _waveenemies :!label _label
        (`self.CE_SpawnEnemy` 3.0 _array_element)))
    (:`NewEnumerator2`
      (goto _label))
    (:`NewEnumerator1`
      (for _array_element_2 _waveenemies
        (bind _output_get (set `local.TimeValues` (+ _typevalue (`local.TimeValues`))))
        (`self.CE_SpawnEnemy` _output_get _array_element_2))))
  (`/Engine/EditorBlueprintResources/StandardMacros.IncrementInt` _currentwave))

(fn `HandleDeadEnemy`
  (params (UnitDied :type "/Game/Core/Blueprints/AI/BP_BaseEnemy Object Reference"))
  (bind _liveenemies (`self.LiveEnemies`))
  (bind _returnvalue (`KismetArrayLibrary.Array_IsEmpty` _liveenemies))
  (bind _returnvalue_2 (`KismetArrayLibrary.Array_RemoveItem` _liveenemies UnitDied))
  (if _returnvalue_2
    ;[1 1 1] Is Final Wave?
    (if (== (`KismetArrayLibrary.Array_Length` (`self.ArenaWaves`)) (`self.CurrentWave`))
      (if _returnvalue
        (set `self.ArenaState` "NewEnumerator3"))
      (else
        (switch `/Game/Core/Blueprints/Arena/Enum_WaveType` (`.WaveType_19_92FFA006427A9E4DD51771B8D956D0BC` (break `/Game/Core/Blueprints/Arena/ST_ArenaWave` (`|GetArrayItem` (`self.ArenaWaves`) (- (`self.CurrentWave`) 1))))
          (:`NewEnumerator0`
            (if _returnvalue
              (`self.HandleArenaWave`))))))))

(fn `OnRep_ArenaState`
  (bind _arenastate (`self.ArenaState`))
  (`|ExecutionSequence`
    (:`then_0`
      ;[1 1 1] Server Only
      (if (`KismetSystemLibrary.IsServer`)
        (`self.SetupGates`)
        (switch `/Game/Core/Blueprints/Arena/Enum_ArenaState` _arenastate
          (:`NewEnumerator1`
            (set `self.ArenaState` "NewEnumerator2"))
          (:`NewEnumerator2`
            (`self.HandleArenaWave`)))))
    (:`then_1`
      (`self.ED_OnArenaStateChange` _arenastate)
      (switch `/Game/Core/Blueprints/Arena/Enum_ArenaState` _arenastate
        (:`NewEnumerator0`
          (`/Game/Core/Blueprints/Library/FL_Utils.FL_PopMsg` "Arena cleared"))
        (:`NewEnumerator2`
          (`/Game/Core/Blueprints/Library/FL_Utils.FL_PopMsg` "Arena is ready"))
        (:`NewEnumerator3`
          (`/Game/Core/Blueprints/Library/FL_Utils.FL_PopMsg` "Arena ends"))))))

(fn `SetupGates`)

(fn `UserConstructionScript`)