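; Base arena gate actor that players highlight and interact with once to swing open.
; Client interaction is relayed through the player controller to the server, which fires a gate-interaction event dispatcher and sets IsOpened.
; RepNotifies clear custom-depth highlights, enable Tick on opening and zero hinge rotations on closing.
; Tick interpolates each hinge's yaw toward its mapped target at constant speed, disabling itself once all arrive.
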(event `self.ReceiveTick`
  (params (DeltaSeconds :type "Float (single-precision)"))
  (`self.UpdateHinges` DeltaSeconds))

(event `/Game/Core/Blueprints/Interface/BPI_Interactable.Client_ToggleHightlight`
  (params (Toggle :type Boolean))
  (bind _highlightmeshrefs (`self.HighlightMeshRefs`))
  (if Toggle
    (if (and (not (`self.IsOpened`)) (`self.bCanBeInteracted`))
      (for _array_element _highlightmeshrefs
        (`PrimitiveComponent.SetRenderCustomDepth` _array_element true)))
    (else
      (for _array_element_2 _highlightmeshrefs
        (`PrimitiveComponent.SetRenderCustomDepth` _array_element_2 false)))))

(event `/Game/Core/Blueprints/Interface/BPI_Interactable.Client_Interaction`
  (if (and (not (`self.IsOpened`)) (`self.bCanBeInteracted`))
    (message `/Game/Core/Blueprints/Interface/BPI_PlayerController.InteractActorOnServer` (`GameplayStatics.GetPlayerController` 0) self)))

(event `/Game/Core/Blueprints/Interface/BPI_Interactable.Server_Interaction`
  (params (Player :type "PlayerController Object Reference"))
  (if (`self.bCanBeInteracted`)
    (if (not (`self.IsOpened`))
      (`self.ED_OnGateInteraction` Player self)
      (set `self.IsOpened` true))))

(fn `Client_GetItemInfo`
  (returns (Show :type Boolean) (ItemInfo :type "ItemInfo Structure"))
  (return false))

(fn `OnRep_bCanBeInteracted`
  (for _array_element (`self.HighlightMeshRefs`)
    (`PrimitiveComponent.SetRenderCustomDepth` _array_element false)))

(fn `OnRep_IsOpened`
  (if (`self.IsOpened`)
    (for _array_element (`self.HighlightMeshRefs`)
      (`PrimitiveComponent.SetRenderCustomDepth` _array_element false)
      (`self.SetActorTickEnabled` true))
    (else
      (bind _keys (`BlueprintMapLibrary.Map_Keys` (`self.HingeRefs`)))
      (for _array_element_2 _keys
        (`SceneComponent.K2_SetRelativeRotation` :`self` _array_element_2)))))

(fn `UpdateHinges`
  (params (DeltaTime :type "Float (double-precision)"))
  (locals (OpenedDoor :type Integer))
  (bind _hingerefs (`self.HingeRefs`))
  (bind _keys (`BlueprintMapLibrary.Map_Keys` _hingerefs))
  (bind _values (`BlueprintMapLibrary.Map_Values` _hingerefs))
  (for (_array_element _array_index) _keys
    (bind (_relativerotation_roll _relativerotation_pitch _relativerotation_yaw) (`KismetMathLibrary.BreakRotator` (`SceneComponent.RelativeRotation` _array_element)))
    (bind _output (`|GetArrayItem` _values _array_index))
    (`SceneComponent.K2_SetRelativeRotation` _array_element (`KismetMathLibrary.MakeRotator` _relativerotation_roll _relativerotation_pitch (`KismetMathLibrary.FInterpTo_Constant` _relativerotation_yaw _output DeltaTime 150.0)) false false)
    (if (< (`KismetMathLibrary.Abs` (- _relativerotation_yaw _output)) 1.0)
      (`/Engine/EditorBlueprintResources/StandardMacros.IncrementInt` (`local.OpenedDoor`))))
  (if (== (`KismetArrayLibrary.Array_Length` _values) (`local.OpenedDoor`))
    (`self.SetActorTickEnabled` false)))

(fn `UserConstructionScript`)