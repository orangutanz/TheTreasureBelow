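; World pickup for an inventory item, either spawned with item info or placed from a data table row with a clamped quantity.
; Construction and BeginPlay load its mesh and materials by item ID, falling back to a cube mesh or an icon-textured dynamic material.
; Interaction routes through the player controller to the server, which adds it to the pawn's InventoryComponent, destroying it when fully taken or keeping the remainder.
; Highlighting uses custom depth.
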(event `/Game/Core/Blueprints/Interface/BPI_Interactable.Client_ToggleHightlight`
  (params (Toggle :type Boolean))
  ;[1 1 1] Interact hightlight
  (`PrimitiveComponent.SetRenderCustomDepth` (`self.StaticMesh`) Toggle))

(event `/Game/Core/Blueprints/Interface/BPI_Interactable.Client_Interaction`
  ;[1 1 1] Interaction - Pick Up
  (message `/Game/Core/Blueprints/Interface/BPI_PlayerController.InteractActorOnServer` (`GameplayStatics.GetPlayerController` 0) self))

(event `/Game/Core/Blueprints/Interface/BPI_Interactable.Server_Interaction`
  (params (Player :type "PlayerController Object Reference"))
  (bind _returnvalue (`Controller.K2_GetPawn` Player))
  (bind _returnvalue_2 (`self.GetComponentByClass` _returnvalue "/Script/Ape_Inventory.InventoryComponent"))
  ;[1 1 1] Interaction - Pick Up
  (`/Engine/EditorBlueprintResources/StandardMacros.IsValid` _returnvalue_2
    (:`Is Valid`
      (bind _returnvalue_3 (`|GenericCreateObject` "/Script/Ape_Inventory.ItemSlot"))
      (`ItemSlot.SetItemInfo` _returnvalue_3 (`self.Item_Info`))
      (bind _returnvalue_4 (`InventoryComponent.AddItem` _returnvalue_2 _returnvalue_3))
      (if _returnvalue_4
        (message `/Game/Core/Blueprints/Interface/BPI_Pawn.BroadcastMontage` _returnvalue "/Game/Assets/Animation/Montages/Action/AM_Pickup.AM_Pickup")
        ;;[1 1 1] Destroy this pickup
        (`self.K2_DestroyActor`)
        (else
          ;;[1 1 1] If partially added, update quantity
          (bind _returnvalue_5 (`ItemSlot.GetItemInfo` _returnvalue_3))
          (set `self.Item_Info` _returnvalue_5))))))

(event `self.ReceiveBeginPlay`
  (`self.InitializeItem`))

(fn `Client_GetItemInfo`
  (returns (Show :type Boolean) (ItemInfo :type "ItemInfo Structure"))
  (return true (`self.Item_Info`)))

(fn `InitializeItem`
  (locals (ItemInfo :type "/Game/Core/Database/Item/ST_Item Structure"))
  (bind _staticmesh (`self.StaticMesh`))
  (bind (_datatable _rowname) (break `DataTableRowHandle` (`self.PlacedItem`)))
  ;[1 1 1] Using reference
  (if (not (`self.FromSpawn`))
    (bind _returnvalue (`|GetDataTableRow` _datatable _rowname)
      (:`then`
        (bind (_itemid _name _description _maxstack _itemtype) (break `/Game/Core/Database/Item/ST_Item` _returnvalue))
        (set `self.Item_Info` (make `ItemInfo` _itemid _maxstack (`KismetMathLibrary.Clamp` (`self.PlacedAmount`) 1 _maxstack) _itemtype)))))
  (bind _st_item (`/Game/Core/Blueprints/Library/FL_ItemUtil.FL_GetItemInfo` (`.ItemID` (break `ItemInfo` (`self.Item_Info`)))))
  (`|ExecutionSequence`
    (:`then_0`
      (bind (_itemid_2 _name_2 _description_2 _maxstack_2 _itemtype_2 _icon _mesh _materialinstances) (break `/Game/Core/Database/Item/ST_Item` _st_item))
      (bind _returnvalue_2 (`KismetSystemLibrary.LoadAsset_Blocking` _mesh))
      (bind _asstatic_mesh (cast `StaticMesh` _returnvalue_2)
        (:`then`
          (`StaticMeshComponent.SetStaticMesh` _staticmesh _asstatic_mesh))
        (:`CastFailed`
          (`StaticMeshComponent.SetStaticMesh` _staticmesh "/Game/Assets/LevelPrototyping/Meshes/Item_Cube.Item_Cube"))))
    (:`then_1`
      (if (`KismetArrayLibrary.Array_IsEmpty` _materialinstances)
        (bind _returnvalue_3 (`KismetSystemLibrary.LoadAsset_Blocking` _icon))
        (bind _astexture_2d (cast `Texture2D` _returnvalue_3))
        (bind _returnvalue_4 (`PrimitiveComponent.CreateDynamicMaterialInstance` _staticmesh 0 "/Game/Assets/Materials/MAT_PickUp.MAT_PickUp" "None"))
        (`MaterialInstanceDynamic.SetTextureParameterValue` _returnvalue_4 "Normal" _astexture_2d)
        (`PrimitiveComponent.SetMaterial` _staticmesh 0 _returnvalue_4)
        (else
          (for (_array_element _array_index) _materialinstances
            (bind _returnvalue_5 (`KismetSystemLibrary.LoadAsset_Blocking` _array_element))
            (bind _asmaterial_instance (cast `MaterialInstance` _returnvalue_5))
            (`PrimitiveComponent.SetMaterial` _staticmesh _array_index _asmaterial_instance)))))))

(fn `UserConstructionScript`
  (`self.InitializeItem`))