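; Arena manager that runs server-side enemy spawning, replacing each enemy that dies with a new GoblinMelee; wave logic is still a TODO.
; Spawning starts a countdown on a random free spawn location, whose dispatcher triggers a DT_EnemyList lookup, blocking class load and pawn spawn.
; Live enemies are tracked, and their death events request the next spawn.
; On BeginPlay it also registers itself with player controller 0.
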(event `CE_ServerSetup`
  ;[1 1 1] Spawn entity flow
  (for _array_element (`self.SpawnLocations`)
    (add `/Game/Core/Blueprints/BP_SpawnLocation.ED_OnSpawning` _array_element (delegate `CE_OnSpawningEntity`))))

(event `CE_OnSpawningEntity`
  (params (SpawnEntityName :type Name) (SpawnLocation :type "/Game/Core/Blueprints/BP_SpawnLocation Object Reference"))
  ;[1 1 1] Spawn entity flow
  (bind _returnvalue (`|GetDataTableRow` "/Game/Core/Database/AI/DT_EnemyList.DT_EnemyList" SpawnEntityName)
    (:`then`
      (bind ((`NameID_15_850DA2BB440BE3CEFA7F87A224E39BC5` _nameid) (`PawnRef_31_887DF8C2413C039B55AC6F9E9964DB29` _pawnref)) (break `/Game/Core/Database/AI/ST_EnemyEntity` _returnvalue))
      (bind _returnvalue_2 (`KismetSystemLibrary.LoadClassAsset_Blocking` _pawnref))
      (bind _aspawn (castclass `Pawn` _returnvalue_2))
      (bind _returnvalue_3 (`|SpawnActorFromClass` _aspawn (`KismetMathLibrary.MakeTransform` (+ (`self.K2_GetActorLocation` SpawnLocation) (0.0 0.0 50.0)) (`self.K2_GetActorRotation` SpawnLocation)) "AdjustIfPossibleButAlwaysSpawn" "OverrideRootScale" null null))
      (bind _asbp_base_enemy (cast `/Game/Core/Blueprints/AI/BP_BaseEnemy` _returnvalue_3))
      (message `/Game/Core/Blueprints/AI/BPI_Enemy.SetEnemyTypeName` _asbp_base_enemy _returnvalue _nameid)
      (`KismetArrayLibrary.Array_Add` (`self.LiveEnemies`) _asbp_base_enemy)
      (add `/Game/Core/Blueprints/AI/BP_BaseEnemy.ED_OnDeath` _asbp_base_enemy (delegate `CE_OnEnemyDeath`)))))

(event `CE_SpawnEnemies`
  ;[1 1 1] TO DO: Wave based enemies
  (bind (_spawnlocation _success) (`self.GetFreeSpawnLocation`))
  (if _success
    (`/Game/Core/Blueprints/BP_SpawnLocation.CE_StartSpawnCountDown` _spawnlocation 3.0 "GoblinMelee")
    (else
      (`KismetSystemLibrary.PrintString` "Failed to spawn enemy"))))

(event `CE_OnEnemyDeath`
  (params (DeadUnit :type "/Game/Core/Blueprints/AI/BP_BaseEnemy Object Reference"))
  ;[1 1 1] Spawn entity flow
  (bind _returnvalue (`KismetArrayLibrary.Array_RemoveItem` (`self.LiveEnemies`) DeadUnit))
  (if _returnvalue
    (`self.CE_SpawnEnemies`)))

(event `self.ReceiveBeginPlay`
  ;[1 0 0] Begin
  (if (`KismetSystemLibrary.IsServer`)
    (`self.CE_SpawnEnemies`)
    (`self.CE_ServerSetup`))
  (message `/Game/Core/Blueprints/Interface/BPI_PlayerController.SetArenaManager` (`GameplayStatics.GetPlayerController` 0) self))

(fn `GetFreeSpawnLocation`
  (returns (SpawnLocation :type "/Game/Core/Blueprints/BP_SpawnLocation Object Reference") (Success :type Boolean))
  (locals (FreeLocations :type "Array of /Game/Core/Blueprints/BP_SpawnLocation Object Reference"))
  (bind _freelocations (`local.FreeLocations`))
  (bind (_outitem _outindex) (`KismetArrayLibrary.Array_Random` _freelocations))
  (for _array_element (`self.SpawnLocations`)
    (if (not (`/Game/Core/Blueprints/BP_SpawnLocation.IsSpawning` _array_element))
      (`KismetArrayLibrary.Array_Add` _freelocations _array_element)))
  (return _outitem (!= _outindex -1)))

(fn `UserConstructionScript`)