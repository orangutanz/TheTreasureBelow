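; BP_DamageText is a pooled actor that shows a floating damage number through a WB_DamageText widget component.
; On activation, OnDamage sets the widget text and starts a looping timer for the animation.
; Timer steps drive the widget's manual animation, briefly popping the text larger, then lerping it upward while shrinking.
; After half a second it pauses the timer, deactivates and asks the HUD to return it to the pool.
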(event `self.OnActorToggled`
  (params (bNewActive :type Boolean))
  (if bNewActive
    (`self.OnDamage`)))

(event `CE_FloatingAnim`
  (bind _curranimtime (`self.CurrAnimTime`))
  (bind _as_wb_damage_text (`self.As WB Damage Text`))
  (bind _returnvalue (* (- (`self.CurrAnimTime`) 0.1) 2.0))
  (`|ExecutionSequence`
    (:`then_0`
      (if (< _curranimtime 0.5)
        (if (< _curranimtime 0.1)
          (`/Game/Core/Widgets/World/WB_DamageText.ManualAnimation` _as_wb_damage_text 0.0 1.5)
          (else
            (`/Game/Core/Widgets/World/WB_DamageText.ManualAnimation` _as_wb_damage_text (`KismetMathLibrary.Lerp` 0.0 -20.0 _returnvalue) (`KismetMathLibrary.Lerp` 1.5 0.8 _returnvalue))))
        (else
          (`KismetSystemLibrary.K2_PauseTimerHandle` (`self.AnimHandle`))
          (`self.SetActorActive` false)
          (message `/Game/Core/Blueprints/Framework/BPI_HUD.ReturnPoolActor` (`PlayerController.GetHUD` (`GameplayStatics.GetPlayerController` 0)) self))))
    (:`then_1`
      (set `self.CurrAnimTime` (+ (`self.CurrAnimTime`) 0.05)))))

(fn `OnDamage`
  (bind _as_wb_damage_text (`self.As WB Damage Text`))
  (`/Engine/EditorBlueprintResources/StandardMacros.IsValid` (`self.As WB Damage Text`)
    (:`Is Valid`
      _)
    (:`Is Not Valid`
      (bind _aswb_damage_text (cast `/Game/Core/Widgets/World/WB_DamageText` (`WidgetComponent.GetWidget` (`self.Widget`))))
      (set `self.As WB Damage Text` _aswb_damage_text)))
  (`/Game/Core/Widgets/World/WB_DamageText.SetDamageText` _as_wb_damage_text (`self.Damage`))
  (set `self.CurrAnimTime` 0.0)
  (`WidgetComponent.SetTickMode` (`self.Widget`) "Enabled")
  (`/Game/Core/Widgets/World/WB_DamageText.ManualAnimation` _as_wb_damage_text 0.0 1.0)
  (bind _returnvalue (`KismetSystemLibrary.K2_SetTimerDelegate` (`|CreateDelegate` :!event `CE_FloatingAnim`) 0.05 true))
  (set `self.AnimHandle` _returnvalue))

(fn `UserConstructionScript`
  (bind _aswb_damage_text (cast `/Game/Core/Widgets/World/WB_DamageText` (`WidgetComponent.GetWidget` (`self.Widget`))))
  (set `self.As WB Damage Text` _aswb_damage_text))