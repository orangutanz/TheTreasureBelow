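; BP_SpellBall is a pooled electric projectile that homes on a target actor and damages players it overlaps.
; A multicast launch starts homing and sound, and the authority enables the capsule's query collision after a short delay.
; Tick drops homing near the target, continuing straight with a timer that accelerates it toward max speed.
; Pool toggling activates or resets movement and Niagara, and a hit list prevents repeat damage.
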(event `MULTICAST_HomingTarget`
  (params (TargetActor :type "Actor Object Reference"))
  (bind _audio (`self.Audio`))
  (bind _projectilemovement (`self.ProjectileMovement`))
  (`/Engine/EditorBlueprintResources/StandardMacros.IsValid` TargetActor
    (:`Is Valid`
      (`KismetArrayLibrary.Array_Clear` (`self.Other Actor`))
      (set `ProjectileMovementComponent.bIsHomingProjectile` true _projectilemovement)
      (set `ProjectileMovementComponent.HomingTargetComponent` (`Actor.RootComponent` TargetActor) _projectilemovement)
      (`AudioComponent.SetSound` _audio "/Game/Audio/SmallSoundKit/SSKWav/MagicWav/Mgc_Electric_Throw_01.Mgc_Electric_Throw_01")
      (`AudioComponent.Play` _audio 0.0)
      (`/Engine/EditorBlueprintResources/ActorMacros.Switch Has Authority`
        (:`Authority`
          (`KismetSystemLibrary.Delay` 0.3)
          (`PrimitiveComponent.SetCollisionEnabled` (`self.CapsuleCollider`) "QueryOnly"))))))

(event `MULTICAST_StraightLine`
  (bind _projectilemovement (`self.ProjectileMovement`))
  (bind _projectilemovement_2 (`self.ProjectileMovement`))
  (bind _maxspeed (`ProjectileMovementComponent.MaxSpeed` _projectilemovement))
  (`/Engine/EditorBlueprintResources/StandardMacros.IsValid` _projectilemovement_2
    (:`Is Valid`
      (set `ProjectileMovementComponent.bIsHomingProjectile` false _projectilemovement_2)
      (set `ProjectileMovementComponent.HomingTargetComponent` null _projectilemovement_2)
      (if (`MovementComponent.IsExceedingMaxSpeed` _projectilemovement _maxspeed)
        (set `MovementComponent.Velocity` (* (`KismetMathLibrary.GetDirectionUnitVector` (`self.K2_GetActorLocation`) (`self.K2_GetActorLocation` (`ActorComponent.GetOwner` (`ProjectileMovementComponent.HomingTargetComponent` _projectilemovement_2)))) _maxspeed) _projectilemovement_2)
        (else
          (bind _returnvalue (`KismetSystemLibrary.K2_SetTimerDelegate` (delegate `CE_SpeedUp`) 0.1 true))
          (set `self.SpeedUpTimer` _returnvalue))))))

(event `CE_SpeedUp`
  (bind _projectilemovement (`self.ProjectileMovement`))
  (bind _projectilemovement_2 (`self.ProjectileMovement`))
  (set `MovementComponent.Velocity` (+ (`MovementComponent.Velocity` _projectilemovement) (* (`self.GetActorForwardVector`) 10.0)) _projectilemovement)
  (if (`MovementComponent.IsExceedingMaxSpeed` _projectilemovement_2 (`ProjectileMovementComponent.MaxSpeed` _projectilemovement_2))
    (`KismetSystemLibrary.K2_PauseTimerHandle` (`self.SpeedUpTimer`))))

(event `self.ReceiveTick`
  (params (DeltaSeconds :type "Float (single-precision)"))
  (bind _projectilemovement (`self.ProjectileMovement`))
  (if (`ProjectileMovementComponent.bIsHomingProjectile` _projectilemovement)
    (if (< (`self.GetSquaredHorizontalDistanceTo` (`ActorComponent.GetOwner` (`ProjectileMovementComponent.HomingTargetComponent` _projectilemovement))) 50000.0)
      (`self.MULTICAST_StraightLine`)
      (`self.SetActorTickEnabled` false))))

(event `self.OnActorToggled`
  (params (bNewActive :type Boolean))
  (bind _projectilemovement (`self.ProjectileMovement`))
  (bind _ns_niagara (`self.NS_Niagara`))
  (if bNewActive
    (`ActorComponent.SetActive` _ns_niagara true true)
    (`ActorComponent.SetActive` (`self.ProjectileMovement`) true true)
    (else
      (`ActorComponent.Deactivate` _ns_niagara)
      (`ActorComponent.Deactivate` (`self.ProjectileMovement`))
      (set `ProjectileMovementComponent.bIsHomingProjectile` false _projectilemovement)
      (set `ProjectileMovementComponent.HomingTargetComponent` null _projectilemovement)
      (`PrimitiveComponent.SetCollisionEnabled` (`self.CapsuleCollider`) "NoCollision"))))

(event `self.CapsuleCollider.OnComponentBeginOverlap`
  (params (OverlappedComponent :type "PrimitiveComponent Object Reference") (OtherActor :type "Actor Object Reference") (OtherComp :type "PrimitiveComponent Object Reference") (OtherBodyIndex :type Integer) (bFromSweep :type Boolean) (SweepResult :type "HitResult Structure (by ref)"))
  (if (`Actor.bCanBeDamaged` OtherActor)
    (cast `/Game/Core/Blueprints/Interface/BPI_Player` OtherActor)
    (bind _returnvalue (`KismetArrayLibrary.Array_AddUnique` (`self.Other Actor`) (`|ConvertAsset` OtherActor)))
    (if (!= _returnvalue -1)
      (`GameplayStatics.ApplyDamage` OtherActor (`KismetMathLibrary.Conv_IntToDouble` (+ (`KismetMathLibrary.RandomBool`) 4)))
      (`GameplayStatics.PlaySoundAtLocation` "/Game/Audio/SmallSoundKit/SSKWav/MagicWav/Mgc_Electric_Hit_01.Mgc_Electric_Hit_01" (`SceneComponent.K2_GetComponentLocation` (`self.DefaultSceneRoot`)) (struct) 1.0 (`KismetMathLibrary.RandomFloatInRange` 0.9 1.1) 0.0 "/Game/Audio/SA_Basic.SA_Basic" null null null))))

(fn `UserConstructionScript`)