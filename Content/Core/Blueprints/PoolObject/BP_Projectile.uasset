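; Thrown-item projectile that deals damage and can leave an item pickup behind.
; FromItem's data table rows supply mesh and damage, while the construction script sets velocity and detects a player instigator.
; Box overlap, gated by an instigator comparison, filters targets through player, enemy and interactable interfaces, applying server-side damage before destroying itself.
; Stopping also destroys it, and destruction conditionally spawns BP_Item_Pickup on the server, based on ItemID.
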(event `self.ReceiveBeginPlay`
  (`self.Initialize`))

(event `self.Box.OnComponentBeginOverlap`
  (params (OverlappedComponent :type "PrimitiveComponent Object Reference") (OtherActor :type "Actor Object Reference") (OtherComp :type "PrimitiveComponent Object Reference") (OtherBodyIndex :type Integer) (bFromSweep :type Boolean) (SweepResult :type "HitResult Structure (by ref)"))
  (bind _returnvalue (`self.GetInstigator`))
  (bind _damageamount (`self.DamageAmount`))
  (if (not (!= OtherActor (`self.GetInstigator`)))
    (if (`self.FromPlayer`)
      (bind _asbpi_enemy (cast `/Game/Core/Blueprints/Pawn/Enemy/BPI_Enemy` OtherActor)
        (:`then`
          (`/Game/Core/Blueprints/Pawn/Enemy/BPI_Enemy.Enemy_DamageReaction` _asbpi_enemy _damageamount _returnvalue))
        (:`CastFailed`
          (cast `/Game/Core/Blueprints/Interface/BPI_Interactable` OtherActor :!label _label)))
      (else
        (cast `/Game/Core/Blueprints/Interface/BPI_Player` OtherActor
          (:`then`
            _)
          (:`CastFailed`
            (goto _label)))))
    (if (`KismetSystemLibrary.IsServer`)
      (`GameplayStatics.ApplyDamage` OtherActor _damageamount (`Pawn.GetController` _returnvalue) self))
    (`self.K2_DestroyActor`)))

(event `self.ProjectileMovement.OnProjectileStop`
  (params (ImpactResult :type "HitResult Structure (by ref)"))
  (`self.K2_DestroyActor`))

(event `self.ReceiveDestroyed`
  (bind _fromitem (`self.FromItem`))
  (bind _itemid (break `ItemInfo` _fromitem))
  (if (`KismetSystemLibrary.IsServer`)
    (if (not (or (!= _itemid "0") (== _itemid "None") (== _itemid "None")))
      (`|SpawnActorFromClass` "/Game/Core/Blueprints/LevelBP/BP_Item_Pickup.BP_Item_Pickup_C" (`KismetMathLibrary.MakeTransform` (.location (`self.GetTransform`)) (`KismetMathLibrary.RandomRotator` false)) "Undefined" "OverrideRootScale" null true _fromitem null))))

(fn `Initialize`
  (bind _returnvalue (`|GetDataTableRow` "/Game/Core/Database/Item/DT_Items.DT_Items" (`.ItemID` (break `ItemInfo` (`self.FromItem`))))
    (:`then`
      (bind _returnvalue_2 (`KismetSystemLibrary.LoadAsset_Blocking` (`.Mesh_30_B96C434B42EC0E522FCFEEA86F5A6C18` (break `/Game/Core/Database/Item/ST_Item` _returnvalue))))
      (bind _asstatic_mesh (cast `StaticMesh` _returnvalue_2))
      (`StaticMeshComponent.SetStaticMesh` (`self.StaticMesh`) _asstatic_mesh))))

(fn `UserConstructionScript`
  (set `MovementComponent.Velocity` (`self.Velocity`) (`self.ProjectileMovement`))
  (cast `/Game/Core/Blueprints/Interface/BPI_Player` (`self.GetInstigator`)
    (:`then`
      (set `self.FromPlayer` true))
    (:`CastFailed`
      _))
  (bind _returnvalue (`|GetDataTableRow` "/Game/Core/Database/Item/Thrown/DT_Thorwable.DT_Thorwable" (`.ItemID` (break `ItemInfo` (`self.FromItem`))))
    (:`then`
      (set `self.DamageAmount` (`KismetMathLibrary.Conv_IntToDouble` (`.Damage_11_062802D24BE3AAEE3529E1911294B20D` (break `/Game/Core/Database/Item/Thrown/ST_Thrown` _returnvalue)))))))