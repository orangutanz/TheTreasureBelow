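; BP_Target_Decal is a targeting indicator actor that shows a transparent-outline preview of a character performing a skill.
; SetSkeletalMeshRef copies a given skeletal mesh and scale, loops the montage looked up by skill name in DT_Skills, and mirrors any weapon mesh at its socket and transform.
; Both meshes have every material slot swapped to MI_Transparent_Outline.
; SetSize scales the whole actor uniformly; ToggleVisibility is an empty stub.
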(fn `SetSize`
  (params (Size :type "Float (double-precision)"))
  (`SceneComponent.SetWorldScale3D` (`self.DefaultSceneRoot`) (`KismetMathLibrary.MakeVector` Size Size Size)))

(fn `SetSkeletalMeshRef`
  (params (SKRef :type "SkeletalMeshComponent Object Reference") (SkillName :type Name) (WeaponRef :type "StaticMeshComponent Object Reference") (Scale :type "Vector Structure"))
  (bind _weapon (`self.Weapon`))
  (bind _previewmesh (`self.PreviewMesh`))
  (`SkeletalMeshComponent.SetSkeletalMeshAsset` _previewmesh (`SkeletalMeshComponent.GetSkeletalMeshAsset` SKRef))
  (`SceneComponent.SetRelativeScale3D` (`self.PreviewMesh`) Scale)
  (for (_ _array_index) (`MeshComponent.GetMaterials` _previewmesh)
    (`PrimitiveComponent.SetMaterial` _previewmesh _array_index "/Game/Assets/FX/Materials/MI_Transparent_Outline.MI_Transparent_Outline"))
  (`|ExecutionSequence`
    (:`then_0`
      (bind _returnvalue (`|GetDataTableRow` "/Game/Core/Database/Animation/DT_Skills.DT_Skills" SkillName)
        (:`then`
          (`SkeletalMeshComponent.PlayAnimation` _previewmesh (`.MontageRef_7_CF634A204B92BC94ADC634AC4FFDA278` (break `/Game/Core/Database/Animation/ST_AnimMontage` (`.SkillMontage_57_713C38E24745108B71876CAD45DD3232` (break `/Game/Core/Database/Animation/ST_Skill` _returnvalue)))) true))))
    (:`then_1`
      (`/Engine/EditorBlueprintResources/StandardMacros.IsValid` WeaponRef
        (:`Is Valid`
          (`StaticMeshComponent.SetStaticMesh` (`self.Weapon`) (`StaticMeshComponent.StaticMesh` WeaponRef))
          (`SceneComponent.K2_AttachToComponent` (`self.Weapon`) (`self.PreviewMesh`) (`SceneComponent.GetAttachSocketName` WeaponRef) "SnapToTarget" "SnapToTarget" "KeepRelative" true)
          (`SceneComponent.K2_SetRelativeTransform` (`self.Weapon`) (`SceneComponent.GetRelativeTransform` WeaponRef) false true)
          (for (_ _array_index_2) (`MeshComponent.GetMaterials` _weapon)
            (`PrimitiveComponent.SetMaterial` _weapon _array_index_2 "/Game/Assets/FX/Materials/MI_Transparent_Outline.MI_Transparent_Outline")
            (`MeshComponent.SetScalarParameterValueOnMaterials` _weapon "Opacity" 1.0)))))))

(fn `ToggleVisibility`
  (params (Visibility :type Boolean)))

(fn `UserConstructionScript`)