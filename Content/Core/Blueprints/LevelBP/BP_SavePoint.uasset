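; BP_SavePoint is a brazier save point that lights when its sphere is first overlapped while unlit.
; The server sets IsLit and notifies the game mode of the new safe point.
; The IsLit RepNotify calls ToggleLight, which swaps the brazier to a lit or unlit dynamic material and toggles the point light and ember effect.
; Its item info query returns hidden.
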(event `self.Sphere.OnComponentBeginOverlap`
  (params (OverlappedComponent :type "PrimitiveComponent Object Reference") (OtherActor :type "Actor Object Reference") (OtherComp :type "PrimitiveComponent Object Reference") (OtherBodyIndex :type Integer) (bFromSweep :type Boolean) (SweepResult :type "HitResult Structure (by ref)"))
  (if (`KismetSystemLibrary.IsServer`)
    (if (not (`self.IsLit`))
      (set `self.IsLit` true)
      (message `/Game/Core/Blueprints/Interface/BPI_GameMode.UpdateNewSafePoint` (`GameplayStatics.GetGameMode`) self))))

(fn `Client_GetItemInfo`
  (returns (Show :type Boolean) (ItemInfo :type "ItemInfo Structure"))
  (return false))

(fn `OnRep_IsLit`
  (`self.ToggleLight` (`self.IsLit`)))

(fn `ToggleLight`
  (params (Toggle :type Boolean))
  (bind _returnvalue (`KismetMaterialLibrary.CreateDynamicMaterialInstance` (select `bool` Toggle :`false` "/Game/Assets/Kobo_Dungeon/Materials/M-Instance/MI-Brazier-01-03.MI-Brazier-01-03" :`true` "/Game/Assets/Kobo_Dungeon/Materials/M-Instance/MI-Brazier-01-02.MI-Brazier-01-02" :!type "MaterialInterface Object Reference")))
  (`PrimitiveComponent.SetMaterial` (`self.SM-Brazier-01-02`) 0 _returnvalue)
  (`SceneComponent.SetVisibility` (`self.PointLight`) Toggle false)
  (`SceneComponent.SetVisibility` (`self.FX-BrazierEmbers-01`) Toggle false))

(fn `UserConstructionScript`)