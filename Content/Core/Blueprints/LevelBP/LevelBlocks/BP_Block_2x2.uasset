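; BP_Block_2x2 is a modular level block with seven wall connection points, used to grow a level from random neighboring blocks.
; UpdateConnectionMesh swaps a connection's wall and foot meshes between solid and door variants, printing the index for doors.
; BPGetRandomPossibleBlockAndIndex overlap-tests candidate blocks (only itself currently) at non-door connections with a temporary query box.
; It returns a random fitting class, transform and connection index.
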(event `self.BP_UpdateConnectionMesh`
  (params (Index :type Integer) (bDoor :type Boolean))
  (`self.SwitchWallMesh` (select `int` Index :`0` (`self.E0_Wall`) :`1` (`self.E1_Wall`) :`2` (`self.E2_Wall`) :`3` (`self.E3_Wall`) :`4` (`self.E4_Wall`) :`5` (`self.E5_Wall`) :`6` (`self.E6_Wall`)) (select `int` Index :`0` (`self.E0_Foot`) :`1` (`self.E1_Foot`) :`2` (`self.E2_Foot`) :`3` (`self.E3_Foot`) :`4` (`self.E4_Foot`) :`5` (`self.E5_Foot`) :`6` (`self.E6_Foot`)) bDoor)
  (if bDoor
    (`KismetSystemLibrary.PrintString` (`KismetStringLibrary.Conv_IntToString` Index))))

(fn `BP_GetRandomPossibleBlockAndIndex`
  (returns (OutBlockBP :type "DungeonBlock_Base Class Reference") (OutTransform :type "Transform Structure") (OutConnectionIndex :type Integer))
  (locals (ValidBlocks :type "Array of DungeonBlock_Base Class Reference") (ValidIndex :type "Array of Integer") (ValidTransform :type "Array of Transform Structure") (CacheRandomBlocks :type "Array of DungeonBlock_Base Class Reference") (QueryActor :type "/Game/Core/Blueprints/LevelBP/LevelBlocks/BP_BlockQueryBox Object Reference") (CacheTransform :type "Array of Transform Structure"))
  (bind _queryactor (`local.QueryActor`))
  (bind _cacherandomblocks (`local.CacheRandomBlocks`))
  (bind _validblocks (`local.ValidBlocks`))
  (bind (_outitem _outindex) (`KismetArrayLibrary.Array_Random` _cacherandomblocks))
  (bind (_outitem_2 _outindex_2) (`KismetArrayLibrary.Array_Random` _validblocks))
  (bind _returnvalue (`|SpawnActorFromClass` "/Game/Core/Blueprints/LevelBP/LevelBlocks/BP_BlockQueryBox.BP_BlockQueryBox_C" (`KismetMathLibrary.MakeTransform` (0.0 0.0 0.0) (`KismetMathLibrary.MakeRotator` 0.0)) "AlwaysSpawn" "OverrideRootScale" null null))
  (set `local.QueryActor` _returnvalue)
  (for (_array_element _array_index) (`self.ConnectionPoints`)
    (if (not (`.bIsDoor` (break `BlockConnectionPoint` _array_element)))
      (`KismetArrayLibrary.Array_Clear` (`local.CacheRandomBlocks`))
      (`KismetArrayLibrary.Array_Clear` (`local.CacheTransform`))
      (for _array_element_2 (`|MakeArray` "BP_Block_2x2_C" :!type "DungeonBlock_Base Class Reference")
        (bind _returnvalue_2 (select `int` _array_index :`0` (`self.E0_Foot`) :`1` (`self.E1_Foot`) :`2` (`self.E2_Foot`) :`3` (`self.E3_Foot`) :`4` (`self.E4_Foot`) :`5` (`self.E5_Foot`) :`6` (`self.E6_Foot`)))
        (bind _returnvalue_3 (`SceneComponent.K2_GetComponentLocation` _returnvalue_2))
        (bind (_returnvalue_roll _returnvalue_pitch _returnvalue_yaw) (`KismetMathLibrary.BreakRotator` (`SceneComponent.K2_GetComponentRotation` _returnvalue_2)))
        (bind (_connectionpoints _collisionboxlocation _collisionboxextent _collisionboxrotyaw) (defaults `Object` _array_element_2))
        (bind _returnvalue_4 (+ _returnvalue_yaw _collisionboxrotyaw))
        (`self.K2_SetActorLocationAndRotation` _queryactor _returnvalue_3 (`KismetMathLibrary.MakeRotator` 0.0 0.0 _returnvalue_4) false false)
        (`BoxComponent.SetBoxExtent` (`/Game/Core/Blueprints/LevelBP/LevelBlocks/BP_BlockQueryBox.Box` _queryactor) _collisionboxextent true)
        (bind _isoverlapping (`/Game/Core/Blueprints/LevelBP/LevelBlocks/BP_BlockQueryBox.GetIsOverlapping?` _queryactor))
        (if (not _isoverlapping)
          (`KismetArrayLibrary.Array_Add` (`local.CacheRandomBlocks`) _array_element_2)
          (`KismetArrayLibrary.Array_Add` (`local.CacheTransform`) (`KismetMathLibrary.MakeTransform` _returnvalue_3 (`KismetMathLibrary.MakeRotator` 0.0 0.0 _returnvalue_4)))))
      (if (`KismetArrayLibrary.Array_IsNotEmpty` _cacherandomblocks)
        (`KismetArrayLibrary.Array_Add` (`local.ValidBlocks`) _outitem)
        (`KismetArrayLibrary.Array_Add` (`local.ValidIndex`) _array_index)
        (`KismetArrayLibrary.Array_Add` (`local.ValidTransform`) (`|GetArrayItem` (`local.CacheTransform`) _outindex)))))
  (`self.K2_DestroyActor` (`local.QueryActor`))
  (if (`KismetArrayLibrary.Array_IsNotEmpty` _validblocks)
    (return _outitem_2 (`|GetArrayItem` (`local.ValidTransform`) _outindex_2) (`|GetArrayItem` (`local.ValidIndex`) _outindex_2))
    (else
      (return null (struct) 0))))

(fn `UserConstructionScript`)