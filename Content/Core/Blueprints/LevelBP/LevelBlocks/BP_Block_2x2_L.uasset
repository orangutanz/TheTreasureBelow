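; BP_Block_2x2_L is a level block Blueprint, named as an L-shaped 2x2 piece, with seven indexed edges that can each show a wall or a door.
; UpdateConnectionMesh selects an edge's Wall and Foot components by index and passes them to SwitchWallMesh, which swaps both static meshes between door and solid variants.
; GetEntryMesh returns the Foot component for a given edge index.
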(event `self.BP_UpdateConnectionMesh`
  (params (Index :type Integer) (bDoor :type Boolean))
  (`self.SwitchWallMesh` (select `int` Index :`0` (`self.E0_Wall`) :`1` (`self.E1_Wall`) :`2` (`self.E2_Wall`) :`3` (`self.E3_Wall`) :`4` (`self.E4_Wall`) :`5` (`self.E5_Wall`) :`6` (`self.E6_Wall`)) (select `int` Index :`0` (`self.E0_Foot`) :`1` (`self.E1_Foot`) :`2` (`self.E2_Foot`) :`3` (`self.E3_Foot`) :`4` (`self.E4_Foot`) :`5` (`self.E5_Foot`) :`6` (`self.E6_Foot`)) bDoor))

(fn `GetEntryMesh`
  (params (Index :type Integer))
  (returns (OutMesh :type "StaticMeshComponent Object Reference"))
  (return (select `int` Index :`0` (`self.E0_Foot`) :`1` (`self.E1_Foot`) :`2` (`self.E2_Foot`) :`3` (`self.E3_Foot`) :`4` (`self.E4_Foot`) :`5` (`self.E5_Foot`) :`6` (`self.E6_Foot`))))

(fn `UserConstructionScript`)