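; BP_BlockQueryBox is a helper actor in the level block Blueprints that tests whether a box volume overlaps any actors.
; SetCollisionOffsetExtent moves the Box component to a given relative location and resizes it, updating overlaps.
; GetIsOverlapping? then reports whether the box's overlapping actor list is non-empty, with a disconnected debug loop that would print those actors' names.
; It has no active events or construction logic, so it relies on external calls.
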(fn `GetIsOverlapping?`
  (returns (IsOverlapping :type Boolean))
  (return (`KismetArrayLibrary.Array_IsNotEmpty` (`PrimitiveComponent.GetOverlappingActors` (`self.Box`) null))))

(fn `SetCollisionOffsetExtent`
  (params (NewRelativeLocation :type "Vector Structure") (InBoxExtent :type "Vector Structure"))
  (bind _box (`self.Box`))
  (`SceneComponent.K2_SetRelativeLocation` _box NewRelativeLocation false false)
  (`BoxComponent.SetBoxExtent` _box InBoxExtent true))

(fn `UserConstructionScript`)