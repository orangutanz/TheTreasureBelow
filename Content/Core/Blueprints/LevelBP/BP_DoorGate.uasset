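; Interactable gate door that can be locked behind an inventory key item, with custom-depth highlighting and key info for the player.
; The client checks for the key, showing a message if missing, then the server consumes one and sets IsOpened.
; OnRep_IsOpened fires the open dispatcher, hides the look-at tooltip, plays a creak and streams in an optional level.
; It also enables Tick, which swings the hinge open then disables itself.
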(event `self.ReceiveTick`
  (params (DeltaSeconds :type "Float (single-precision)"))
  (bind _hinge (`self.Hinge`))
  (if (< (.yaw (`SceneComponent.RelativeRotation` _hinge)) 120.0)
    (`SceneComponent.K2_AddRelativeRotation` _hinge (`KismetMathLibrary.MakeRotator` 0.0 0.0 (* DeltaSeconds 150.0)) false false)
    (else
      (`self.SetActorTickEnabled` false)
      (`KismetSystemLibrary.PrintString` "Hello"))))

(event `/Game/Core/Blueprints/Interface/BPI_Interactable.Client_ToggleHightlight`
  (params (Toggle :type Boolean))
  (if Toggle
    (if (not (`self.IsOpened`))
      (`PrimitiveComponent.SetRenderCustomDepth` (`self.Door`) Toggle :!label _label))
    (else
      (goto _label))))

(event `/Game/Core/Blueprints/Interface/BPI_Interactable.Client_Interaction`
  (bind _returnvalue (`GameplayStatics.GetPlayerController` 0))
  (bind _keynamerequired (`self.KeyNameRequired`))
  (if (`self.IsOpened`)
    _
    (elif (`self.Locked?`)
      (if (!= _keynamerequired "None")
        (bind _returnvalue_2 (`InventoryComponent.FindItemQuantity` (`self.GetComponentByClass` (`Controller.K2_GetPawn` _returnvalue) "/Script/Ape_Inventory.InventoryComponent") _keynamerequired))
        (if (> _returnvalue_2 0)
          (message `/Game/Core/Blueprints/Interface/BPI_PlayerController.InteractActorOnServer` _returnvalue self :!label _label_2)
          (else
            (bind _st_item (`/Game/Core/Blueprints/Library/FL_ItemUtil.FL_GetItemInfo` _keynamerequired :!label _label_3))
            (`/Game/Core/Blueprints/Library/FL_Utils.FL_PopMsg` (`|FormatText` "Requires \"{item}\" to open" (`.Name_19_3609B74E46FC585B5AE4DF873DE4032A` (break `/Game/Core/Database/Item/ST_Item` _st_item))))
            (`GameplayStatics.PlaySound2D` "/Game/Audio/WAV/Opening_Locker.Opening_Locker" 1.0 1.0 0.0 null null)))
        (else
          (goto _label_3)))
      (else
        (goto _label_2)))))

(event `/Game/Core/Blueprints/Interface/BPI_Interactable.Server_Interaction`
  (params (Player :type "PlayerController Object Reference"))
  (if (`self.Locked?`)
    (if (not (`self.IsOpened`))
      (bind _returnvalue (`InventoryComponent.RemoveItemByName` (`self.GetComponentByClass` (`Controller.K2_GetPawn` Player) "/Script/Ape_Inventory.InventoryComponent") (`self.KeyNameRequired`) 1))
      (if _returnvalue
        (set `self.IsOpened` true :!label _label_4)))
    (else
      (goto _label_4))))

(event `LoadStreamLevel`
  (`GameplayStatics.LoadStreamLevelBySoftObjectPtr` (`self.LoadLevel`) true)
  (set `self.IsLevelLoaded` true))

(fn `Client_GetItemInfo`
  (returns (Show :type Boolean) (ItemInfo :type "ItemInfo Structure"))
  (if (`self.Locked?`)
    (if (`self.IsOpened`)
      _
      (else
        (bind _st_item (`/Game/Core/Blueprints/Library/FL_ItemUtil.FL_GetItemInfo` (`self.KeyNameRequired`)))
        (bind (_itemid _name _description _maxstack _itemtype) (break `/Game/Core/Database/Item/ST_Item` _st_item))
        (return true (make `ItemInfo` _itemid _maxstack 1 _itemtype)))))
  (return false))

(fn `OnRep_IsOpened`
  (bind _returnvalue (`PlayerController.GetHUD` (`GameplayStatics.GetPlayerController` 0)))
  (if (`self.IsOpened`)
    (`self.ED_OnDoorOpen`)
    (`|ExecutionSequence`
      (:`then_0`
        (bind (_hastarget _targetactor) (message `/Game/Core/Blueprints/Interface/BPI_HUD.GetLookAt` _returnvalue))
        (if (== _targetactor self)
          (message `/Game/Core/Blueprints/Interface/BPI_HUD.ToggleLookatTooltip` _returnvalue false)))
      (:`then_1`
        (`GameplayStatics.PlaySoundAtLocation` "/Game/Audio/WAV/Door_Creak_3.Door_Creak_3" (`self.K2_GetActorLocation`) (struct) 1.0 1.0 0.0 null null null null)
        (`self.SetActorTickEnabled` true))
      (:`then_2`
        (if (`KismetSystemLibrary.IsValidSoftObjectReference` (`self.LoadLevel`))
          (`self.LoadStreamLevel`))))))

(fn `UserConstructionScript`)