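; BP_TP_Interact is an interactable teleporter that requests a level change for the interacting player.
; Client interaction sends the actor to the server through the first player controller's interact message.
; Server interaction then requests the configured LevelName with teleport on load.
; Highlighting toggles custom depth on the static mesh, and the item info query returns hidden.
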(event `/Game/Core/Blueprints/Interface/BPI_Interactable.Client_ToggleHightlight`
  (params (Toggle :type Boolean))
  ;[1 1 1] Interact hightlight
  (`PrimitiveComponent.SetRenderCustomDepth` (`self.StaticMesh`) Toggle))

(event `/Game/Core/Blueprints/Interface/BPI_Interactable.Client_Interaction`
  (message `/Game/Core/Blueprints/Interface/BPI_PlayerController.InteractActorOnServer` (`GameplayStatics.GetPlayerController` 0) self))

(event `/Game/Core/Blueprints/Interface/BPI_Interactable.Server_Interaction`
  (params (Player :type "PlayerController Object Reference"))
  (message `/Game/Core/Blueprints/Interface/BPI_PlayerController.RequestLevel` (`GameplayStatics.GetPlayerController` 0) Player (`self.LevelName`) true))

(fn `Client_GetItemInfo`
  (returns (Show :type Boolean) (ItemInfo :type "ItemInfo Structure"))
  (return false))

(fn `UserConstructionScript`)